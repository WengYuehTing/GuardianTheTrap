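; Cost_BP is a short-lived floating cost popup that shows two resource types and their amounts in a VR game.
; On BeginPlay it passes the resource data to its W_Cost widget and starts a timeline.
; The timeline offsets the actor's height and drives the widget's Alpha, then destroys the actor when finished.
; Every Tick, the widget turns on yaw only to face the VRPawn's head.
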(event `self.ReceiveBeginPlay`
  (bind (_origin_x _origin_y _origin_z) (`KismetMathLibrary.BreakVector` (`self.Origin`)))
  (set `self.Origin` (`self.K2_GetActorLocation`))
  (bind _asw_cost (cast `/Game/Resources/W_Cost` (`WidgetComponent.GetUserWidgetObject` (`self.Widget`))))
  (set `/Game/Resources/W_Cost.FirstResource` (`self.FirstResource`) _asw_cost)
  (set `/Game/Resources/W_Cost.SecondResource` (`self.SecondResource`) _asw_cost)
  (set `/Game/Resources/W_Cost.FirstAmount` (`self.FirstAmount`) _asw_cost)
  (set `/Game/Resources/W_Cost.SecondAmount` (`self.SecondAmount`) _asw_cost)
  (bind (_direction _height _alpha) (`Timeline|Timeline_0` :!via `PlayFromStart`)
    (:`Update`
      (`self.K2_SetActorLocation` (`KismetMathLibrary.MakeVector` _origin_x _origin_y (+ _origin_z _height)))
      (bind _asw_cost_2 (cast `/Game/Resources/W_Cost` (`WidgetComponent.GetUserWidgetObject` (`self.Widget`))))
      (set `/Game/Resources/W_Cost.Alpha` _alpha _asw_cost_2))
    (:`Finished`
      (`self.K2_DestroyActor`))))

(event `self.ReceiveTick`
  (params (DeltaSeconds :type "Float (single-precision)"))
  (bind _asvrpawn (cast `/Game/Player/VRPawn` (`GameplayStatics.GetPlayerPawn` 0)))
  (bind (_returnvalue_roll _returnvalue_pitch _returnvalue_yaw) (`KismetMathLibrary.BreakRotator` (`KismetMathLibrary.FindLookAtRotation` (`SceneComponent.K2_GetComponentLocation` (`self.Widget`)) (`SceneComponent.K2_GetComponentLocation` (`/Game/Player/VRPawn.Head` _asvrpawn)))))
  (`SceneComponent.K2_SetWorldRotation` (`self.Widget`) (`KismetMathLibrary.MakeRotator` 0.0 0.0 _returnvalue_yaw) false false))

(fn `UserConstructionScript`)