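; Barn socket actor that tracks whether its assigned customer Animal has arrived and which unclaimed Animal is closest.
; Each Tick scans all Animals for the nearest self-aware one without a valid SelectedSocket and stores it as NearestIdleAnimal.
; Tick then sets Idle from CustomerAnimal's arrival flag, or true when no customer is valid.
; Box overlap handlers for toggling Idle exist but are disconnected.
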(event `self.ReceiveTick`
  (params (DeltaSeconds :type "Float (single-precision)"))
  (bind _customeranimal (`self.CustomerAnimal`))
  (`self.Set Nearest Idle Enemy`)
  (`/Engine/EditorBlueprintResources/StandardMacros.IsValid` _customeranimal
    (:`Is Valid`
      (bind _asanimal (cast `Animal` _customeranimal))
      (set `self.Idle` (not (`Animal.IsArriveAtSocket` _asanimal))))
    (:`Is Not Valid`
      (set `self.Idle` true))))

(event `Set Nearest Idle Enemy`
  (bind _outactors (`GameplayStatics.GetAllActorsOfClass` "/Script/Guardian_TheTrap.Animal"))
  (for (_array_element _array_index) _outactors
    (bind _asanimal (cast `Animal` _array_element))
    (if (and (not (`KismetSystemLibrary.IsValid` (`Animal.SelectedSocket` _asanimal))) (`Animal.SelfAwareness` _asanimal))
      (bind _returnvalue (`self.GetDistanceTo` _asanimal))
      (if (<= _returnvalue (`self.Min`))
        (set `self.Min` _returnvalue)
        (set `self.Index` _array_index))))
  (if (>= (`self.Index`) 0)
    (set `self.NearestIdleAnimal` (`|GetArrayItem` _outactors (`self.Index`)))
    (else
      (set `self.NearestIdleAnimal` (`self.NullActor`))))
  (set `self.Min` 100000.0)
  (set `self.Index` -1))

(event `self.Box.OnComponentBeginOverlap`
  (params (OverlappedComponent :type "PrimitiveComponent Object Reference") (OtherActor :type "Actor Object Reference") (OtherComp :type "PrimitiveComponent Object Reference") (OtherBodyIndex :type Integer) (bFromSweep :type Boolean) (SweepResult :type "HitResult Structure (by ref)")))

(event `HandleBeginOverlap`
  (params (`Other Actor` :type "Actor Object Reference"))
  (if (and (== (`GameplayStatics.GetObjectClass` `Other Actor`) "/Script/Guardian_TheTrap.Animal") (== `Other Actor` (`self.CustomerAnimal`)))
    (set `self.Idle` false)))

(event `self.Box.OnComponentEndOverlap`
  (params (OverlappedComponent :type "PrimitiveComponent Object Reference") (OtherActor :type "Actor Object Reference") (OtherComp :type "PrimitiveComponent Object Reference") (OtherBodyIndex :type Integer)))

(event `HandleEndOverlap`
  (params (`Other Actor` :type "Actor Object Reference"))
  (if (and (== (`GameplayStatics.GetObjectClass` `Other Actor`) "/Script/Guardian_TheTrap.Animal") (== `Other Actor` (`self.CustomerAnimal`)))
    (set `self.Idle` true)))

(fn `UserConstructionScript`)