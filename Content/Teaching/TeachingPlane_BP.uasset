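; A teaching panel for VR: a plane that shows an assigned material and scales up when play begins.
; Pickup clears the VR pawn's teaching UI flag and scales the plane down.
; An event selector then either destroys the actor, opens the teaching manager's next stage light, or reveals the animal teleport door's text and resets its first wave delay.
; Only the no-event branch destroys the panel.
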(event `self.ReceiveBeginPlay`
  (`PrimitiveComponent.SetMaterial` (`self.Plane`) 0 (`self.Material`))
  (`SceneComponent.K2_SetWorldRotation` (`self.Plane`) (struct :`Pitch` 180.0 :`Roll` 270.0) false false)
  (bind (_direction _scaleup) (`Timeline|ScaleTimeLine` :!via `PlayFromStart`)
    (:`Update`
      (`SceneComponent.SetWorldScale3D` (`self.Plane`) (`KismetMathLibrary.Conv_DoubleToVector` _scaleup)))))

(event `/Game/VirtualRealityBP/Blueprints/PickupActorInterface.Pickup`
  (params (AttachTo :type "SceneComponent Object Reference"))
  (bind _asvrpawn (cast `/Game/Player/VRPawn` (`GameplayStatics.GetPlayerPawn` 0)))
  (set `/Game/Player/VRPawn.IsTeachingUIActive` false _asvrpawn)
  (bind (_direction _scaleup _scaledown) (`Timeline|Timeline_0` :!via `PlayFromStart`)
    (:`Update`
      (`SceneComponent.SetWorldScale3D` (`self.Plane`) (`KismetMathLibrary.Conv_DoubleToVector` _scaledown)))
    (:`Finished`
      (switch `/Game/Teaching/ETeachingUIEvent` (`self.Event`)
        (:`NewEnumerator0`
          (`self.K2_DestroyActor`))
        (:`NewEnumerator1`
          (bind _outactors (`GameplayStatics.GetAllActorsOfClass` "/Game/Teaching/TeachingManager_BP.TeachingManager_BP_C"))
          (if (> (`KismetArrayLibrary.Array_Length` _outactors) 0)
            (`/Game/Teaching/TeachingManager_BP.OpenNextStageLight` (`|GetArrayItem` _outactors))))
        (:`NewEnumerator2`
          (bind _outactors_2 (`GameplayStatics.GetAllActorsOfClass` "/Game/TeleportDoor/Blueprints/AnimalTeleportDoor_BP.AnimalTeleportDoor_BP_C"))
          (if (> (`KismetArrayLibrary.Array_Length` _outactors_2) 0)
            (bind _output (`|GetArrayItem` _outactors_2))
            (`SceneComponent.SetVisibility` (`/Game/TeleportDoor/Blueprints/AnimalTeleportDoor_BP.TextRender` _output) true false)
            (bind _animalsinfo (`EnemyTeleport.AnimalsInfo` _output))
            (bind (_localwavedelay _spawnedrate _animalsorder _currentamount) (break `AnimalsWave` (`|GetArrayItem` _animalsinfo)))
            (`KismetArrayLibrary.Array_Set` _animalsinfo 0 (make `AnimalsWave` 5.0 _spawnedrate _animalsorder _currentamount))))))))

(fn `UserConstructionScript`)