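; Drawer actor for the preparation room that slides along world Y while a hand component holds it.
; Pickup stores the hand and its position, and Drop releases it.
; Each tick applies the hand's Y movement, clamped between the mesh's starting Y and CanMoveLength below it.
; Tick also passes the actor's transform to a server update every frame, held or not, apparently for network sync.
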(event `self.ReceiveBeginPlay`
  (set `self.Origin` (`SceneComponent.K2_GetComponentLocation` (`self.StaticMesh`))))

(event `self.ReceiveTick`
  (params (DeltaSeconds :type "Float (single-precision)"))
  (bind (_returnvalue_x _returnvalue_y _returnvalue_z) (`KismetMathLibrary.BreakVector` (`self.K2_GetActorLocation`)))
  (bind (_pickuplocation_x _pickuplocation_y) (`KismetMathLibrary.BreakVector` (`self.PickUpLocation`)))
  (bind (_origin_x _origin_y) (`KismetMathLibrary.BreakVector` (`self.Origin`)))
  (bind _hand (`self.Hand`))
  (bind (_returnvalue_x_2 _returnvalue_y_2) (`KismetMathLibrary.BreakVector` (`SceneComponent.K2_GetComponentLocation` _hand)))
  (`|ExecutionSequence`
    (:`then_0`
      (`/Engine/EditorBlueprintResources/StandardMacros.IsValid` _hand
        (:`Is Valid`
          (`self.K2_SetActorLocation` (`KismetMathLibrary.MakeVector` _returnvalue_x (`KismetMathLibrary.FClamp` (+ (- _returnvalue_y_2 _pickuplocation_y) _returnvalue_y) (- _origin_y (`self.CanMoveLength`)) _origin_y) _returnvalue_z))
          (set `self.PickUpLocation` (`SceneComponent.K2_GetComponentLocation` (`self.Hand`))))))
    (:`then_1`
      (`self.UpdatePosAndRot_Server` (`self.K2_GetActorLocation`) (`self.K2_GetActorRotation`)))))

(event `/Game/VirtualRealityBP/Blueprints/PickupActorInterface.Pickup`
  (params (AttachTo :type "SceneComponent Object Reference"))
  (set `self.Hand` AttachTo)
  (set `self.PickUpLocation` (`SceneComponent.K2_GetComponentLocation` AttachTo)))

(event `/Game/VirtualRealityBP/Blueprints/PickupActorInterface.Drop`
  (set `self.Hand` null))

(event `UpdatePosAndRot_Server`
  (params (NewLocation :type "Vector Structure") (NewRotation :type "Rotator Structure"))
  (`self.K2_SetActorLocationAndRotation` NewLocation NewRotation))

(fn `UserConstructionScript`)