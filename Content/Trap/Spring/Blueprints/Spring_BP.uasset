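; Spring trap owned by a VR player that launches animals away when one enters its activate zone, and can be picked up, dropped and highlighted.
; An authority-only overlap calls Fire; HandleFire plays animation, sound and particles, hides the hint zone, impulses bounceable animals, then optionally re-arms after a cooldown.
; Tick syncs the transform to the server, drives a material-mask fade-in and forces CanGrab true, leaving the LevelManager grab check unwired.
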(event `self.ReceiveBeginPlay`
  ;[0 0.8148 1] Main BeginPlay
  (bind _asvrpawn (cast `/Game/Player/VRPawn` (`self.GetOwner`)))
  (set `self.PlayerSpawned` _asvrpawn)
  (`self.SetOwner` null))

(event `/Game/VirtualRealityBP/Blueprints/PickupActorInterface.Pickup`
  (params (AttachTo :type "SceneComponent Object Reference"))
  ;[1 0.4394 0] PickUp interface
  (if (`self.CanGrab`)
    (`PrimitiveComponent.SetSimulatePhysics` (`self.SkeletalMesh`) false)
    (`SceneComponent.K2_AttachToComponent` (`self.K2_GetRootComponent`) AttachTo "None" "KeepWorld" "KeepWorld" "KeepWorld" false)))

(event `UpdatePosAndRot_Server`
  (params (NewLocation :type "Vector Structure") (NewRotation :type "Rotator Structure"))
  ;[1 1 1] Sync Position and Rotation
  (`self.K2_SetActorLocationAndRotation` NewLocation NewRotation))

(event `self.ReceiveTick`
  (params (DeltaSeconds :type "Float (single-precision)"))
  (bind _returnvalue (+ (`self.LocalFadeInDuration`) (`GameplayStatics.GetWorldDeltaSeconds`)))
  (`|ExecutionSequence`
    (:`then_0`
      ;[1 1 1] Sync Position and Rotation
      (`self.UpdatePosAndRot_Server` (`self.K2_GetActorLocation`) (`self.K2_GetActorRotation`)))
    (:`then_1`
      ;[1 1 1] Fade In Effect
      (`self.FadeInEffect` _returnvalue)
      (set `self.LocalFadeInDuration` _returnvalue))
    (:`then_2`
      (set `self.CanGrab` true))))

(event `/Game/VirtualRealityBP/Blueprints/PickupActorInterface.Drop`
  ;[1 0.4394 0] PickUp interface
  (`PrimitiveComponent.SetSimulatePhysics` (`self.SkeletalMesh`) true)
  (`self.K2_DetachFromActor` "KeepWorld" "KeepWorld" "KeepWorld"))

(event `/Game/Trap/HighlightInterface.Highlight`
  ;[0.0488 1 0] Hightlight interface
  (if (`self.CanTrigger`)
    (`PrimitiveComponent.SetRenderCustomDepth` (`self.SkeletalMesh`) true)))

(event `/Game/Trap/HighlightInterface.CancelHighlight`
  ;[0.0488 1 0] Hightlight interface
  (`PrimitiveComponent.SetRenderCustomDepth` (`self.SkeletalMesh`) false))

(event `self.Activate Zone.OnComponentBeginOverlap`
  (params (OverlappedComponent :type "PrimitiveComponent Object Reference") (OtherActor :type "Actor Object Reference") (OtherComp :type "PrimitiveComponent Object Reference") (OtherBodyIndex :type Integer) (bFromSweep :type Boolean) (SweepResult :type "HitResult Structure (by ref)"))
  ;[1 0.03408 0] Detect Animal
  (`/Engine/EditorBlueprintResources/ActorMacros.Switch Has Authority`
    (:`Authority`
      (cast `Animal` OtherActor)
      (if (`self.CanFire`)
        (set `self.CanFire` false)
        (`self.Fire` (`self.PlayerSpawned`))))))

(event `self.HandleFire`
  (params (Player :type "Pawn Object Reference"))
  ;[1 0.007073 0] Fire Event
  (bind _asspring_anim_bp (cast `/Game/Trap/Spring/Models/SpringAnim_BP` (`SkeletalMeshComponent.GetAnimInstance` (`self.SkeletalMesh`))))
  (set `/Game/Trap/Spring/Models/SpringAnim_BP.ShouldFire` true _asspring_anim_bp)
  (`AudioComponent.Play` (`self.FireSound`) 0.0)
  (`ActorComponent.Activate` (`self.FireParticle`) true)
  (bind _returnvalue (`PrimitiveComponent.CreateDynamicMaterialInstance` (`self.HintZone`) 0 "/Game/Trap/Materials/MI_ActivateZone.MI_ActivateZone" "None"))
  (`MaterialInstanceDynamic.SetScalarParameterValue` _returnvalue "OpacityMultipier" 0.0)
  (for _array_element (`PrimitiveComponent.GetOverlappingActors` (`self.Activate Zone`) "/Script/Guardian_TheTrap.Animal")
    (bind _asanimal (cast `Animal` _array_element))
    (if (`Animal.CanBeBounceOff` _asanimal)
      (bind _charactermovement (`Character.CharacterMovement` _asanimal))
      (`MovementComponent.StopMovementImmediately` _charactermovement)
      (`CharacterMovementComponent.AddImpulse` _charactermovement (* (`KismetMathLibrary.Normal` (- (`SceneComponent.K2_GetComponentLocation` (`MovementComponent.UpdatedPrimitive` _charactermovement)) (`self.K2_GetActorLocation`))) (`self.ImpulseLength`)) false)))
  (if (`self.CanRepeating`)
    (`KismetSystemLibrary.Delay` (`self.CD`))
    (bind _asspring_anim_bp_2 (cast `/Game/Trap/Spring/Models/SpringAnim_BP` (`SkeletalMeshComponent.GetAnimInstance` (`self.SkeletalMesh`))))
    (set `/Game/Trap/Spring/Models/SpringAnim_BP.ShouldFire` false _asspring_anim_bp_2)
    (set `self.CanFire` true)
    (bind _returnvalue_2 (`PrimitiveComponent.CreateDynamicMaterialInstance` (`self.HintZone`) 0 "/Game/Trap/Materials/MI_ActivateZone.MI_ActivateZone" "None"))
    (`MaterialInstanceDynamic.SetScalarParameterValue` _returnvalue_2 "OpacityMultipier" 1.0)))

(event `FadeInEffect`
  (params (Duration :type "Float (double-precision)"))
  ;[1 1 1] Fade In Effect
  (if (<= Duration 3.0)
    (bind _returnvalue (`PrimitiveComponent.CreateDynamicMaterialInstance` (`self.SkeletalMesh`) 0 "/Game/Trap/Materials/MI_Spring_0.MI_Spring_0" "None"))
    (`MaterialInstanceDynamic.SetScalarParameterValue` _returnvalue "MaskScale" Duration)
    (bind _returnvalue_2 (`PrimitiveComponent.CreateDynamicMaterialInstance` (`self.SkeletalMesh`) 1 "/Game/Trap/Materials/MI_Spring_1.MI_Spring_1" "None"))
    (`MaterialInstanceDynamic.SetScalarParameterValue` _returnvalue_2 "MaskScale" Duration)
    (bind _returnvalue_3 (`PrimitiveComponent.CreateDynamicMaterialInstance` (`self.SkeletalMesh`) 2 "/Game/Trap/Materials/MI_Spring_2.MI_Spring_2" "None"))
    (`MaterialInstanceDynamic.SetScalarParameterValue` _returnvalue_3 "MaskScale" Duration)
    (bind _returnvalue_4 (`PrimitiveComponent.CreateDynamicMaterialInstance` (`self.SkeletalMesh`) 3 "/Game/Trap/Materials/MI_Spring_3.MI_Spring_3" "None"))
    (`MaterialInstanceDynamic.SetScalarParameterValue` _returnvalue_4 "MaskScale" Duration)))

(fn `UserConstructionScript`)