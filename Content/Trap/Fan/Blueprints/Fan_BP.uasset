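; Fan trap that VR players can pick up and drop, halving the speed of Animals inside its ActivateZone.
; Tick sends its transform through a server update, calls Fire on authority until the looping fan animation starts, and keeps it grabbable.
; A fade-in drives MaskScale on three dynamic materials for the first seconds.
; Highlighting uses custom depth; the LevelManager-based grab check is disconnected.
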(event `self.ReceiveBeginPlay`
  ;[0 0.8853 1] Main BeginPlay
  (bind _asvrpawn (cast `/Game/Player/VRPawn` (`self.GetOwner`)))
  (set `self.PlayerSpawned` _asvrpawn)
  (`self.SetOwner` null))

(event `self.ReceiveTick`
  (params (DeltaSeconds :type "Float (single-precision)"))
  ;[1 0.79 0] Main Tick
  (`|ExecutionSequence`
    (:`then_0`
      ;;[1 1 1] Sync Position and Rotation
      (`self.UpdatePosAndRot_Server` (`self.K2_GetActorLocation`) (`self.K2_GetActorRotation`)))
    (:`then_1`
      ;;[1 1 1] Open When Game Start
      (if (not (`self.Is Opening`))
        (`/Engine/EditorBlueprintResources/ActorMacros.Switch Has Authority`
          (:`Authority`
            (`self.Fire` (`self.PlayerSpawned`))))))
    (:`then_2`
      ;;[1 1 1] Fade In Effect
      (bind _output_get (set `self.LocalFadeInDuration` (+ (`GameplayStatics.GetWorldDeltaSeconds`) (`self.LocalFadeInDuration`))))
      (`self.FadeInEffect` _output_get))
    (:`then_3`
      (set `self.CanGrab` true))))

(event `UpdatePosAndRot_Server`
  (params (NewLocation :type "Vector Structure") (NewRotation :type "Rotator Structure"))
  ;[1 0.79 0] Main Tick
  ;;[1 1 1] Sync Position and Rotation
  (`self.K2_SetActorLocationAndRotation` NewLocation NewRotation))

(event `/Game/VirtualRealityBP/Blueprints/PickupActorInterface.Pickup`
  (params (AttachTo :type "SceneComponent Object Reference"))
  ;[1 0.3914 0] PickUp interface
  (if (`self.CanGrab`)
    (`PrimitiveComponent.SetSimulatePhysics` (`self.SkeletalMesh`) false)
    (`SceneComponent.K2_AttachToComponent` (`self.K2_GetRootComponent`) AttachTo "None" "KeepWorld" "KeepWorld" "KeepWorld" false)))

(event `/Game/VirtualRealityBP/Blueprints/PickupActorInterface.Drop`
  ;[1 0.3914 0] PickUp interface
  (`PrimitiveComponent.SetSimulatePhysics` (`self.SkeletalMesh`) true)
  (`self.K2_DetachFromActor` "KeepWorld" "KeepWorld" "KeepWorld"))

(event `/Game/Trap/HighlightInterface.Highlight`
  ;[0 1 0.157] Highlight
  (`PrimitiveComponent.SetRenderCustomDepth` (`self.SkeletalMesh`) true))

(event `/Game/Trap/HighlightInterface.CancelHighlight`
  ;[0 1 0.157] Highlight
  (`PrimitiveComponent.SetRenderCustomDepth` (`self.SkeletalMesh`) false))

(event `self.HandleFire`
  (params (Player :type "Pawn Object Reference"))
  ;[1 0 0.005218] Fire Event
  (if (`self.CanFire`)
    (set `self.Is Opening` true)
    (set `self.CanFire` false)
    (`SkeletalMeshComponent.PlayAnimation` (`self.SkeletalMesh`) "/Game/Trap/Fan/Models/test/fan_new_ani_Anim.fan_new_ani_Anim" true)))

(event `FadeInEffect`
  (params (Duration :type "Float (double-precision)"))
  ;[1 1 1] Fade In Effect
  (if (<= Duration 3.0)
    (bind _returnvalue (`PrimitiveComponent.CreateDynamicMaterialInstance` (`self.SkeletalMesh`) 0 "/Game/Trap/Materials/MI_FanNew_0.MI_FanNew_0" "None"))
    (`MaterialInstanceDynamic.SetScalarParameterValue` _returnvalue "MaskScale" Duration)
    (bind _returnvalue_2 (`PrimitiveComponent.CreateDynamicMaterialInstance` (`self.SkeletalMesh`) 1 "/Game/Trap/Materials/MI_FanNew_1.MI_FanNew_1" "None"))
    (`MaterialInstanceDynamic.SetScalarParameterValue` _returnvalue_2 "MaskScale" Duration)
    (bind _returnvalue_3 (`PrimitiveComponent.CreateDynamicMaterialInstance` (`self.SkeletalMesh`) 2 "/Game/Trap/Materials/MI_FanNew_2.MI_FanNew_2" "None"))
    (`MaterialInstanceDynamic.SetScalarParameterValue` _returnvalue_3 "MaskScale" Duration)))

(event `self.ActivateZone.OnComponentBeginOverlap`
  (params (OverlappedComponent :type "PrimitiveComponent Object Reference") (OtherActor :type "Actor Object Reference") (OtherComp :type "PrimitiveComponent Object Reference") (OtherBodyIndex :type Integer) (bFromSweep :type Boolean) (SweepResult :type "HitResult Structure (by ref)"))
  (bind _asanimal (cast `Animal` OtherActor))
  (set `Animal.Speed` (/ (`Animal.MaxSpeed` _asanimal) 2.0) _asanimal))

(event `self.ActivateZone.OnComponentEndOverlap`
  (params (OverlappedComponent :type "PrimitiveComponent Object Reference") (OtherActor :type "Actor Object Reference") (OtherComp :type "PrimitiveComponent Object Reference") (OtherBodyIndex :type Integer))
  (bind _asanimal (cast `Animal` OtherActor))
  (set `Animal.Speed` (`Animal.MaxSpeed` _asanimal) _asanimal))

(fn `UserConstructionScript`)