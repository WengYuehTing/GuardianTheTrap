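; Game instance that handles LAN multiplayer sessions and saving of VR player cosmetics.
; Host creates a two-slot LAN session and opens Hall as a listen server, Search tries joining every found session, and PlayGame joins the first found or hosts if none exist.
; Save loads or creates a SaveGame_BP in the SaveTest slot, using Id as user index, and stores the VRPawn's head mesh and both hand colors.
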(event `Host`
  (`CreateSessionCallbackProxy.CreateSession` (`GameplayStatics.GetPlayerController` 0) 2 true
    (:`OnSuccess`
      (`GameplayStatics.OpenLevel` "Hall" true "listen"))
    (:`OnFailure`
      (`KismetSystemLibrary.PrintString` "Can't create session"))))

(event `Search`
  (bind _returnvalue (`GameplayStatics.GetPlayerController` 0))
  (bind _results (`FindSessionsCallbackProxy.FindSessions` _returnvalue 5 true)
    (:`OnSuccess`
      (for _array_element _results
        (`JoinSessionCallbackProxy.JoinSession` _returnvalue _array_element
          (:`OnSuccess`
            (`KismetSystemLibrary.PrintString` "join success"))
          (:`OnFailure`
            (`KismetSystemLibrary.PrintString` "Can't join session")))))
    (:`OnFailure`
      (`KismetSystemLibrary.PrintString` "Can't find session"))))

(event `Save`
  (params (id :type Integer))
  (bind _returnvalue (`GameplayStatics.LoadGameFromSlot` "SaveTest" id))
  (bind _assave_game_bp (cast `/Game/Player/PersonalSettings/SaveGame_BP` _returnvalue)
    (:`then`
      (bind _asvrpawn (cast `/Game/Player/VRPawn` (`GameplayStatics.GetPlayerPawn` 0)))
      (set `/Game/Player/PersonalSettings/SaveGame_BP.HeadPlayerChoose` (`StaticMeshComponent.StaticMesh` (`/Game/Player/VRPawn.Head` _asvrpawn)) _assave_game_bp)
      (set `/Game/Player/PersonalSettings/SaveGame_BP.RightHandColor` (`/Game/Player/VRPawn.LocalRightHandColor` _asvrpawn) _assave_game_bp)
      (set `/Game/Player/PersonalSettings/SaveGame_BP.LeftHandColor` (`/Game/Player/VRPawn.LocalLeftHandColor` _asvrpawn) _assave_game_bp)
      (`GameplayStatics.SaveGameToSlot` _assave_game_bp "SaveTest" id))
    (:`CastFailed`
      (bind _returnvalue_2 (`GameplayStatics.CreateSaveGameObject` "/Game/Player/PersonalSettings/SaveGame_BP.SaveGame_BP_C"))
      (bind _asvrpawn_2 (cast `/Game/Player/VRPawn` (`GameplayStatics.GetPlayerPawn` 0)))
      (set `/Game/Player/PersonalSettings/SaveGame_BP.HeadPlayerChoose` (`StaticMeshComponent.StaticMesh` (`/Game/Player/VRPawn.Head` _asvrpawn_2)) _returnvalue_2)
      (set `/Game/Player/PersonalSettings/SaveGame_BP.RightHandColor` (`/Game/Player/VRPawn.LocalRightHandColor` _asvrpawn_2) _returnvalue_2)
      (set `/Game/Player/PersonalSettings/SaveGame_BP.LeftHandColor` (`/Game/Player/VRPawn.LocalLeftHandColor` _asvrpawn_2) _returnvalue_2)
      (`GameplayStatics.SaveGameToSlot` _returnvalue_2 "SaveTest" id))))

(event `PlayGame`
  (bind _results (`FindSessionsCallbackProxy.FindSessions` (`GameplayStatics.GetPlayerController` 0) 5 true)
    (:`OnSuccess`
      (if (> (`KismetArrayLibrary.Array_Length` _results) 0)
        (`KismetSystemLibrary.PrintString` "Find")
        (`JoinSessionCallbackProxy.JoinSession` (`GameplayStatics.GetPlayerController` 0) (`|GetArrayItem` _results))
        (else
          (`KismetSystemLibrary.PrintString` "Not Found")
          (`self.Host`))))))