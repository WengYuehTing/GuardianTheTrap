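; Teleport door in the teaching content that spawns timed waves of pigs and rabbits.
; StartCountDown loads the next wave on the server; Tick updates the countdown text and multicasts a sound timed to end near zero.
; At zero, the server sets the LevelManager state and spawns animals through a delayed self-calling loop.
; Highlight enables custom depth on the body and shows a trace to the Barn door.
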(event `self.ReceiveBeginPlay`
  (`self.SetupSpawnLocation`)
  (`self.SetActorHiddenInGame` false)
  (bind _outactors (`GameplayStatics.GetAllActorsOfClass` "/Game/Barn/Blueprints/Barn_BP.Barn_BP_C"))
  (set `self.Barn` (`|GetArrayItem` _outactors))
  (set `self.TotalWaveAmounts` (`KismetArrayLibrary.Array_Length` (`self.AnimalsInfo`))))

(event `self.ReceiveTick`
  (params (DeltaSeconds :type "Float (single-precision)"))
  (bind _audio (`self.Audio`))
  (`|ExecutionSequence`
    (:`then_0`
      (if (`self.IsStartCountDown`)
        (if (> (`self.CountDownSecond`) 0.0)
          (bind _output_get (set `self.CountDownSecond` (- (`self.CountDownSecond`) (`GameplayStatics.GetWorldDeltaSeconds`))))
          (`|ExecutionSequence`
            (:`then_0`
              (`TextRenderComponent.K2_SetText` (`self.TextRender`) (`KismetTextLibrary.Conv_IntToText` (`KismetMathLibrary.Round` _output_get))))
            (:`then_1`
              (if (and (<= _output_get (`SoundBase.Duration` (`AudioComponent.Sound` _audio))) (not (`AudioComponent.IsPlaying` _audio)) (not (`self.IsPlayAudio`)))
                (set `self.IsPlayAudio` true)
                (`self.Multicast PlaySound`))))
          (else
            (set `self.IsStartCountDown` false)
            (`self.SpawnAnimals`)))))))

(event `SetupSpawnLocation`
  (bind (_returnvalue_x _returnvalue_y _returnvalue_z) (`KismetMathLibrary.BreakVector` (`self.K2_GetActorLocation`)))
  (set `self.SpawnLocation` (`KismetMathLibrary.MakeVector` (+ _returnvalue_x 50.0) _returnvalue_y _returnvalue_z)))

(event `StartCountDown`
  (bind _output (`|GetArrayItem` (`self.AnimalsInfo`) (`self.WaveIndex`)))
  ;[1 1 1] Count Down
  (`/Engine/EditorBlueprintResources/ActorMacros.Switch Has Authority`
    (:`Authority`
      (if (`self.IsStartCountDown`)
        _
        (elif (not (>= (`self.WaveIndex`) (`self.TotalWaveAmounts`)))
          (set `self.IsStartCountDown` true)
          (set `self.IsPlayAudio` false)
          (set `self.LocalAnimalWave` _output)
          (set `self.CountDownSecond` (`.LocalWaveDelay` (break `AnimalsWave` _output)))
          (set `self.WaveIndex` (+ (`self.WaveIndex`) 1))
          (else
            (set `self.IsFinishSpawning` true)))))))

(event `/Game/Trap/HighlightInterface.Highlight`
  (bind _body (`self.Body`))
  ;[1 1 1] Highlight
  (`PrimitiveComponent.SetRenderCustomDepth` (`self.Body`) true)
  (`PrimitiveComponent.K2_LineTraceComponent` _body (`SceneComponent.K2_GetComponentLocation` _body) (`SceneComponent.K2_GetComponentLocation` (`/Game/Barn/Blueprints/Barn_BP.Door` (`self.Barn`))) true true))

(event `/Game/Trap/HighlightInterface.CancelHighlight`
  ;[1 1 1] Highlight
  (`PrimitiveComponent.SetRenderCustomDepth` (`self.Body`) false))

(event `Multicast PlaySound`
  ;[1 1 1] Multicast PlaySound
  (`AudioComponent.Play` (`self.Audio`) 0.0))

(event `Looping`
  (bind (_localwavedelay _spawnedrate _animalsorder) (break `AnimalsWave` (`self.LocalAnimalWave`)))
  (bind _returnvalue (`KismetMathLibrary.Conv_VectorToTransform` (`self.SpawnLocation`)))
  ;[1 1 1] Spawn Animal
  (if (> (`KismetArrayLibrary.Array_Length` _animalsorder) (`self.Index`)) :!label _label
    (switch `EAnimals` (`|GetArrayItem` _animalsorder (`self.Index`))
      (:`Pig`
        (`|SpawnActorFromClass` "/Game/Enemy/Pig/Blueprints/Pig_BP.Pig_BP_C" _returnvalue "AlwaysSpawn" "OverrideRootScale" null null))
      (:`Rabbit`
        (`|SpawnActorFromClass` "/Game/Enemy/Rabbit/Blueprints/Rabbit_BP.Rabbit_BP_C" _returnvalue "AlwaysSpawn" "OverrideRootScale" null null)))
    (set `self.Index` (+ (`self.Index`) 1))
    (`KismetSystemLibrary.Delay` (`self.LocalWaveDelay`))
    (`self.Looping`)
    (else
      (set `self.IsStartSpawning` false))))

(event `SpawnAnimals`
  ;[1 1 1] Spawn Animal
  (`/Engine/EditorBlueprintResources/ActorMacros.Switch Has Authority`
    (:`Authority`
      (bind _outactors (`GameplayStatics.GetAllActorsOfClass` "/Game/LevelManager/LevelManager_BP.LevelManager_BP_C"))
      (set `/Game/LevelManager/LevelManager_BP.State` "NewEnumerator4" (`|GetArrayItem` _outactors))
      (if (not (`self.IsStartSpawning`))
        (set `self.IsStartSpawning` true)
        (set `self.Index` 0)
        (set `self.LocalWaveDelay` (`.SpawnedRate` (break `AnimalsWave` (`self.LocalAnimalWave`))))
        (goto _label)))))

(fn `UserConstructionScript`)