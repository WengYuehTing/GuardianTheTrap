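; Grabbable VR bow trap that automatically shoots arrows at living Animals in its line of fire, with three upgrade levels.
; After a timed fade-in, Tick traces along the arrow and launches it as a physics impulse, spawning a replacement after a cooldown if repeating is enabled.
; Arrow hits damage animals and can knock them back.
; Level, initially read from TrapManager_BP, sets mesh, damage and particles.
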(event `self.ReceiveBeginPlay`
  ;[0 0.8608 1] Main BeginPlay
  (`|ExecutionSequence`
    (:`then_0`
      (bind _asvrpawn (cast `/Game/Player/VRPawn` (`self.GetOwner`)))
      (set `self.PlayerSpawned` _asvrpawn)
      (`self.SetOwner` null))
    (:`then_1`
      (`self.UpdateProperty`))))

(event `UpdatePosAndRot_Server`
  (params (NewLocation :type "Vector Structure") (NewRotation :type "Rotator Structure"))
  ;[1 0.901 0] Main Tick
  ;;[1 1 1] Sync Position and Rotation
  (`self.K2_SetActorLocationAndRotation` NewLocation NewRotation))

(event `self.ReceiveTick`
  (params (DeltaSeconds :type "Float (single-precision)"))
  (bind _arrowref (`self.ArrowRef`))
  (bind _returnvalue (`SceneComponent.K2_GetComponentLocation` _arrowref))
  ;[1 0.901 0] Main Tick
  (`|ExecutionSequence`
    (:`then_0`
      ;;[1 1 1] Sync Position and Rotation
      (`self.UpdatePosAndRot_Server` (`self.K2_GetActorLocation`) (`self.K2_GetActorRotation`)))
    (:`then_1`
      ;;[1 1 1] Fade In
      (bind _output_get (set `self.LocalDuration` (+ (`GameplayStatics.GetWorldDeltaSeconds`) (`self.LocalDuration`))))
      (`self.FadeInEffect` _output_get))
    (:`then_2`
      ;;[1 1 1] Keep Arrow Ref
      (for _array_element (`SceneComponent.GetChildrenComponents` (`self.SkeletalMesh`) false)
        (bind _asstatic_mesh_component (cast `StaticMeshComponent` _array_element))
        (set `self.ArrowRef` _asstatic_mesh_component)
        (`self.Multicast BindEvent`)))
    (:`then_3`
      ;;[1 1 1] Line Tracing Animal
      (`/Engine/EditorBlueprintResources/StandardMacros.IsValid` (`self.ArrowRef`)
        (:`Is Valid`
          (if (and (`self.FinishFadeIn`) (`self.CanFire`))
            (bind _outhit (`KismetSystemLibrary.LineTraceSingleByProfile` :`Start` _returnvalue :`End` (+ _returnvalue (* (`SceneComponent.GetRightVector` _arrowref) (`self.DetectAnimalDistance`))) :`DrawDebugType` "ForOneFrame"))
            (bind _asanimal (cast `Animal` (`.HitActor` (`GameplayStatics.BreakHitResult` _outhit))))
            (if (> (`Animal.HP` _asanimal) 0.5)
              (if (`self.CanFire`)
                (set `self.CanFire` false)
                (`self.BowFireLocalEvent`)))))))
    (:`then_4`
      (set `self.CanGrab` true))))

(event `/Game/VirtualRealityBP/Blueprints/PickupActorInterface.Pickup`
  (params (AttachTo :type "SceneComponent Object Reference"))
  ;[1 0.3928 0] PickUp interface
  (if (`self.CanGrab`)
    (`PrimitiveComponent.SetSimulatePhysics` (`self.SkeletalMesh`) false)
    (`SceneComponent.K2_AttachToComponent` (`self.K2_GetRootComponent`) AttachTo "None" "KeepWorld" "KeepWorld" "KeepWorld" false)))

(event `/Game/VirtualRealityBP/Blueprints/PickupActorInterface.Drop`
  ;[1 0.3928 0] PickUp interface
  (`PrimitiveComponent.SetSimulatePhysics` (`self.SkeletalMesh`) true)
  (`self.K2_DetachFromActor` "KeepWorld" "KeepWorld" "KeepWorld"))

(event `/Game/Trap/HighlightInterface.Highlight`
  ;[0 1 0.3268] Highlight
  (`PrimitiveComponent.SetRenderCustomDepth` (`self.SkeletalMesh`) true))

(event `/Game/Trap/HighlightInterface.CancelHighlight`
  ;[0 1 0.3268] Highlight
  (`PrimitiveComponent.SetRenderCustomDepth` (`self.SkeletalMesh`) false))

(event `BowFireLocalEvent`
  (bind _skeletalmesh (`self.SkeletalMesh`))
  (bind _arrowref (`self.ArrowRef`))
  (bind _returnvalue (`SceneComponent.K2_GetComponentToWorld` (`self.ArrowPosition`)))
  ;[1 0 0] Fire Event
  (switch `TrapLevel` (`self.Level`)
    (:`Level_1`
      (`SkeletalMeshComponent.PlayAnimation` _skeletalmesh "/Game/Trap/Bow/Models/Bow_Anim.Bow_Anim" false))
    (:`Level_2`
      (`SkeletalMeshComponent.PlayAnimation` _skeletalmesh "/Game/Trap/Bow/Models/test/Bow_lv2__2__Anim.Bow_lv2__2__Anim" false))
    (:`Level_3`
      (`SkeletalMeshComponent.PlayAnimation` _skeletalmesh "/Game/Trap/Bow/Models/test/cannon_lv3_ani_Anim.cannon_lv3_ani_Anim" false)))
  (`AudioComponent.Play` (`self.FireSound`) 0.0)
  (`SceneComponent.K2_DetachFromComponent` _arrowref "KeepWorld" "KeepWorld" "KeepWorld" true)
  (`PrimitiveComponent.SetSimulatePhysics` _arrowref true)
  (`PrimitiveComponent.SetCollisionEnabled` _arrowref "PhysicsOnly")
  (`PrimitiveComponent.SetCollisionResponseToChannel` _arrowref "ECC_PhysicsBody" "ECR_Ignore")
  (`PrimitiveComponent.AddImpulse` _arrowref (* (`SceneComponent.GetRightVector` _arrowref) (`self.ArrowSpeed`)) "None" false)
  (set `self.IsArrowShooting` true)
  (if (`self.CanRepeating`)
    (`KismetSystemLibrary.Delay` (`self.CD`))
    (set `self.CanFire` true)
    (set `self.IsArrowShooting` false)
    (bind _returnvalue_2 (`AddComponent|NODE_AddStaticMeshComponent-0` :`bManualAttachment` true :`RelativeTransform` _returnvalue))
    (bind _returnvalue_3 (`AddComponent|NODE_AddParticleSystemComponent-0` :`bManualAttachment` true :`RelativeTransform` _returnvalue))
    (`ParticleSystemComponent.SetTemplate` _returnvalue_3 "/Game/Trap/Bow/P_ArrowDrag.P_ArrowDrag")
    (`SceneComponent.K2_AttachToComponent` _returnvalue_3 _returnvalue_2 "None" "KeepWorld" "KeepWorld" "KeepWorld" true)
    (`PrimitiveComponent.SetNotifyRigidBodyCollision` _returnvalue_2 true)
    (`PrimitiveComponent.SetEnableGravity` _returnvalue_2 false)
    (`PrimitiveComponent.SetCollisionResponseToAllChannels` _returnvalue_2 "ECR_Ignore")
    (`PrimitiveComponent.SetCollisionResponseToChannel` _returnvalue_2 "ECC_Pawn" "ECR_Block")
    (`StaticMeshComponent.SetStaticMesh` _returnvalue_2 "/Game/Trap/Bow/Models/arrow.arrow")
    (`SceneComponent.K2_SetWorldTransform` _returnvalue_2 (`SceneComponent.K2_GetComponentToWorld` (`self.ArrowPosition`)) false false)
    (`SceneComponent.K2_AttachToComponent` _returnvalue_2 (`self.SkeletalMesh`) "None" "KeepWorld" "KeepWorld" "KeepWorld" true)))

(event `Multicast BindEvent`
  ;[1 1 1] Arrow Hit Something
  (add `PrimitiveComponent.OnComponentHit` (`self.ArrowRef`) (delegate `ArrowHitEvent`)))

(event `ArrowHitEvent`
  (params (HitComponent :type "PrimitiveComponent Object Reference") (OtherActor :type "Actor Object Reference") (OtherComp :type "PrimitiveComponent Object Reference") (NormalImpulse :type "Vector Structure") (Hit :type "HitResult Structure (by ref)"))
  (bind (_arrowrot_roll _arrowrot_pitch _arrowrot_yaw) (`KismetMathLibrary.BreakRotator` (`self.ArrowRot`)))
  ;[1 1 1] Arrow Hit Something
  (bind _asanimal (cast `Animal` OtherActor)
    (:`then`
      (if (`self.IsArrowShooting`)
        (set `self.ArrowPosWhenDestroy` (`SceneComponent.K2_GetComponentLocation` (`self.ArrowRef`)))
        (set `self.ArrowRot` (`SceneComponent.K2_GetComponentRotation` (`self.ArrowRef`)))
        (`ActorComponent.K2_DestroyComponent` (`self.ArrowRef`))
        (`GameplayStatics.ApplyDamage` _asanimal (`self.Damage`) null (`self.PlayerSpawned`) "/Game/Enemy/DamageType/NormalDamage_BP.NormalDamage_BP_C")
        (if (`Animal.CanBeBounceOff` _asanimal)
          (bind _charactermovement (`Character.CharacterMovement` _asanimal))
          (`MovementComponent.StopMovementImmediately` _charactermovement)
          (`CharacterMovementComponent.AddImpulse` _charactermovement (* (`KismetMathLibrary.Normal` (- (`SceneComponent.K2_GetComponentLocation` (`MovementComponent.UpdatedPrimitive` _charactermovement)) (`self.ArrowPosWhenDestroy`))) (`self.ArrowImpulse`)) false)
          (bind _asvrpawn (cast `/Game/Player/VRPawn` (`GameplayStatics.GetPlayerPawn` 0)))
          (`/Game/Player/VRPawn.Server SpawnEmitter` _asvrpawn "/Game/Trap/Bow/ArrowHit/P_ArrowHit.P_ArrowHit" (`.Location` (`GameplayStatics.BreakHitResult` Hit)) (`KismetMathLibrary.MakeRotator` 0.0 0.0 (+ _arrowrot_yaw 90.0)) (2.5 2.5 2.5) true))))
    (:`CastFailed`
      (`PrimitiveComponent.SetSimulatePhysics` (`self.ArrowRef`) false)
      (set `self.IsArrowShooting` false))))

(event `self.HandleLevelUp`
  (bind _level (`self.Level`))
  (bind _skeletalmesh (`self.SkeletalMesh`))
  (bind _skeletalmesh_2 (`self.SkeletalMesh`))
  ;[1 0.7878 0] Level Up
  (if (not (`|EnumEquality` _level (`self.MaxLevel`)))
    (switch `TrapLevel` _level
      (:`Level_1`
        (set `self.Level` "Level_2")
        (`SkinnedMeshComponent.SetSkinnedAssetAndUpdate` _skeletalmesh "/Game/Trap/Bow/Models/test/Bow_lv2__2_.Bow_lv2__2_" true)
        (`PrimitiveComponent.SetMaterial` _skeletalmesh 0 "/Game/Trap/Materials/MI_cannonLv2_0.MI_cannonLv2_0")
        (`PrimitiveComponent.SetMaterial` _skeletalmesh 1 "/Game/Trap/Materials/MI_cannonLv2_1.MI_cannonLv2_1")
        (`PrimitiveComponent.SetMaterial` _skeletalmesh 2 "/Game/Trap/Materials/MI_cannonLv2_2.MI_cannonLv2_2")
        (set `self.Damage` 100.0)
        (`ActorComponent.Activate` (`self.LevelUp`) true)
        (`ActorComponent.Activate` (`self.Level2Particle`) false))
      (:`Level_2`
        (set `self.Level` "Level_3")
        (`SkinnedMeshComponent.SetSkinnedAssetAndUpdate` _skeletalmesh_2 "/Game/Trap/Bow/Models/test/cannon_lv3_ani.cannon_lv3_ani" true)
        (`PrimitiveComponent.SetMaterial` _skeletalmesh_2 0 "/Game/Trap/Materials/MI_cannonLv3_0.MI_cannonLv3_0")
        (`PrimitiveComponent.SetMaterial` _skeletalmesh_2 1 "/Game/Trap/Materials/MI_cannonLv3_1.MI_cannonLv3_1")
        (`PrimitiveComponent.SetMaterial` _skeletalmesh_2 2 "/Game/Trap/Materials/MI_cannonLv3_2.MI_cannonLv3_2")
        (set `self.Damage` 150.0)
        (`ActorComponent.Activate` (`self.LevelUp`) true)
        (`ActorComponent.Activate` (`self.Level3Particle`) false)
        (`ActorComponent.Deactivate` (`self.Level2Particle`))))))

(event `UpdateProperty`
  ;[1 1 1] Update Property When beginplay
  (bind _outactors (`GameplayStatics.GetAllActorsOfClass` "/Game/LevelManager/TrapManager_BP.TrapManager_BP_C"))
  (switch `TrapLevel` (`/Game/LevelManager/TrapManager_BP.BowLevel` (`|GetArrayItem` _outactors))
    (:`Level_2`
      (set `self.Level` "Level_2")
      (`SkinnedMeshComponent.SetSkinnedAssetAndUpdate` (`self.SkeletalMesh`) "/Game/Trap/Bow/Models/test/Bow_lv2__2_.Bow_lv2__2_" true)
      (set `self.Damage` 100.0)
      (`KismetSystemLibrary.Delay` 0.2)
      (`ActorComponent.Activate` (`self.Level2Particle`) false))
    (:`Level_3`
      (set `self.Level` "Level_3")
      (`SkinnedMeshComponent.SetSkinnedAssetAndUpdate` (`self.SkeletalMesh`) "/Game/Trap/Bow/Models/test/cannon_lv3_ani.cannon_lv3_ani" true)
      (set `self.Damage` 150.0)
      (`KismetSystemLibrary.Delay` 0.2)
      (`ActorComponent.Activate` (`self.Level3Particle`) false)
      (`ActorComponent.Deactivate` (`self.Level2Particle`)))))

(event `FadeInEffect`
  (params (Duration :type "Float (double-precision)"))
  (bind _arrowref (`self.ArrowRef`))
  ;[1 1 1] Fade In Effect
  (if (<= Duration 3.0)
    (switch `TrapLevel` (`self.Level`)
      (:`Level_1`
        (bind _returnvalue (`PrimitiveComponent.CreateDynamicMaterialInstance` (`self.SkeletalMesh`) 0 "/Game/Trap/Materials/MI_cannon_0.MI_cannon_0" "None"))
        (`MaterialInstanceDynamic.SetScalarParameterValue` _returnvalue "MaskScale" Duration)
        (bind _returnvalue_2 (`PrimitiveComponent.CreateDynamicMaterialInstance` (`self.SkeletalMesh`) 1 "/Game/Trap/Materials/MI_cannon_1.MI_cannon_1" "None"))
        (`MaterialInstanceDynamic.SetScalarParameterValue` _returnvalue_2 "MaskScale" Duration)
        (bind _returnvalue_3 (`PrimitiveComponent.CreateDynamicMaterialInstance` (`self.SkeletalMesh`) 2 "/Game/Trap/Materials/MI_cannon_2.MI_cannon_2" "None"))
        (`MaterialInstanceDynamic.SetScalarParameterValue` _returnvalue_3 "MaskScale" Duration)))
    (else
      (set `self.FinishFadeIn` true)
      (`/Engine/EditorBlueprintResources/StandardMacros.IsValid` _arrowref
        (:`Is Valid`
          (`SceneComponent.SetVisibility` _arrowref true false))))))

(fn `UserConstructionScript`)