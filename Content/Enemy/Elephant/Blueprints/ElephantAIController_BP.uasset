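; AI controller for the Elephant enemy that targets the Barn and moves to an elephant socket.
; After a short delay it caches the pawn, picks the first Barn and ElephantSocket, and starts the behavior tree and blackboard.
; Each tick it updates the pawn's speed, grounded state, socket distance and multicast arrival status, releasing the socket if no Barn remains.
; A timer flags it stuck after idling near the Barn unarrived.
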(event `self.ReceiveBeginPlay`
  (`KismetSystemLibrary.Delay` 0.2)
  ;[1 1 1] Init : Proprecessing property
  (`self.SetControlledElephantRef`)
  (`self.FindBarn`)
  (`self.SelectBarnSocket`)
  (bind _returnvalue (`self.RunBehaviorTree` "/Game/Enemy/Elephant/AI/Elephant_BT.Elephant_BT"))
  (if _returnvalue
    (`self.UseBlackboard` "/Game/Enemy/Elephant/AI/Elephant_BD.Elephant_BD")
    (set `Animal.SelfAwareness` true (`self.ControlledElephant`))
    (set `self.InitFinish` true)))

(event `self.ReceiveTick`
  (params (DeltaSeconds :type "Float (single-precision)"))
  (if (`self.InitFinish`)
    ;[1 1 1] RunTime: Update
    (`self.UpdateSpeed`)
    (`self.CheckOnGround`)
    (`self.UpdateBarn`)
    (`self.UpdateArrivalStatus`)
    (`/Engine/EditorBlueprintResources/StandardMacros.IsValid` (`Animal.Barn` (`self.ControlledElephant`))
      (:`Is Valid`
        (`self.CalculateDistance`)
        (`self.CheckForStucking`)))))

(event `SetControlledElephantRef`
  ;[1 1 1] Get Controlled Pig References
  (bind _aselephant_bp (cast `/Game/Enemy/Elephant/Blueprints/Elephant_BP` (`self.K2_GetPawn`)))
  (set `self.ControlledElephant` _aselephant_bp))

(event `FIndBarn`
  ;[1 1 1] Find Barn Method, Set to Controlled Pig Target, And Set Distance Between Pig & Barn.
  (bind _outactors (`GameplayStatics.GetAllActorsOfClass` "/Game/Barn/Blueprints/Barn_BP.Barn_BP_C"))
  (set `Animal.Barn` (`|GetArrayItem` _outactors) (`self.ControlledElephant`)))

(event `InitHealthBar`
  (bind _controlledelephant (`self.ControlledElephant`))
  ;[1 1 1] Init Health Bar
  (bind _asw_animal_health_bar (cast `/Game/Enemy/Widgets/W_AnimalHealthBar` (`WidgetComponent.GetUserWidgetObject` (`/Game/Enemy/Elephant/Blueprints/Elephant_BP.HealthBar` _controlledelephant))))
  (set `/Game/Enemy/Widgets/W_AnimalHealthBar.Animal` _controlledelephant _asw_animal_health_bar))

(event `SelectBarnSocket`
  (bind _controlledelephant (`self.ControlledElephant`))
  ;[1 1 1] Select Barn Socket To Move
  (`/Engine/EditorBlueprintResources/StandardMacros.IsValid` (`Animal.Barn` _controlledelephant)
    (:`Is Valid`
      (bind _outactors (`GameplayStatics.GetAllActorsOfClass` "/Game/Barn/Blueprints/ElephantSocket_BP.ElephantSocket_BP_C"))
      (set `Animal.SelectedSocket` (`|GetArrayItem` _outactors) (`self.ControlledElephant`)))
    (:`Is Not Valid`
      (set `Animal.SelectedSocket` null _controlledelephant))))

(event `UpdateSpeed`
  (bind _controlledelephant (`self.ControlledElephant`))
  ;[1 1 1] Update Speed Method
  (`/Game/Enemy/Elephant/Blueprints/Elephant_BP.SetSpeed` _controlledelephant (`Animal.Speed` _controlledelephant)))

(event `CheckOnGround`
  (bind _controlledelephant (`self.ControlledElephant`))
  ;[1 1 1] Check Pig is on ground on not
  (set `Animal.IsOnGround` (not (`NavMovementComponent.IsFalling` (`Character.CharacterMovement` _controlledelephant))) _controlledelephant))

(event `UpdateBarn`
  (bind _controlledelephant (`self.ControlledElephant`))
  ;[1 1 1] Update Barn Info
  (bind _outactors (`GameplayStatics.GetAllActorsOfClass` "/Game/Barn/Blueprints/Barn_BP.Barn_BP_C"))
  (if (== (`KismetArrayLibrary.Array_Length` _outactors) 0)
    (set `Animal.Barn` null _controlledelephant)
    (`/Game/Enemy/Pig/Blueprints/Pig_BP.ReleaseSocket` _controlledelephant)))

(event `CalculateDistance`
  (bind _controlledelephant (`self.ControlledElephant`))
  ;[1 1 1] Calculate Pig & Barn Distance
  (`/Engine/EditorBlueprintResources/StandardMacros.IsValid` (`Animal.SelectedSocket` _controlledelephant)
    (:`Is Valid`
      (set `Animal.DistanceToSocket` (`self.GetHorizontalDistanceTo` _controlledelephant (`Animal.SelectedSocket` _controlledelephant)) (`self.ControlledElephant`)))
    (:`Is Not Valid`
      (set `Animal.DistanceToSocket` 10000.0 _controlledelephant))))

(event `UpdateArrivalStatus`
  (bind _controlledelephant (`self.ControlledElephant`))
  ;[1 1 1] Update Arrival Status Method, Check Pig Is Arriving At Target Or Not.
  (if (and (<= (`KismetMathLibrary.VSize` (`self.GetVelocity` (`self.ControlledElephant`))) 10.0) (<= (`Animal.DistanceToSocket` _controlledelephant) (`Animal.MinArriveDistance` _controlledelephant)))
    (`/Game/Enemy/Elephant/Blueprints/Elephant_BP.Multicast UpdateArriveStatus` _controlledelephant true)
    (else
      (`/Game/Enemy/Elephant/Blueprints/Elephant_BP.Multicast UpdateArriveStatus` _controlledelephant false))))

(event `CheckForStucking`
  (bind _controlledelephant (`self.ControlledElephant`))
  (bind _controlledelephant_2 (`self.ControlledElephant`))
  (bind _controlledelephant_3 (`self.ControlledElephant`))
  (bind _controlledelephant_4 (`self.ControlledElephant`))
  (bind _barn (`Animal.Barn` _controlledelephant_2))
  ;[1 1 1] Check For Stucking Method.
  (if (and (and (not (`Animal.GetAttacked` _controlledelephant)) (and (and (and (not (`Animal.IsArriveAtSocket` _controlledelephant)) (<= (`KismetMathLibrary.VSize` (`self.GetVelocity` _controlledelephant)) 0.0)) (<= (`self.GetDistanceTo` _controlledelephant_2 _barn) (`Barn.InRange` _barn))) (`KismetSystemLibrary.IsValid` (`Animal.SelectedSocket` (`self.ControlledElephant`))))) (not (`Animal.IsThunderEnchantEffect` (`self.ControlledElephant`))))
    (bind _output_get (set `Animal.StuckSeconds` (+ (`Animal.StuckSeconds` _controlledelephant_3) (`GameplayStatics.GetWorldDeltaSeconds`)) (`self.ControlledElephant`)))
    (if (>= _output_get 1.0)
      (set `Animal.IsStuck` true _controlledelephant_4)
      (set `Animal.StuckSeconds` 0.0 _controlledelephant_4))
    (else
      (set `Animal.StuckSeconds` 0.0 _controlledelephant_3))))

(fn `UserConstructionScript`)