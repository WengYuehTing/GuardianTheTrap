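; Choppable tree resource that randomizes its yaw, scale and mesh on the authority at BeginPlay.
; Shake handles each hit: the authority spawns a Reward_BP and credits wood to the player and ResourceManager_BP, HP drops, and the local player's controller rumbles.
; A timeline drives a material wobble and gates repeat hits.
; At zero HP the tree topples with physics, fades through chop-down materials and destroys itself.
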(event `self.ReceiveBeginPlay`
  (bind (_returnvalue_roll _returnvalue_pitch) (`KismetMathLibrary.BreakRotator` (`SceneComponent.K2_GetComponentRotation` (`self.StaticMesh`))))
  (`/Engine/EditorBlueprintResources/ActorMacros.Switch Has Authority`
    (:`Authority`
      (`SceneComponent.K2_SetWorldRotation` (`self.StaticMesh`) (`KismetMathLibrary.MakeRotator` _returnvalue_roll _returnvalue_pitch (`KismetMathLibrary.Conv_IntToDouble` (`KismetMathLibrary.RandomIntegerInRange` 0 360))) false false)
      (`SceneComponent.SetWorldScale3D` (`self.StaticMesh`) (`KismetMathLibrary.Conv_DoubleToVector` (`KismetMathLibrary.RandomFloatInRange` 0.7 1.0)))
      (switch `int` (`KismetMathLibrary.RandomIntegerInRange` 0 4)
        (:`0`
          (`self.ChangeSkin` "/Game/Maps/Level1/Environment_Level1/Tree007.Tree007"))
        (:`1`
          (`self.ChangeSkin` "/Game/Maps/Level1/Environment_Level1/Tree008.Tree008"))
        (:`2`
          (`self.ChangeSkin` "/Game/Maps/Level1/Environment_Level1/Tree009.Tree009"))
        (:`3`
          (`self.ChangeSkin` "/Game/Maps/Level1/Environment_Level1/Tree010.Tree010"))
        (:`4`
          (`self.ChangeSkin` "/Game/Maps/Level1/Environment_Level1/Tree011.Tree011"))))))

(event `ChangeSkin`
  (params (NewMesh :type "StaticMesh Object Reference"))
  (`StaticMeshComponent.SetStaticMesh` (`self.StaticMesh`) NewMesh))

(event `self.ReceiveTick`
  (params (DeltaSeconds :type "Float (single-precision)")))

(event `Shake`
  (params (PlayerCut :type "/Game/Player/VRPawn Object Reference") (`MC Component` :type "MotionControllerComponent Object Reference") (Damage :type "Float (double-precision)") (Velocity :type "Vector Structure"))
  (bind _staticmesh (`self.StaticMesh`))
  (bind _staticmesh_2 (`self.StaticMesh`))
  (if (not (`self.BeCut`))
    (`|ExecutionSequence`
      (:`then_0`
        (set `self.BeCut` true)
        (`AudioComponent.Play` (`self.Audio`) 0.0)
        (`/Engine/EditorBlueprintResources/ActorMacros.Switch Has Authority`
          (:`Authority`
            (`self.Server Spawn Reward` PlayerCut Damage)
            (set `/Game/Player/VRPawn.Woods` (+ (`/Game/Player/VRPawn.Woods` PlayerCut) Damage) PlayerCut)
            (bind _outactors (`GameplayStatics.GetAllActorsOfClass` "/Game/LevelManager/ResourceManager_BP.ResourceManager_BP_C"))
            (bind _output (`|GetArrayItem` _outactors))
            (set `/Game/LevelManager/ResourceManager_BP.Woods` (+ (`/Game/LevelManager/ResourceManager_BP.Woods` _output) Damage) _output))
          (:`Remote`
            _))
        (bind _output_get (set `self.HP` (- (`self.HP`) 1.0)))
        (if (> _output_get 0.0)
          (bind (_direction _duration) (`Timeline|ShakeEffect` :!via `PlayFromStart`)
            (:`Update`
              (bind _returnvalue (`PrimitiveComponent.CreateDynamicMaterialInstance` (`self.StaticMesh`) 0 null "None"))
              (`MaterialInstanceDynamic.SetScalarParameterValue` _returnvalue "ShaveScale" _duration)
              (bind _returnvalue_2 (`PrimitiveComponent.CreateDynamicMaterialInstance` (`self.StaticMesh`) 1 null "None"))
              (`MaterialInstanceDynamic.SetScalarParameterValue` _returnvalue_2 "ShaveScale" _duration))
            (:`Finished`
              (set `self.BeCut` false)))
          (else
            (`AudioComponent.Play` (`self.DestroySound`) 0.0)
            (`PrimitiveComponent.SetSimulatePhysics` _staticmesh true)
            (`PrimitiveComponent.AddImpulse` _staticmesh (+ (* Velocity 10.0) (`SceneComponent.K2_GetComponentLocation` _staticmesh)) "None" false)
            (`KismetSystemLibrary.Delay` 4.0)
            (bind _returnvalue_3 (`PrimitiveComponent.CreateDynamicMaterialInstance` _staticmesh_2 0 "/Game/Resources/Wood/M_LeavesChopDown_Inst.M_LeavesChopDown_Inst" "None"))
            (bind _returnvalue_4 (`PrimitiveComponent.CreateDynamicMaterialInstance` _staticmesh_2 1 "/Game/Resources/Wood/M_WoodChopDown_Inst.M_WoodChopDown_Inst" "None"))
            (bind (_direction_2 _duration_2) (`Timeline|FadeOut` :!via `PlayFromStart`)
              (:`Update`
                (`MaterialInstanceDynamic.SetScalarParameterValue` _returnvalue_3 "opacity" _duration_2)
                (`MaterialInstanceDynamic.SetScalarParameterValue` _returnvalue_4 "opacity" _duration_2))
              (:`Finished`
                (`self.K2_DestroyActor`))))))
      (:`then_1`
        (if (`Pawn.IsLocallyControlled` PlayerCut)
          (`/Game/Player/VRPawn.RumbleController` PlayerCut 0.8 `MC Component`))))))

(event `Server Spawn Reward`
  (params (`Player Cut` :type "/Game/Player/VRPawn Object Reference") (Damage :type "Float (double-precision)"))
  (bind (_returnvalue_x _returnvalue_y _returnvalue_z) (`KismetMathLibrary.BreakVector` (`self.K2_GetActorLocation`)))
  (`|SpawnActorFromClass` "/Game/Resources/Reward_BP.Reward_BP_C" (`KismetMathLibrary.MakeTransform` (`KismetMathLibrary.MakeVector` _returnvalue_x _returnvalue_y (+ _returnvalue_z 80.0))) "AlwaysSpawn" "OverrideRootScale" `Player Cut` Damage "NewEnumerator1" null))

(fn `UserConstructionScript`)