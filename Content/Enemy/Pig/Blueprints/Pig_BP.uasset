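; Pig enemy character for a VR game that claims a target socket, attacks, and can spawn a reward.
; AnyDamage branches on damage type, crediting direct hits to the VRPawn and spawning damage numbers.
; Fire, ice and thunder enchants run duration-set timelines for burn, slow and paralysis, with multicast tint, particles and animation rate.
; Tick turns the health bar toward the player and drains HP when a server-side watchdog detects a stuck or runaway pig.
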(event `HealthBar face player`
  ;[0.01179 0.6964 1] HealthBar setting
  (bind _asvrpawn (cast `/Game/Player/VRPawn` (`GameplayStatics.GetPlayerPawn` 0)))
  (`SceneComponent.K2_SetWorldRotation` (`self.HealthBar`) (`KismetMathLibrary.FindLookAtRotation` (`SceneComponent.K2_GetComponentLocation` (`self.HealthBar`)) (`SceneComponent.K2_GetComponentLocation` (`/Game/Player/VRPawn.Head` _asvrpawn))) false false))

(event `self.ReceiveBeginPlay`
  (`self.InitHealthBar`))

(event `self.ReceiveTick`
  (params (DeltaSeconds :type "Float (single-precision)"))
  (`self.HealthBar face player`)
  (bind _startsuicide (`self.Suicide`))
  (if _startsuicide
    (set `self.HP` (- (`self.HP`) (* (`GameplayStatics.GetWorldDeltaSeconds`) (/ (`self.MaxHP`) 6.0))))))

(event `InitHealthBar`
  ;[0.01179 0.6964 1] HealthBar setting
  (bind _asw_animal_health_bar (cast `/Game/Enemy/Widgets/W_AnimalHealthBar` (`WidgetComponent.GetUserWidgetObject` (`self.HealthBar`))))
  (set `/Game/Enemy/Widgets/W_AnimalHealthBar.Animal` self _asw_animal_health_bar))

(event `self.ReceiveDestroyed`
  (`self.ReleaseSocket`))

(event `SetSpeed`
  (params (SpeedToSet :type "Float (double-precision)"))
  (if (not (== SpeedToSet (`self.PreviousSpeed`)))
    (set `CharacterMovementComponent.MaxWalkSpeed` SpeedToSet (`self.CharacterMovement`))
    (set `self.PreviousSpeed` SpeedToSet)))

(event `AcquireSocket`
  (params (TargetSocket :type "/Game/Barn/Blueprints/BarnSocket_BP Object Reference"))
  (bind _output_get (set `self.SelectedSocket` TargetSocket))
  (set `BarnSocket.BeSeleced` true _output_get)
  (set `self.DistanceToSocket` (`self.GetDistanceTo` _output_get))
  (set `BarnSocket.CustomerAnimal` self _output_get))

(event `self.ReceiveAnyDamage`
  (params (Damage :type "Float (single-precision)") (DamageType :type "DamageType Object Reference") (InstigatedBy :type "Controller Object Reference") (DamageCauser :type "Actor Object Reference"))
  (bind (_returnvalue_x _returnvalue_y _returnvalue_z) (`KismetMathLibrary.BreakVector` (`SceneComponent.K2_GetComponentLocation` (`self.HealthBar`))))
  (bind _returnvalue (`KismetMathLibrary.FClamp` (`self.LocalDamage`) 0.0 (`self.HP`)))
  (bind _returnvalue_2 (`KismetMathLibrary.FClamp` (`self.LocalDamage`) 0.0 (`self.HP`)))
  (bind (_returnvalue_x_2 _returnvalue_y_2 _returnvalue_z_2) (`KismetMathLibrary.BreakVector` (`SceneComponent.K2_GetComponentLocation` (`self.HealthBar`))))
  (set `self.LocalDamage` Damage)
  (set `self.LocalDamageType` DamageType)
  (set `self.LocalDamageCauser` DamageCauser)
  (`|ExecutionSequence`
    (:`then_0`
      (if (== (`GameplayStatics.GetObjectClass` (`self.LocalDamageType`)) "/Game/Enemy/DamageType/NormalDamage_BP.NormalDamage_BP_C")
        (`self.Multicast PlayBeAttackedSound`)
        (bind _asvrpawn (cast `/Game/Player/VRPawn` (`self.LocalDamageCauser`))
          (:`then`
            (set `/Game/Player/VRPawn.Damage` (+ (`/Game/Player/VRPawn.Damage` _asvrpawn) _returnvalue) _asvrpawn))
          (:`CastFailed`
            _))
        (set `self.HP` (- (`self.HP`) _returnvalue))
        (set `self.GetAttacked` true)
        (`|SpawnActorFromClass` "/Game/Enemy/DamageValue_BP.DamageValue_BP_C" (`KismetMathLibrary.MakeTransform` (`KismetMathLibrary.MakeVector` (+ _returnvalue_x_2 (`KismetMathLibrary.RandomFloatInRange` -15.0 15.0)) (+ _returnvalue_y_2 (`KismetMathLibrary.RandomFloatInRange` -15.0 15.0)) (+ _returnvalue_z_2 (`KismetMathLibrary.RandomFloatInRange` -10.0 5.0)))) "Undefined" "OverrideRootScale" null (`self.LocalDamage`) null)
        (`KismetSystemLibrary.Delay` (`self.RecoveryCD`))
        (set `self.GetAttacked` false)))
    (:`then_1`
      (if (== (`GameplayStatics.GetObjectClass` (`self.LocalDamageType`)) "/Game/Enemy/DamageType/FireDamage_BP.FireDamage_BP_C")
        (`self.ProcessingBurnDamage` (`self.LocalDamage`) (`self.FireDuration`) (`self.LocalDamageCauser`))))
    (:`then_2`
      (if (== (`GameplayStatics.GetObjectClass` (`self.LocalDamageType`)) "/Game/Enemy/DamageType/IceDamage_BP.IceDamage_BP_C")
        (`self.ProcessingIceDamage` (`self.IceDuration`) (`self.LocalDamageCauser`))))
    (:`then_3`
      (if (== (`GameplayStatics.GetObjectClass` (`self.LocalDamageType`)) "/Game/Enemy/DamageType/ThunderDamage_BP.ThunderDamage_BP_C")
        (`self.ProcessingPalsy` (`self.ThunderDuration`) (`self.LocalDamageCauser`))))
    (:`then_4`
      (if (== (`GameplayStatics.GetObjectClass` (`self.LocalDamageType`)) "/Game/Enemy/DamageType/WeaponDamage_BP.WeaponDamage_BP_C")
        (if (not (`self.IsHurtByWeapon`))
          (set `self.IsHurtByWeapon` true)
          (`self.Multicast PlayBeAttackedSound`)
          (bind _asvrpawn_2 (cast `/Game/Player/VRPawn` (`self.LocalDamageCauser`))
            (:`then`
              (set `/Game/Player/VRPawn.Damage` (+ (`/Game/Player/VRPawn.Damage` _asvrpawn_2) _returnvalue_2) _asvrpawn_2))
            (:`CastFailed`
              _))
          (set `self.HP` (- (`self.HP`) _returnvalue_2))
          (`|SpawnActorFromClass` "/Game/Enemy/DamageValue_BP.DamageValue_BP_C" (`KismetMathLibrary.MakeTransform` (`KismetMathLibrary.MakeVector` (+ _returnvalue_x (`KismetMathLibrary.RandomFloatInRange` -15.0 15.0)) (+ _returnvalue_y (`KismetMathLibrary.RandomFloatInRange` -15.0 15.0)) (+ _returnvalue_z (`KismetMathLibrary.RandomFloatInRange` -10.0 5.0)))) "Undefined" "OverrideRootScale" null (`self.LocalDamage`) null)
          (`KismetSystemLibrary.Delay` (`self.HurtWeaponCD`))
          (set `self.IsHurtByWeapon` false))))))

(event `/Game/ElementBottle/EnchantableInterface.Enchanted`
  (params (EnchantType :type "EnchantType Enum" :default "Fire") (Duration :type "Float (single-precision)") (Damage :type "Float (single-precision)") (EnchantBottle :type "ElementBottle Object Reference") (Player :type "/Game/Player/VRPawn Object Reference"))
  (switch `EnchantType` EnchantType
    (:`Fire`
      (set `self.FireSufferDamage` Damage)
      (set `self.FireDuration` Duration)
      (`GameplayStatics.ApplyDamage` self (`self.FireSufferDamage`) null Player "/Game/Enemy/DamageType/FireDamage_BP.FireDamage_BP_C")
      (set `self.IsFireEnchantEffect` true))
    (:`Ice`
      (set `self.IceDuration` Duration)
      (`GameplayStatics.ApplyDamage` self Damage null Player "/Game/Enemy/DamageType/IceDamage_BP.IceDamage_BP_C")
      (set `self.IsIceEnchantEffect` true))
    (:`Thunder`
      (set `self.ThunderDuration` Duration)
      (`GameplayStatics.ApplyDamage` self Damage null Player "/Game/Enemy/DamageType/ThunderDamage_BP.ThunderDamage_BP_C")
      (set `self.IsThunderEnchantEffect` true))))

(event `Server SpawnReward`
  (bind (_returnvalue_x _returnvalue_y _returnvalue_z) (`KismetMathLibrary.BreakVector` (`self.K2_GetActorLocation`)))
  (`|SpawnActorFromClass` "/Game/Resources/Reward_BP.Reward_BP_C" (`KismetMathLibrary.MakeTransform` (`KismetMathLibrary.MakeVector` _returnvalue_x _returnvalue_y (+ _returnvalue_z 90.0))) "AlwaysSpawn" "OverrideRootScale" (`self.LocalDamageCauser`) (`self.Reward`) "NewEnumerator0" null))

(event `Attack`
  (set `self.IsAttacking` true)
  (`self.Multicast PlayAttackSound`)
  (`KismetSystemLibrary.Delay` (`self.AttackAnimDuration`))
  (set `self.IsAttacking` false))

(event `ProcessingBurnDamage`
  (params (`Fire Damage` :type "Float (double-precision)") (Duration :type "Float (double-precision)") (DamageCauser :type "Actor Object Reference"))
  (bind _hp (`self.HP`))
  (bind _returnvalue (* (`GameplayStatics.GetWorldDeltaSeconds`) `Fire Damage`))
  (`self.Multicast Activate ElementBottle` "Fire")
  (bind _asvrpawn (cast `/Game/Player/VRPawn` DamageCauser))
  (bind _result (`/Engine/EditorBlueprintResources/StandardMacros.IncrementFloat` (`self.FireColorBoost`))
    (:`  `
      (`self.Multicast ChangeEnchantColor` (`self.Mesh`) "/Game/Enemy/Pig/Models/MI_Pig.MI_Pig" "BoostColor" (`KismetMathLibrary.MakeColor` _result (`self.IceColorBoost`) (`self.ThunderColorBoost`)))
      (`TimelineComponent.SetTimelineLength` (`self.Burn`) Duration)
      (`Timeline|Burn` :!via `PlayFromStart`
        (:`Update`
          (if (>= _hp 0.0)
            (set `self.HP` (- _hp _returnvalue))
            (set `/Game/Player/VRPawn.Damage` (+ _returnvalue (`/Game/Player/VRPawn.Damage` _asvrpawn)) _asvrpawn)))
        (:`Finished`
          (set `self.IsFireEnchantEffect` false)
          (set `self.FireColorBoost` 0.0)
          (`self.Multicast ChangeEnchantColor` (`self.Mesh`) "/Game/Enemy/Pig/Models/MI_Pig.MI_Pig" "BoostColor" (`KismetMathLibrary.MakeColor` 0.0 (`self.IceColorBoost`) (`self.ThunderColorBoost`)))
          (`self.Multicast Deactivate ElementBottle` "Fire"))))))

(event `Multicast PigWalkOnly`
  (`SkeletalMeshComponent.K2_SetAnimInstanceClass` (`self.Mesh`) "/Game/Enemy/Pig/Animation/PigAnim_BP.PigAnim_BP_C"))

(event `Multicast PlayAttackSound`
  ;[1 1 1] Sound
  (`AudioComponent.Play` (`self.AttackSound`) 0.0))

(event `ProcessingIceDamage`
  (params (Duration :type "Float (double-precision)") (DamageCauser :type "Actor Object Reference"))
  (`self.Multicast Activate ElementBottle` "Ice")
  (set `self.AttackAnimDuration` 2.2)
  (`TimelineComponent.SetTimelineLength` (`self.Ice`) Duration)
  (bind _result (`/Engine/EditorBlueprintResources/StandardMacros.IncrementFloat` (`self.IceColorBoost`))
    (:`  `
      (`self.Multicast ChangeEnchantColor` (`self.Mesh`) "/Game/Enemy/Pig/Models/MI_Pig.MI_Pig" "BoostColor" (`KismetMathLibrary.MakeColor` (`self.FireColorBoost`) _result (`self.ThunderColorBoost`)))
      (`Timeline|Ice` :!via `PlayFromStart`
        (:`Update`
          (if (>= (`SkeletalMeshComponent.GlobalAnimRateScale` (`self.Mesh`)) 0.1)
            (set `self.Speed` (/ (`self.MaxSpeed`) 2.0))
            (set `self.AttackSpeed` (* (`self.MaxAttackSpeed`) 2.0))
            (`self.Multicast ChangeAnimationSpeed` 0.5)))
        (:`Finished`
          (set `self.Speed` (`self.MaxSpeed`))
          (set `self.AttackSpeed` (`self.MaxAttackSpeed`))
          (set `self.AttackAnimDuration` 1.1)
          (set `self.IsIceEnchantEffect` false)
          (if (>= (`SkeletalMeshComponent.GlobalAnimRateScale` (`self.Mesh`)) 0.1)
            (`self.Multicast ChangeAnimationSpeed` 1.0))
          (set `self.IceColorBoost` 0.0)
          (`self.Multicast ChangeEnchantColor` (`self.Mesh`) "/Game/Enemy/Pig/Models/MI_Pig.MI_Pig" "BoostColor" (`KismetMathLibrary.MakeColor` (`self.FireColorBoost`) 0.0 (`self.ThunderColorBoost`)))
          (`self.Multicast Deactivate ElementBottle` "Ice"))))))

(event `Multicast PlayDeadSound`
  ;[1 1 1] Sound
  (`AudioComponent.Play` (`self.DeadSound`) 0.0))

(event `Multicast PlayBeAttackedSound`
  ;[1 1 1] Sound
  (if (not (`self.GetAttacked`))
    (`AudioComponent.Play` (`self.HurtSound`) 0.3)))

(event `ProcessingPalsy`
  (params (Duration :type "Float (double-precision)") (DamageCauser :type "Actor Object Reference"))
  (`self.Multicast Activate ElementBottle` "Thunder")
  (`self.Multicast ChangeAnimationSpeed` 0.0)
  (bind _result (`/Engine/EditorBlueprintResources/StandardMacros.IncrementFloat` (`self.FireColorBoost`))
    (:`  `
      (bind _result_2 (`/Engine/EditorBlueprintResources/StandardMacros.IncrementFloat` (`self.ThunderColorBoost`))
        (:`  `
          (`self.Multicast ChangeEnchantColor` (`self.Mesh`) "/Game/Enemy/Pig/Models/MI_Pig.MI_Pig" "BoostColor" (`KismetMathLibrary.MakeColor` _result (`self.IceColorBoost`) _result_2))
          (`TimelineComponent.SetTimelineLength` (`self.Palsy`) Duration)
          (`Timeline|Palsy` :!via `PlayFromStart`
            (:`Update`
              (set `self.Speed` 0.0))
            (:`Finished`
              (set `self.Speed` (`self.MaxSpeed`))
              (set `self.IsThunderEnchantEffect` false)
              (`self.Multicast ChangeAnimationSpeed` 1.0)
              (set `self.FireColorBoost` 0.0)
              (set `self.ThunderColorBoost` 0.0)
              (`self.Multicast ChangeEnchantColor` (`self.Mesh`) "/Game/Enemy/Pig/Models/MI_Pig.MI_Pig" "BoostColor" (`KismetMathLibrary.MakeColor` 0.0 (`self.IceColorBoost`)))
              (`self.Multicast Deactivate ElementBottle` "Thunder"))))))))

(event `Multicast ChangeAnimationSpeed`
  (params (GlobalAnimRateScale :type "Float (double-precision)"))
  (set `SkeletalMeshComponent.GlobalAnimRateScale` GlobalAnimRateScale (`self.Mesh`)))

(event `Multicast ChangeEnchantColor`
  (params (Target :type "PrimitiveComponent Object Reference") (SourceMaterial :type "MaterialInterface Object Reference") (ParamName :type Name) (Color :type "LinearColor Structure"))
  (bind _returnvalue (`PrimitiveComponent.CreateDynamicMaterialInstance` Target 0 SourceMaterial "None"))
  (`MaterialInstanceDynamic.SetVectorParameterValue` _returnvalue ParamName Color))

(event `Multicast Activate ElementBottle`
  (params (`Enchant Type` :type "EnchantType Enum" :default "Fire"))
  (switch `EnchantType` `Enchant Type`
    (:`Fire`
      (`ActorComponent.Activate` (`self.OnFire`) false))
    (:`Ice`
      (`SceneComponent.SetVisibility` (`self.OnIce`) true false))
    (:`Thunder`
      (`ActorComponent.Activate` (`self.OnPalsy`) false))))

(event `Multicast Deactivate ElementBottle`
  (params (`Enchant Type` :type "EnchantType Enum" :default "Fire"))
  (switch `EnchantType` `Enchant Type`
    (:`Fire`
      (`ActorComponent.Deactivate` (`self.OnFire`)))
    (:`Ice`
      (`SceneComponent.SetVisibility` (`self.OnIce`) false false))
    (:`Thunder`
      (`ActorComponent.Deactivate` (`self.OnPalsy`)))))

(event `Multicast PlayBuffParticle`
  (`ActorComponent.Activate` (`self.Buff`) false))

(fn `Suicide`
  (returns (StartSuicide :type Boolean))
  (`/Engine/EditorBlueprintResources/ActorMacros.Switch Has Authority`
    (:`Authority`
      (`/Engine/EditorBlueprintResources/StandardMacros.IsValid` (`self.Barn`)
        (:`Is Valid`
          (if (or (and (> (`self.GetDistanceTo` (`self.SelectedSocket`)) (`self.MinArriveDistance`)) (<= (`KismetMathLibrary.VSize` (`self.GetVelocity`)) 0.0) (not (`self.GetAttacked`)) (not (`self.IsThunderEnchantEffect`))) (>= (`KismetMathLibrary.VSize` (`self.GetVelocity`)) 1000.0))
            (bind _output_get (set `self.CurrentSecondsToSuicide` (+ (`self.CurrentSecondsToSuicide`) (`GameplayStatics.GetWorldDeltaSeconds`))))
            (return (>= _output_get (`self.MaxSecondsToSuicide`)))
            (else
              (set `self.CurrentSecondsToSuicide` 0.0))))))))

(fn `UserConstructionScript`)