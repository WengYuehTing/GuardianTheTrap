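; Ice zone actor from the element bottle system that applies an Ice enchant to Animals in its box.
; Animals receive EnchantedMessage with duration, damage, bottle and spawning VR pawn on both begin and end overlap.
; Tick also checks for Animals already inside until one is found and enchanted, then AutoActive disables the check.
; On authority, the zone destroys itself after Duration.
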(event `self.ReceiveBeginPlay`
  (`/Engine/EditorBlueprintResources/ActorMacros.Switch Has Authority`
    (:`Authority`
      (`KismetSystemLibrary.Delay` (`self.Duration`))
      (`self.K2_DestroyActor`))))

(event `self.ReceiveTick`
  (params (DeltaSeconds :type "Float (single-precision)"))
  (if (not (`self.AutoActive`))
    (for _array_element (`PrimitiveComponent.GetOverlappingActors` (`self.Box`) "/Script/Guardian_TheTrap.Animal")
      (bind _asvrpawn (cast `/Game/Player/VRPawn` (`self.PlayerSpawned`)))
      (message `/Game/ElementBottle/EnchantableInterface.Enchanted` _array_element "Ice" (`self.Duration`) (`self.Damage`) (`self.ElementBottle`) _asvrpawn)
      (set `self.AutoActive` true))))

(event `self.Box.OnComponentBeginOverlap`
  (params (OverlappedComponent :type "PrimitiveComponent Object Reference") (OtherActor :type "Actor Object Reference") (OtherComp :type "PrimitiveComponent Object Reference") (OtherBodyIndex :type Integer) (bFromSweep :type Boolean) (SweepResult :type "HitResult Structure (by ref)"))
  (bind _asanimal (cast `Animal` OtherActor))
  (bind _asvrpawn (cast `/Game/Player/VRPawn` (`self.PlayerSpawned`)))
  (message `/Game/ElementBottle/EnchantableInterface.Enchanted` _asanimal "Ice" (`self.Duration`) (`self.Damage`) (`self.ElementBottle`) _asvrpawn))

(event `self.Box.OnComponentEndOverlap`
  (params (OverlappedComponent :type "PrimitiveComponent Object Reference") (OtherActor :type "Actor Object Reference") (OtherComp :type "PrimitiveComponent Object Reference") (OtherBodyIndex :type Integer))
  (bind _asanimal (cast `Animal` OtherActor))
  (bind _asvrpawn (cast `/Game/Player/VRPawn` (`self.PlayerSpawned`)))
  (message `/Game/ElementBottle/EnchantableInterface.Enchanted` _asanimal "Ice" (`self.Duration`) (`self.Damage`) (`self.ElementBottle`) _asvrpawn))

(fn `UserConstructionScript`)