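; Reward_BP is a short-lived floating reward popup actor for VR, showing a W_Reward widget on its Text component.
; On BeginPlay it passes itself to the widget and plays the Reward timeline, which offsets the actor's height from its spawn point and drives the text alpha.
; Each tick the widget turns on yaw only to face the VRPawn's head.
; The actor destroys itself when the timeline finishes.
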(event `self.ReceiveBeginPlay`
  (bind (_origin_x _origin_y _origin_z) (`KismetMathLibrary.BreakVector` (`self.Origin`)))
  (set `self.Origin` (`self.K2_GetActorLocation`))
  (bind _asw_reward (cast `/Game/Resources/W_Reward` (`WidgetComponent.GetUserWidgetObject` (`self.Text`))))
  (set `/Game/Resources/W_Reward.Reward_BP` self _asw_reward)
  (bind (_direction _height _alpha) (`Timeline|Reward` :!via `PlayFromStart`)
    (:`Update`
      (`self.K2_SetActorLocation` (`KismetMathLibrary.MakeVector` _origin_x _origin_y (+ _origin_z _height)))
      (bind _asw_reward_2 (cast `/Game/Resources/W_Reward` (`WidgetComponent.GetUserWidgetObject` (`self.Text`))))
      (set `/Game/Resources/W_Reward.TextAlpha` _alpha _asw_reward_2))
    (:`Finished`
      (`self.K2_DestroyActor`))))

(event `self.ReceiveTick`
  (params (DeltaSeconds :type "Float (single-precision)"))
  (bind _asvrpawn (cast `/Game/Player/VRPawn` (`GameplayStatics.GetPlayerPawn` 0)))
  (bind (_returnvalue_roll _returnvalue_pitch _returnvalue_yaw) (`KismetMathLibrary.BreakRotator` (`KismetMathLibrary.FindLookAtRotation` (`SceneComponent.K2_GetComponentLocation` (`self.Text`)) (`SceneComponent.K2_GetComponentLocation` (`/Game/Player/VRPawn.Head` _asvrpawn)))))
  (`SceneComponent.K2_SetWorldRotation` (`self.Text`) (`KismetMathLibrary.MakeRotator` 0.0 0.0 _returnvalue_yaw) false false))

(fn `UserConstructionScript`)