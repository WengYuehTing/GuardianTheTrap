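; Level resource manager that tracks money, wood and ore and answers affordability queries.
; LendResource checks one resource type and CheckAvaliable checks all three, neither deducting anything.
; CheckLevelUp reads Spike, Bow and Catcher levels from the first TrapManager_BP found in the world, returning upgrade availability and money cost by level.
; Top-level traps and Barrel, Fan and Spring traps always report unavailable.
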(fn `CheckAvaliable`
  (params (Money :type "Float (double-precision)") (Wood :type "Float (double-precision)") (Ore :type "Float (double-precision)"))
  (returns (Avaliable :type Boolean))
  (return (and (>= (`self.Money`) Money) (>= (`self.Woods`) Wood) (>= (`self.Ores`) Ore))))

(fn `CheckLevelUp`
  (params (Trap :type "/Game/Player/Widgets/BubbleMenu/ETrapBubbleType Enum" :default "NewEnumerator0"))
  (returns (Avaliable :type Boolean) (ToCost :type "Float (double-precision)"))
  (switch `/Game/Player/Widgets/BubbleMenu/ETrapBubbleType` Trap
    (:`NewEnumerator0`
      (return false 0.0))
    (:`NewEnumerator1`
      (bind _outactors (`GameplayStatics.GetAllActorsOfClass` "/Game/LevelManager/TrapManager_BP.TrapManager_BP_C"))
      (switch `TrapLevel` (`/Game/LevelManager/TrapManager_BP.SpikeLevel` (`|GetArrayItem` _outactors))
        (:`Level_1`
          (return (>= (`self.Money`) 5.0) 5.0))
        (:`Level_2`
          (return (>= (`self.Money`) 10.0) 10.0))
        (:`Level_3`
          (return false 0.0))))
    (:`NewEnumerator2`
      (bind _outactors_2 (`GameplayStatics.GetAllActorsOfClass` "/Game/LevelManager/TrapManager_BP.TrapManager_BP_C"))
      (switch `TrapLevel` (`/Game/LevelManager/TrapManager_BP.BowLevel` (`|GetArrayItem` _outactors_2))
        (:`Level_1`
          (return (>= (`self.Money`) 5.0) 5.0))
        (:`Level_2`
          (return (>= (`self.Money`) 10.0) 10.0))
        (:`Level_3`
          (return false 0.0))))
    (:`NewEnumerator3`
      (bind _outactors_3 (`GameplayStatics.GetAllActorsOfClass` "/Game/LevelManager/TrapManager_BP.TrapManager_BP_C"))
      (switch `TrapLevel` (`/Game/LevelManager/TrapManager_BP.CatcherLevel` (`|GetArrayItem` _outactors_3))
        (:`Level_1`
          (return (>= (`self.Money`) 5.0) 5.0))
        (:`Level_2`
          (return (>= (`self.Money`) 10.0) 10.0))
        (:`Level_3`
          (return false 0.0))))
    (:`NewEnumerator4`
      (return false 0.0))
    (:`NewEnumerator5`
      (return false 0.0))))

(fn `LendResource`
  (params (Type :type "/Game/Resources/EResourceType Enum" :default "NewEnumerator0") (Amounts :type "Float (double-precision)"))
  (returns (Success :type Boolean))
  (locals (LocalAmounts :type "Float (double-precision)"))
  (set `local.LocalAmounts` Amounts)
  (switch `/Game/Resources/EResourceType` Type
    (:`NewEnumerator0`
      (if (>= (`self.Money`) (`local.LocalAmounts`))
        (return true)
        (else
          (return false))))
    (:`NewEnumerator1`
      (if (>= (`self.Woods`) (`local.LocalAmounts`))
        (return true)
        (else
          (return false))))
    (:`NewEnumerator2`
      (if (>= (`self.Ores`) (`local.LocalAmounts`))
        (return true)
        (else
          (return false))))))

(fn `UserConstructionScript`)