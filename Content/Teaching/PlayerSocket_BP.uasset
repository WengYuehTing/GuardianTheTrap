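; PlayerSocket_BP is a teaching trigger that shows teaching UI when the VR player arrives at its capsule.
; Each tick it polls the capsule for overlapping VRPawn actors instead of using overlap events.
; On the first detected arrival it calls SpawnTeachingUI on player pawn 0, passing its configured material and event.
; A flag that is never reset here limits this to one successful spawn.
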(event `self.ReceiveTick`
  (params (DeltaSeconds :type "Float (single-precision)"))
  (`|ExecutionSequence`
    (:`then_0`
      (set `self.IsPlayerArrived` (> (`KismetArrayLibrary.Array_Length` (`PrimitiveComponent.GetOverlappingActors` (`self.Capsule`) "/Game/Player/VRPawn.VRPawn_C")) 0)))
    (:`then_1`
      (if (`self.IsPlayerArrived`)
        (if (`self.AlreadyPawnTeaching`)
          _
          (elif true
            (bind _asvrpawn (cast `/Game/Player/VRPawn` (`GameplayStatics.GetPlayerPawn` 0)))
            (`/Game/Player/VRPawn.SpawnTeachingUI` _asvrpawn (`self.MaterialToShow`) (`self.EventToTrigger`))
            (set `self.AlreadyPawnTeaching` true)))))))

(fn `UserConstructionScript`)