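; Game mode for a multiplayer VR game that spawns and possesses a VR pawn for each player who logs in.
; On the server, PostLogin places each pawn at the next PlayerStart, offset by PlayerHeightMinus, tags it with a player index and has the player controller possess it.
; The game instance's level check leads to two identical spawn branches.
; BeginPlay enables stereo rendering by console command and resets the start-point index.
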(event `self.ReceiveBeginPlay`
  (`KismetSystemLibrary.ExecuteConsoleCommand` "stereo on" null)
  (set `self.PlayerStateIndex` 0))

(event `self.K2_PostLogin`
  (params (NewPlayer :type "PlayerController Object Reference"))
  (`/Engine/EditorBlueprintResources/ActorMacros.Switch Has Authority`
    (:`Authority`
      (bind _outactors (`GameplayStatics.GetAllActorsOfClass` "/Script/Engine.PlayerStart"))
      (bind _asgtt_game_instance_bp (cast `/Game/GameInstance/GTT_GameInstance_BP` (`GameplayStatics.GetGameInstance`)))
      (if (`|EnumEquality` (`/Game/GameInstance/GTT_GameInstance_BP.GameLevel` _asgtt_game_instance_bp) "NewEnumerator0")
        (bind _returnvalue (`KismetMathLibrary.MakeTransform` (- (.location (`self.GetTransform` (`|GetArrayItem` _outactors (`self.PlayerStateIndex`)))) (`self.PlayerHeightMinus`)) (.rotation (`self.GetTransform` (`|GetArrayItem` _outactors (`self.PlayerStateIndex`)))) (.scale (`self.GetTransform` (`|GetArrayItem` _outactors (`self.PlayerStateIndex`))))))
        (bind _returnvalue_2 (`|SpawnActorFromClass` "/Game/Player/VRPawn.VRPawn_C" _returnvalue "AlwaysSpawn" "OverrideRootScale" null null))
        (set `/Game/Player/VRPawn.UniqueID` (`self.playerIndex`) _returnvalue_2)
        (bind _asplayer_controller_bp (cast `/Game/PlayerController/PlayerController_BP` NewPlayer))
        (`Controller.Possess` _asplayer_controller_bp _returnvalue_2)
        (`/Engine/EditorBlueprintResources/StandardMacros.IncrementInt` (`self.playerIndex`)
          (:`  `
            (`/Engine/EditorBlueprintResources/StandardMacros.IncrementInt` (`self.PlayerStateIndex`))))
        (else
          (bind _returnvalue_3 (`|SpawnActorFromClass` "/Game/Player/VRPawn.VRPawn_C" _returnvalue "AlwaysSpawn" "OverrideRootScale" null null))
          (set `/Game/Player/VRPawn.UniqueID` (`self.playerIndex`) _returnvalue_3)
          (bind _asplayer_controller_bp_2 (cast `/Game/PlayerController/PlayerController_BP` NewPlayer))
          (`Controller.Possess` _asplayer_controller_bp_2 _returnvalue_3)
          (`/Engine/EditorBlueprintResources/StandardMacros.IncrementInt` (`self.playerIndex`)
            (:`  `
              (`/Engine/EditorBlueprintResources/StandardMacros.IncrementInt` (`self.PlayerStateIndex`)))))))))

(event `self.ReceiveTick`
  (params (DeltaSeconds :type "Float (single-precision)")))

(fn `UserConstructionScript`)