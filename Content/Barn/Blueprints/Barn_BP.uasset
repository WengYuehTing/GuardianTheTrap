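; Barn actor for a VR game that loses health from any damage and plays a lose sound when it falls.
; Damage subtracts HP and plays an attacked sound; Tick watches for zero HP to trigger a one-time collapse sound, then the lose sound and destruction.
; BeginPlay links the health bar widget to the barn.
; A yaw-only routine to face the bar toward the VR pawn's head exists, but its call is disconnected.
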(event `self.ReceiveBeginPlay`
  (`self.InitHealthBar`))

(event `self.ReceiveTick`
  (params (DeltaSeconds :type "Float (single-precision)"))
  (if (<= (`self.HP`) 0.0)
    (`self.Collapsed`)))

(event `self.ReceiveAnyDamage`
  (params (Damage :type "Float (single-precision)") (DamageType :type "DamageType Object Reference") (InstigatedBy :type "Controller Object Reference") (DamageCauser :type "Actor Object Reference"))
  (set `self.HP` (- (`self.HP`) Damage))
  (`self.PlayBeAttackedSound`))

(event `PlayBeAttackedSound`
  (`AudioComponent.Play` (`self.BeAttacked`) 0.9))

(event `Collapsed`
  (bind _collapsedsound (`self.CollapsedSound`))
  (if (not (`self.IsCollapsed`))
    (set `self.IsCollapsed` true)
    (`AudioComponent.Play` _collapsedsound 0.0)
    (`KismetSystemLibrary.Delay` (`SoundBase.Duration` (`AudioComponent.Sound` _collapsedsound)))
    (`self.Multicast PlayLoseSound`)
    (`self.K2_DestroyActor`)))

(event `InitHealthBar`
  ;[1 1 1] Handle Health Bar
  (bind _asbarn_health_bar (cast `/Game/Barn/Widgets/BarnHealthBar` (`WidgetComponent.GetUserWidgetObject` (`self.HealthBar`))))
  (set `/Game/Barn/Widgets/BarnHealthBar.Barn` self _asbarn_health_bar))

(event `HealthBar face player`
  ;[1 1 1] Handle Health Bar
  (bind _asvrpawn (cast `/Game/Player/VRPawn` (`GameplayStatics.GetPlayerPawn` 0)))
  (bind (_returnvalue_roll _returnvalue_pitch _returnvalue_yaw) (`KismetMathLibrary.BreakRotator` (`KismetMathLibrary.FindLookAtRotation` (`SceneComponent.K2_GetComponentLocation` (`self.HealthBar`)) (`SceneComponent.K2_GetComponentLocation` (`/Game/Player/VRPawn.Head` _asvrpawn)))))
  (`SceneComponent.K2_SetWorldRotation` (`self.HealthBar`) (`KismetMathLibrary.MakeRotator` 0.0 0.0 _returnvalue_yaw) false false))

(event `Multicast PlayLoseSound`
  (`GameplayStatics.PlaySound2D` "/Game/Sounds/S_Lose.S_Lose" 1.0 1.0 0.0 null null))

(fn `UserConstructionScript`)