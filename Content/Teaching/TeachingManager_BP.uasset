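; TeachingManager_BP is a tutorial manager that advances a teaching sequence by lighting up the next stage.
; OpenNextStageLight increments CurrentStage and switches on it, with only stage 2 wired.
; That stage plays the TurnonLight2 timeline, which drives the second queued spotlight's intensity and, on each update, shows the second player socket while hiding the first.
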(event `self.ReceiveBeginPlay`)

(event `self.ReceiveTick`
  (params (DeltaSeconds :type "Float (single-precision)")))

(event `OpenNextStageLight`
  (bind _playersocketqueue (`self.PlayerSocketQueue`))
  (`/Engine/EditorBlueprintResources/StandardMacros.IncrementInt` (`self.CurrentStage`)
    (:`  `
      (switch `int` (`self.CurrentStage`)
        (:`2`
          (bind (_direction _duration) (`Timeline|TurnonLight2` :!via `PlayFromStart`)
            (:`Update`
              (`LightComponent.SetIntensity` (`Light.LightComponent` (`|GetArrayItem` (`self.SpotLightQueue`) 1)) _duration)
              (`self.SetActorHiddenInGame` (`|GetArrayItem` _playersocketqueue 1) false)
              (`self.SetActorHiddenInGame` (`|GetArrayItem` _playersocketqueue) true))))))))

(fn `UserConstructionScript`)