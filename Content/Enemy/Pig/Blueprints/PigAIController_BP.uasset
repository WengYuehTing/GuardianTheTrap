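; AI controller for the enemy pig that claims a socket at the barn as its movement target.
; After a short delay it finds the barn, picks a socket and runs the Pig_BT behavior tree.
; Each tick it updates pig state, including arrival and stuck flags, and re-evaluates the nearest idle socket.
; A closer pig can take an idle socket from a farther animal, which is released and flagged as reselected.
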(event `self.ReceiveBeginPlay`
  (`KismetSystemLibrary.Delay` 0.2)
  ;[1 1 1] Init : Proprecessing property
  (`self.SetControlledPigRef`)
  (`self.FindBarn`)
  (`self.SelectBarnSocket`)
  (bind _returnvalue (`self.RunBehaviorTree` "/Game/Enemy/Pig/AI/Pig_BT.Pig_BT"))
  (if _returnvalue
    (`self.UseBlackboard` "/Game/Enemy/Pig/AI/Pig_BD.Pig_BD")
    (set `Animal.SelfAwareness` true (`self.ControlledPig`))
    (set `self.InitFinish` true)))

(event `self.ReceiveTick`
  (params (DeltaSeconds :type "Float (single-precision)"))
  (if (`self.InitFinish`)
    ;[1 1 1] RunTime: Update
    (`self.UpdateSpeed`)
    (`self.CheckOnGround`)
    (`self.UpdateBarn`)
    (`/Engine/EditorBlueprintResources/StandardMacros.IsValid` (`Animal.Barn` (`self.ControlledPig`))
      (:`Is Valid`
        (`self.CalculateDistance`)
        (`self.UpdateArrivalStatus`)
        (`self.CheckForStucking`)
        (`self.GetNearestIdleSocket`)
        (`self.ReSelectSocket`)))))

(event `SetControlledPigRef`
  ;[1 1 1] Get Controlled Pig References
  (bind _aspig_bp (cast `/Game/Enemy/Pig/Blueprints/Pig_BP` (`self.K2_GetPawn`)))
  (set `self.ControlledPig` _aspig_bp))

(event `FIndBarn`
  ;[1 1 1] Find Barn Method, Set to Controlled Pig Target, And Set Distance Between Pig & Barn.
  (bind _outactors (`GameplayStatics.GetAllActorsOfClass` "/Game/Barn/Blueprints/Barn_BP.Barn_BP_C"))
  (set `Animal.Barn` (`|GetArrayItem` _outactors) (`self.ControlledPig`)))

(event `InitHealthBar`
  (bind _controlledpig (`self.ControlledPig`))
  ;[1 1 1] Init Health Bar
  (bind _asw_animal_health_bar (cast `/Game/Enemy/Widgets/W_AnimalHealthBar` (`WidgetComponent.GetUserWidgetObject` (`/Game/Enemy/Pig/Blueprints/Pig_BP.HealthBar` _controlledpig))))
  (set `/Game/Enemy/Widgets/W_AnimalHealthBar.Animal` _controlledpig _asw_animal_health_bar))

(event `SelectBarnSocket`
  (bind _controlledpig (`self.ControlledPig`))
  (bind _index (`self.Index`))
  ;[1 1 1] Select Barn Socket To Move
  (`/Engine/EditorBlueprintResources/StandardMacros.IsValid` (`Animal.Barn` _controlledpig)
    (:`Is Valid`
      (set `self.MinDis` 100000.0)
      (set `self.Index` -1)
      (bind _outactors (`GameplayStatics.GetAllActorsOfClass` "/Game/Barn/Blueprints/BarnSocket_BP.BarnSocket_BP_C"))
      (for (_array_element _array_index) _outactors
        (if (not (`BarnSocket.BeSeleced` _array_element))
          (bind _returnvalue (`self.GetDistanceTo` (`self.ControlledPig`) _array_element))
          (if (<= _returnvalue (`self.MinDis`))
            (set `self.MinDis` _returnvalue)
            (set `self.Index` _array_index))
          (elif (`BarnSocket.Idle` _array_element)
            (bind _asanimal (cast `Animal` (`BarnSocket.CustomerAnimal` _array_element)))
            (bind _returnvalue_2 (`self.GetDistanceTo` _array_element (`self.ControlledPig`)))
            (if (> (`Animal.DistanceToSocket` _asanimal) _returnvalue_2)
              (set `self.MinDis` _returnvalue_2)
              (set `self.Index` _array_index)))))
      (if (>= _index 0)
        (bind _output (`|GetArrayItem` _outactors _index))
        (if (not (`BarnSocket.BeSeleced` _output))
          (`/Game/Enemy/Pig/Blueprints/Pig_BP.AcquireSocket` (`self.ControlledPig`) _output)
          (else
            (bind _asanimal_2 (cast `Animal` (`BarnSocket.CustomerAnimal` _output)))
            (`/Game/Enemy/Pig/Blueprints/Pig_BP.ReleaseSocket` _asanimal_2)
            (set `Animal.IsReselected` true _asanimal_2)
            (`/Game/Enemy/Pig/Blueprints/Pig_BP.AcquireSocket` (`self.ControlledPig`) _output)))))
    (:`Is Not Valid`
      (set `Animal.SelectedSocket` null _controlledpig))))

(event `UpdateSpeed`
  (bind _controlledpig (`self.ControlledPig`))
  ;[1 1 1] Update Speed Method
  (`/Game/Enemy/Pig/Blueprints/Pig_BP.SetSpeed` _controlledpig (`Animal.Speed` _controlledpig)))

(event `CheckOnGround`
  (bind _controlledpig (`self.ControlledPig`))
  ;[1 1 1] Check Pig is on ground on not
  (set `Animal.IsOnGround` (not (`NavMovementComponent.IsFalling` (`Character.CharacterMovement` _controlledpig))) _controlledpig))

(event `UpdateBarn`
  (bind _controlledpig (`self.ControlledPig`))
  ;[1 1 1] Update Barn Info
  (bind _outactors (`GameplayStatics.GetAllActorsOfClass` "/Game/Barn/Blueprints/Barn_BP.Barn_BP_C"))
  (if (== (`KismetArrayLibrary.Array_Length` _outactors) 0)
    (set `Animal.Barn` null _controlledpig)
    (`/Game/Enemy/Pig/Blueprints/Pig_BP.ReleaseSocket` _controlledpig)))

(event `CalculateDistance`
  (bind _controlledpig (`self.ControlledPig`))
  ;[1 1 1] Calculate Pig & Barn Distance
  (`/Engine/EditorBlueprintResources/StandardMacros.IsValid` (`Animal.SelectedSocket` _controlledpig)
    (:`Is Valid`
      (set `Animal.DistanceToSocket` (`self.GetHorizontalDistanceTo` _controlledpig (`Animal.SelectedSocket` _controlledpig)) (`self.ControlledPig`)))
    (:`Is Not Valid`
      (set `Animal.DistanceToSocket` 10000.0 _controlledpig))))

(event `UpdateArrivalStatus`
  (bind _controlledpig (`self.ControlledPig`))
  ;[1 1 1] Update Arrival Status Method, Check Pig Is Arriving At Target Or Not.
  (if (and (<= (`KismetMathLibrary.VSize` (`self.GetVelocity` (`self.ControlledPig`))) 0.0) (<= (`Animal.DistanceToSocket` _controlledpig) (`Animal.MinArriveDistance` _controlledpig)))
    (set `Animal.IsArriveAtSocket` true _controlledpig)
    (else
      (set `Animal.IsArriveAtSocket` false _controlledpig))))

(event `ReSelectSocket`
  ;[1 1 1] Reselect Socket If Enemy Can't detech Socket.
  (if (`KismetSystemLibrary.IsValid` (`Animal.SelectedSocket` (`self.ControlledPig`)))
    (`self.CheckBestPath`)
    (else
      (`self.SelectBarnSocket`))))

(event `CheckForStucking`
  (bind _controlledpig (`self.ControlledPig`))
  (bind _controlledpig_2 (`self.ControlledPig`))
  (bind _controlledpig_3 (`self.ControlledPig`))
  (bind _controlledpig_4 (`self.ControlledPig`))
  (bind _barn (`Animal.Barn` _controlledpig))
  ;[1 1 1] Check For Stucking Method.
  (if (and (and (not (`Animal.GetAttacked` _controlledpig_4)) (and (and (and (not (`Animal.IsArriveAtSocket` _controlledpig_4)) (<= (`KismetMathLibrary.VSize` (`self.GetVelocity` _controlledpig_4)) 0.0)) (<= (`self.GetDistanceTo` _controlledpig _barn) (`Barn.InRange` _barn))) (`KismetSystemLibrary.IsValid` (`Animal.SelectedSocket` (`self.ControlledPig`))))) (not (`Animal.IsThunderEnchantEffect` (`self.ControlledPig`))))
    (bind _output_get (set `Animal.StuckSeconds` (+ (`Animal.StuckSeconds` _controlledpig_3) (`GameplayStatics.GetWorldDeltaSeconds`)) (`self.ControlledPig`)))
    (if (>= _output_get 1.0)
      (set `Animal.IsStuck` true _controlledpig_2)
      (set `Animal.StuckSeconds` 0.0 _controlledpig_2))
    (else
      (set `Animal.StuckSeconds` 0.0 _controlledpig_3))))

(event `CheckBestPath`
  (bind _controlledpig (`self.ControlledPig`))
  (bind _controlledpig_2 (`self.ControlledPig`))
  (bind _controlledpig_3 (`self.ControlledPig`))
  (bind _controlledpig_4 (`self.ControlledPig`))
  (bind _nearestsocket (`Animal.NearestSocket` _controlledpig_2))
  ;[1 1 1] Reselect Socket If Need
  (if (not (`Animal.IsArriveAtSocket` (`self.ControlledPig`)))
    (if (`KismetStringLibrary.NotEqual_StrStr` (`KismetSystemLibrary.GetDisplayName` (`Animal.NearestSocket` _controlledpig)) (`KismetSystemLibrary.GetDisplayName` (`Animal.SelectedSocket` _controlledpig)))
      (if (`BarnSocket.BeSeleced` (`Animal.NearestSocket` (`self.ControlledPig`)))
        (if (`BarnSocket.Idle` (`Animal.NearestSocket` (`self.ControlledPig`)))
          (bind _asanimal (cast `Animal` (`BarnSocket.CustomerAnimal` _nearestsocket)))
          (if (> (`Animal.DistanceToSocket` _asanimal) (`self.GetDistanceTo` _nearestsocket _controlledpig_2))
            (`/Game/Enemy/Pig/Blueprints/Pig_BP.ReleaseSocket` _asanimal)
            (set `Animal.IsReselected` true _asanimal)
            (bind _asbarn_socket_bp (cast `/Game/Barn/Blueprints/BarnSocket_BP` (`Animal.NearestSocket` _controlledpig_3)))
            (`/Game/Enemy/Pig/Blueprints/Pig_BP.ReleaseSocket` _controlledpig_3)
            (`/Game/Enemy/Pig/Blueprints/Pig_BP.AcquireSocket` _controlledpig_3 _asbarn_socket_bp)
            (set `Animal.IsReselected` true _controlledpig_3)))
        (else
          (`/Game/Enemy/Pig/Blueprints/Pig_BP.ReleaseSocket` _controlledpig_4)
          (bind _asbarn_socket_bp_2 (cast `/Game/Barn/Blueprints/BarnSocket_BP` (`Animal.NearestSocket` _controlledpig_4)))
          (`/Game/Enemy/Pig/Blueprints/Pig_BP.AcquireSocket` _controlledpig_4 _asbarn_socket_bp_2)
          (set `Animal.IsReselected` true _controlledpig_4))))))

(event `GetNearestIdleSocket`
  (bind _index (`self.Index`))
  ;[1 1 1] Get Nearest Socket
  (set `self.MinDis` 100000.0)
  (set `self.Index` -1)
  (bind _outactors (`GameplayStatics.GetAllActorsOfClass` "/Game/Barn/Blueprints/BarnSocket_BP.BarnSocket_BP_C"))
  (for (_array_element _array_index) _outactors
    (if (`BarnSocket.Idle` _array_element)
      (bind _returnvalue (`self.GetDistanceTo` (`self.ControlledPig`) _array_element))
      (if (<= _returnvalue (`self.MinDis`))
        (set `self.MinDis` _returnvalue)
        (set `self.Index` _array_index))))
  (if (>= _index 0)
    (set `Animal.NearestSocket` (`|GetArrayItem` _outactors _index) (`self.ControlledPig`))))

(fn `UserConstructionScript`)