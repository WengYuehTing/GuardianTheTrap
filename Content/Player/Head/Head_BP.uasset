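; Head actor for a VR player that motion controllers can pick up and drop.
; Pickup records the grabbing VRPawn, disables mesh physics and attaches the root to the supplied component, keeping world transform; Drop clears the pawn, re-enables physics and detaches.
; Every tick it passes its own location and rotation to a server-named event that reapplies them, intended to sync the transform across the network.
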(event `UpdatePosAndRot_Server`
  (params (NewLocation :type "Vector Structure") (NewRotation :type "Rotator Structure"))
  ;[1 1 1] Sync Position and Rotation
  (`self.K2_SetActorLocationAndRotation` NewLocation NewRotation))

(event `self.ReceiveTick`
  (params (DeltaSeconds :type "Float (single-precision)"))
  ;[1 1 1] Sync Position and Rotation
  (`self.UpdatePosAndRot_Server` (`self.K2_GetActorLocation`) (`self.K2_GetActorRotation`)))

(event `/Game/VirtualRealityBP/Blueprints/PickupActorInterface.Pickup`
  (params (AttachTo :type "SceneComponent Object Reference"))
  (bind _asvrpawn (cast `/Game/Player/VRPawn` (`ActorComponent.GetOwner` AttachTo)))
  (set `self.PlayerGrabbed` _asvrpawn)
  (`PrimitiveComponent.SetSimulatePhysics` (`self.StaticMesh`) false)
  (`SceneComponent.K2_AttachToComponent` (`self.K2_GetRootComponent`) AttachTo "None" "KeepWorld" "KeepWorld" "KeepWorld" false))

(event `/Game/VirtualRealityBP/Blueprints/PickupActorInterface.Drop`
  (set `self.PlayerGrabbed` null)
  (`PrimitiveComponent.SetSimulatePhysics` (`self.StaticMesh`) true)
  (`self.K2_DetachFromActor` "KeepWorld" "KeepWorld" "KeepWorld"))

(fn `UserConstructionScript`)