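; Grabbable VR pickaxe that mines ore when swung fast enough.
; Pickup attaches it to the motion controller with physics off and records the pawn and controller, and BeginPlay offsets the mesh by its GrabPoint socket.
; Tick sends its transform to the server and tracks per-frame mesh movement as velocity.
; On overlap, the authority calls Ore_BP's Mining if that velocity reaches the speed limit.
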(event `self.ReceiveBeginPlay`
  (bind _staticmesh (`self.StaticMesh`))
  (`SceneComponent.K2_AddWorldOffset` (`self.StaticMesh`) (- (`SceneComponent.K2_GetComponentLocation` _staticmesh) (`SceneComponent.GetSocketLocation` _staticmesh "GrabPoint")) false false))

(event `UpdatePosAndRot_Server`
  (params (NewLocation :type "Vector Structure") (NewRotation :type "Rotator Structure"))
  ;[1 1 1] Sync Position and Rotation
  (`self.K2_SetActorLocationAndRotation` NewLocation NewRotation))

(event `self.ReceiveTick`
  (params (DeltaSeconds :type "Float (single-precision)"))
  (bind _returnvalue (`SceneComponent.K2_GetComponentLocation` (`self.StaticMesh`)))
  (`|ExecutionSequence`
    (:`then_0`
      ;[1 1 1] Sync Position and Rotation
      (`self.UpdatePosAndRot_Server` (`self.K2_GetActorLocation`) (`self.K2_GetActorRotation`)))
    (:`then_1`
      (set `self.VelocityPerFrame` (- _returnvalue (`self.PreviousLocation`)))
      (set `self.PreviousLocation` _returnvalue))))

(event `/Game/VirtualRealityBP/Blueprints/PickupActorInterface.Pickup`
  (params (AttachTo :type "SceneComponent Object Reference"))
  ;[1 0.3928 0] PickUp interface
  (`PrimitiveComponent.SetSimulatePhysics` (`self.StaticMesh`) false)
  (`SceneComponent.K2_AttachToComponent` (`self.K2_GetRootComponent`) AttachTo "None" "KeepWorld" "KeepWorld" "KeepWorld" false)
  (`PrimitiveComponent.SetCollisionResponseToChannel` (`self.StaticMesh`) "ECC_WorldStatic" "ECR_Overlap")
  (bind _asvrpawn (cast `/Game/Player/VRPawn` (`ActorComponent.GetOwner` AttachTo)))
  (set `self.PlayerGrabbed` _asvrpawn)
  (bind _asmotion_controller_component (cast `MotionControllerComponent` AttachTo))
  (set `self.GrabMCComponent` _asmotion_controller_component))

(event `/Game/VirtualRealityBP/Blueprints/PickupActorInterface.Drop`
  ;[1 0.3928 0] PickUp interface
  (`PrimitiveComponent.SetSimulatePhysics` (`self.StaticMesh`) true)
  (`self.K2_DetachFromActor` "KeepWorld" "KeepWorld" "KeepWorld")
  (`PrimitiveComponent.SetCollisionResponseToChannel` (`self.StaticMesh`) "ECC_WorldStatic" "ECR_Block")
  (set `self.PlayerGrabbed` null)
  (set `self.GrabMCComponent` null))

(event `self.StaticMesh.OnComponentBeginOverlap`
  (params (OverlappedComponent :type "PrimitiveComponent Object Reference") (OtherActor :type "Actor Object Reference") (OtherComp :type "PrimitiveComponent Object Reference") (OtherBodyIndex :type Integer) (bFromSweep :type Boolean) (SweepResult :type "HitResult Structure (by ref)"))
  (`/Engine/EditorBlueprintResources/ActorMacros.Switch Has Authority`
    (:`Authority`
      (bind _asore_bp (cast `/Game/Resources/Ore/Ore_BP` OtherActor))
      (if (>= (`KismetMathLibrary.VSize` (`self.VelocityPerFrame`)) (`self.MiningSpeedLimit`))
        (`/Game/Resources/Ore/Ore_BP.Mining` _asore_bp (`self.PlayerGrabbed`) (`self.GrabMCComponent`) (`self.Damage`) (`self.VelocityPerFrame`) (`SceneComponent.K2_GetComponentLocation` (`self.StaticMesh`)))))))

(fn `UserConstructionScript`)