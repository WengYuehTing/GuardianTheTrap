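; BlackRabbit_BP is a rabbit enemy that reacts to fire, ice and thunder enchantment damage.
; Each element event runs a timeline set to the effect duration: burn drains HP and credits the attacking VRPawn, ice slows movement, attacks and animation, and palsy freezes it.
; Multicast calls toggle element bottles, animation speed and a BoostColor material tint combining active elements, reverting as each timeline finishes.
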(event `self.ProcessingBurnDamage`
  (params (`Fire Damage` :type "Float (single-precision)") (Duration :type "Float (single-precision)") (DamageCauser :type "Actor Object Reference"))
  (bind _hp (`self.HP`))
  (bind _returnvalue (* (`GameplayStatics.GetWorldDeltaSeconds`) `Fire Damage`))
  (`self.Multicast Activate ElementBottle` "Fire")
  (bind _asvrpawn (cast `/Game/Player/VRPawn` DamageCauser))
  (bind _result (`/Engine/EditorBlueprintResources/StandardMacros.IncrementFloat` (`self.FireColorBoost`))
    (:`  `
      (`self.Multicast ChangeEnchantColor` (`self.Mesh`) "/Game/Enemy/Rabbit/Models/MI_BlackRabbit.MI_BlackRabbit" "BoostColor" (`KismetMathLibrary.MakeColor` _result (`self.IceColorBoost`) (`self.ThunderColorBoost`)))
      (`TimelineComponent.SetTimelineLength` (`self.Burn`) Duration)
      (`Timeline|Timeline_0` :!via `PlayFromStart`
        (:`Update`
          (if (>= _hp 0.0)
            (set `self.HP` (- _hp _returnvalue))
            (set `/Game/Player/VRPawn.Damage` (+ _returnvalue (`/Game/Player/VRPawn.Damage` _asvrpawn)) _asvrpawn)))
        (:`Finished`
          (set `self.IsFireEnchantEffect` false)
          (set `self.FireColorBoost` 0.0)
          (`self.Multicast ChangeEnchantColor` (`self.Mesh`) "/Game/Enemy/Rabbit/Models/MI_BlackRabbit.MI_BlackRabbit" "BoostColor" (`KismetMathLibrary.MakeColor` 0.0 (`self.IceColorBoost`) (`self.ThunderColorBoost`)))
          (`self.Multicast Deactivate ElementBottle` "Fire"))))))

(event `self.ProcessingIceDamage`
  (params (Duration :type "Float (single-precision)") (DamageCauser :type "Actor Object Reference"))
  (`self.Multicast Activate ElementBottle` "Ice")
  (`TimelineComponent.SetTimelineLength` (`self.Ice`) Duration)
  (bind _result (`/Engine/EditorBlueprintResources/StandardMacros.IncrementFloat` (`self.IceColorBoost`))
    (:`  `
      (`self.Multicast ChangeEnchantColor` (`self.Mesh`) "/Game/Enemy/Rabbit/Models/MI_BlackRabbit.MI_BlackRabbit" "BoostColor" (`KismetMathLibrary.MakeColor` (`self.FireColorBoost`) _result (`self.ThunderColorBoost`)))
      (`Timeline|Timeline_1` :!via `PlayFromStart`
        (:`Update`
          (if (>= (`SkeletalMeshComponent.GlobalAnimRateScale` (`self.Mesh`)) 0.1)
            (set `self.Speed` (/ (`self.MaxSpeed`) 2.0))
            (set `self.AttackSpeed` (* (`self.MaxAttackSpeed`) 2.0))
            (`self.Multicast ChangeAnimationSpeed` 0.5)))
        (:`Finished`
          (set `self.Speed` (`self.MaxSpeed`))
          (set `self.AttackSpeed` (`self.MaxAttackSpeed`))
          (set `self.IsIceEnchantEffect` false)
          (if (>= (`SkeletalMeshComponent.GlobalAnimRateScale` (`self.Mesh`)) 0.1)
            (`self.Multicast ChangeAnimationSpeed` 1.0))
          (set `self.IceColorBoost` 0.0)
          (`self.Multicast ChangeEnchantColor` (`self.Mesh`) "/Game/Enemy/Rabbit/Models/MI_BlackRabbit.MI_BlackRabbit" "BoostColor" (`KismetMathLibrary.MakeColor` (`self.FireColorBoost`) 0.0 (`self.ThunderColorBoost`)))
          (`self.Multicast Deactivate ElementBottle` "Ice"))))))

(event `self.ProcessingPalsy`
  (params (Duration :type "Float (single-precision)") (DamageCauser :type "Actor Object Reference"))
  (`self.Multicast Activate ElementBottle` "Thunder")
  (`self.Multicast ChangeAnimationSpeed` 0.0)
  (bind _result (`/Engine/EditorBlueprintResources/StandardMacros.IncrementFloat` (`self.FireColorBoost`))
    (:`  `
      (bind _result_2 (`/Engine/EditorBlueprintResources/StandardMacros.IncrementFloat` (`self.ThunderColorBoost`))
        (:`  `
          (`self.Multicast ChangeEnchantColor` (`self.Mesh`) "/Game/Enemy/Rabbit/Models/MI_BlackRabbit.MI_BlackRabbit" "BoostColor" (`KismetMathLibrary.MakeColor` _result (`self.IceColorBoost`) _result_2))
          (`TimelineComponent.SetTimelineLength` (`self.Palsy`) Duration)
          (`Timeline|Timeline_2` :!via `PlayFromStart`
            (:`Update`
              (set `self.Speed` 0.0))
            (:`Finished`
              (set `self.Speed` (`self.MaxSpeed`))
              (set `self.IsThunderEnchantEffect` false)
              (`self.Multicast ChangeAnimationSpeed` 1.0)
              (set `self.FireColorBoost` 0.0)
              (set `self.ThunderColorBoost` 0.0)
              (`self.Multicast ChangeEnchantColor` (`self.Mesh`) "/Game/Enemy/Rabbit/Models/MI_BlackRabbit.MI_BlackRabbit" "BoostColor" (`KismetMathLibrary.MakeColor` 0.0 (`self.IceColorBoost`)))
              (`self.Multicast Deactivate ElementBottle` "Thunder"))))))))

(fn `UserConstructionScript`
  (`parent.UserConstructionScript`))