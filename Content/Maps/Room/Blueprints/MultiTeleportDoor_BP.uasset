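; A VR teleport door that starts multiplayer, either hosting or searching for a session according to its Event setting, which also picks its particle effect.
; While a VRPawn stays in the Box, Tick plays audio and darkens the camera through a post-process material instance created every frame.
; After four seconds it calls Host or Search on GTT_GameInstance_BP, guarded by a flag that is never reset here.
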(event `self.ReceiveBeginPlay`
  (bind _particlesystem (`self.ParticleSystem`))
  (switch `/Game/Maps/Room/MultiplayerOptions` (`self.Event`)
    (:`NewEnumerator0`
      (`ParticleSystemComponent.SetTemplate` _particlesystem "/Game/Maps/Room/TeleportParticle/Door_2.Door_2"))
    (:`NewEnumerator1`
      (`ParticleSystemComponent.SetTemplate` _particlesystem "/Game/Maps/Room/TeleportParticle/Door.Door"))))

(event `self.ReceiveTick`
  (params (DeltaSeconds :type "Float (single-precision)"))
  (if (`self.IsPlayerOverlap`)
    (bind _output_get (set `self.StaySeconds` (+ (`self.StaySeconds`) DeltaSeconds)))
    (`|ExecutionSequence`
      (:`then_0`
        (bind _asvrpawn (cast `/Game/Player/VRPawn` (`GameplayStatics.GetPlayerPawn` 0)))
        (bind _returnvalue (`KismetMaterialLibrary.CreateDynamicMaterialInstance` "/Game/Maps/Level1/Shader/PP_CameraDark_Inst.PP_CameraDark_Inst"))
        (`CameraComponent.AddOrUpdateBlendable` (`/Game/Player/VRPawn.VRCamera` _asvrpawn) _returnvalue 1.0)
        (`MaterialInstanceDynamic.SetScalarParameterValue` _returnvalue "DarkScale" (/ _output_get 4.0))
        (if (`self.IsExecuteingOptions`)
          _
          (elif (>= _output_get 4.0)
            (`self.Execute Multiplayer Options`)
            (set `self.IsExecuteingOptions` true))))
      (:`then_1`
        (if (not (`AudioComponent.IsPlaying` (`self.Audio`)))
          (`AudioComponent.Play` (`self.Audio`) 0.0))))
    (else
      (set `self.StaySeconds` 0.0)
      (`AudioComponent.Stop` (`self.Audio`)))))

(event `self.Box.OnComponentBeginOverlap`
  (params (OverlappedComponent :type "PrimitiveComponent Object Reference") (OtherActor :type "Actor Object Reference") (OtherComp :type "PrimitiveComponent Object Reference") (OtherBodyIndex :type Integer) (bFromSweep :type Boolean) (SweepResult :type "HitResult Structure (by ref)"))
  (cast `/Game/Player/VRPawn` OtherActor)
  (set `self.IsPlayerOverlap` true))

(event `self.Box.OnComponentEndOverlap`
  (params (OverlappedComponent :type "PrimitiveComponent Object Reference") (OtherActor :type "Actor Object Reference") (OtherComp :type "PrimitiveComponent Object Reference") (OtherBodyIndex :type Integer))
  (cast `/Game/Player/VRPawn` OtherActor)
  (set `self.IsPlayerOverlap` false))

(event `Execute Multiplayer Options`
  (bind _asgtt_game_instance_bp (cast `/Game/GameInstance/GTT_GameInstance_BP` (`GameplayStatics.GetGameInstance`)))
  (switch `/Game/Maps/Room/MultiplayerOptions` (`self.Event`)
    (:`NewEnumerator0`
      (`/Game/GameInstance/GTT_GameInstance_BP.Host` _asgtt_game_instance_bp))
    (:`NewEnumerator1`
      (`/Game/GameInstance/GTT_GameInstance_BP.Search` _asgtt_game_instance_bp))))

(fn `UserConstructionScript`)