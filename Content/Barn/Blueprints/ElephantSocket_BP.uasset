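; ElephantSocket_BP is an elephant socket actor in the Barn that tracks whether its assigned customer animal is inside its box.
; Box begin and end overlap events pass the other actor to handlers that check it is exactly of class Animal and matches CustomerAnimal.
; A match clears the Idle flag on entry and sets it again on exit, while construction defers to the parent class.
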(event `self.Box.OnComponentBeginOverlap`
  (params (OverlappedComponent :type "PrimitiveComponent Object Reference") (OtherActor :type "Actor Object Reference") (OtherComp :type "PrimitiveComponent Object Reference") (OtherBodyIndex :type Integer) (bFromSweep :type Boolean) (SweepResult :type "HitResult Structure (by ref)"))
  (`self.HandleBeginOverlap` OtherActor))

(event `HandleBeginOverlap`
  (params (`Other Actor` :type "Actor Object Reference"))
  (if (and (== (`GameplayStatics.GetObjectClass` `Other Actor`) "/Script/Guardian_TheTrap.Animal") (== `Other Actor` (`self.CustomerAnimal`)))
    (set `self.Idle` false)))

(event `self.Box.OnComponentEndOverlap`
  (params (OverlappedComponent :type "PrimitiveComponent Object Reference") (OtherActor :type "Actor Object Reference") (OtherComp :type "PrimitiveComponent Object Reference") (OtherBodyIndex :type Integer))
  (`self.HandleEndOverlap` OtherActor))

(event `HandleEndOverlap`
  (params (`Other Actor` :type "Actor Object Reference"))
  (if (and (== (`GameplayStatics.GetObjectClass` `Other Actor`) "/Script/Guardian_TheTrap.Animal") (== `Other Actor` (`self.CustomerAnimal`)))
    (set `self.Idle` true)))

(fn `UserConstructionScript`
  (`parent.UserConstructionScript`))