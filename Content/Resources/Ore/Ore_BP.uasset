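; Mineable ore node that picks one of three mesh and destructible pairs at random on the server.
; Each Mining hit, gated by a short cooldown, plays audio, rumbles the local player's controller and removes one HP.
; On authority, hits spawn a Reward_BP and add Damage to the player's and ResourceManager_BP's ore totals.
; Surviving hits show particles; depletion swaps in a physics-simulated destructible, then destroys the actor after a delay.
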(event `self.ReceiveBeginPlay`
  (`/Engine/EditorBlueprintResources/ActorMacros.Switch Has Authority`
    (:`Authority`
      (switch `int` (`KismetMathLibrary.RandomIntegerInRange` 0 2)
        (:`0`
          (`self.ChangeSkin` "/Game/Resources/Ore/Resources/Ore01.Ore01")
          (set `self.Destructible` "/Game/Resources/Ore/Resources/Ore01_DM.Ore01_DM"))
        (:`1`
          (`self.ChangeSkin` "/Game/Resources/Ore/Resources/Ore02.Ore02")
          (set `self.Destructible` "/Game/Resources/Ore/Resources/Ore02_DM.Ore02_DM"))
        (:`2`
          (`self.ChangeSkin` "/Game/Resources/Ore/Resources/Ore03.Ore03")
          (set `self.Destructible` "/Game/Resources/Ore/Resources/Ore03_DM.Ore03_DM"))))))

(event `ChangeSkin`
  (params (NewMesh :type "StaticMesh Object Reference"))
  (`StaticMeshComponent.SetStaticMesh` (`self.StaticMesh`) NewMesh))

(event `self.ReceiveTick`
  (params (DeltaSeconds :type "Float (single-precision)")))

(event `Mining`
  (params (Player :type "/Game/Player/VRPawn Object Reference") (`MC Component` :type "MotionControllerComponent Object Reference") (Damage :type "Float (double-precision)") (Velocity :type "Vector Structure") (MiningLocation :type "Vector Structure"))
  (bind _miningparticle (`self.MiningParticle`))
  (if (not (`self.BeMining`))
    (`|ExecutionSequence`
      (:`then_0`
        (set `self.BeMining` true)
        (`AudioComponent.Play` (`self.Audio`) 0.0)
        (`/Engine/EditorBlueprintResources/ActorMacros.Switch Has Authority`
          (:`Authority`
            (`self.Server SpawnReward` Player Damage)
            (set `/Game/Player/VRPawn.Ores` (+ (`/Game/Player/VRPawn.Ores` Player) Damage) Player)
            (bind _outactors (`GameplayStatics.GetAllActorsOfClass` "/Game/LevelManager/ResourceManager_BP.ResourceManager_BP_C"))
            (bind _output (`|GetArrayItem` _outactors))
            (set `/Game/LevelManager/ResourceManager_BP.Ores` (+ (`/Game/LevelManager/ResourceManager_BP.Ores` _output) Damage) _output))
          (:`Remote`
            _))
        (bind _output_get (set `self.HP` (- (`self.HP`) 1.0)))
        (if (> _output_get 0.0)
          (`SceneComponent.K2_SetWorldLocation` _miningparticle MiningLocation false false)
          (`ActorComponent.Activate` _miningparticle true)
          (`KismetSystemLibrary.Delay` 0.2)
          (set `self.BeMining` false)
          (else
            (`AudioComponent.Play` (`self.DestroySound`) 0.0)
            (`SceneComponent.SetVisibility` (`self.StaticMesh`) false false)
            (bind _returnvalue (`AddComponent|NODE_AddDestructibleComponent-1` :`RelativeTransform` (`SceneComponent.K2_GetComponentToWorld` (`self.StaticMesh`))))
            (`SceneComponent.K2_AttachToComponent` _returnvalue (`self.StaticMesh`) "None" "KeepRelative" "KeepRelative" "KeepRelative" true)
            (`DestructibleComponent.SetDestructibleMesh` _returnvalue (`self.Destructible`))
            (`SceneComponent.K2_SetWorldTransform` _returnvalue (`self.GetTransform`) false false)
            (`PrimitiveComponent.SetCollisionEnabled` _returnvalue "QueryAndPhysics")
            (`PrimitiveComponent.SetCollisionResponseToAllChannels` _returnvalue "ECR_Block")
            (`PrimitiveComponent.SetSimulatePhysics` _returnvalue true)
            (`PrimitiveComponent.SetEnableGravity` _returnvalue true)
            (`KismetSystemLibrary.Delay` 5.0)
            (`self.K2_DestroyActor`))))
      (:`then_1`
        (if (`Pawn.IsLocallyControlled` Player)
          (`/Game/Player/VRPawn.RumbleController` Player 0.8 `MC Component`))))))

(event `Server SpawnReward`
  (params (`Player Mining` :type "/Game/Player/VRPawn Object Reference") (Damage :type "Float (double-precision)"))
  (bind (_returnvalue_x _returnvalue_y _returnvalue_z) (`KismetMathLibrary.BreakVector` (`self.K2_GetActorLocation`)))
  (`|SpawnActorFromClass` "/Game/Resources/Reward_BP.Reward_BP_C" (`KismetMathLibrary.MakeTransform` (`KismetMathLibrary.MakeVector` _returnvalue_x _returnvalue_y (+ _returnvalue_z 100.0))) "AlwaysSpawn" "OverrideRootScale" `Player Mining` Damage "NewEnumerator2" null))

(fn `UserConstructionScript`)