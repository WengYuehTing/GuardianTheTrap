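; Level manager for a VR barn-defense game that runs animal waves and decides victory or defeat.
; Tick drives a state machine: the authority starts teleport door countdowns, tracks waves, and sets Win once spawning ends and no animals remain, or Lose when barn HP runs out.
; Tick also switches boss and normal fight music, with a barn-health parameter.
; Results reveal the player's teleport door, swap the board mesh and notify the VR widget manager.
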(event `self.ReceiveBeginPlay`
  (`self.Get PlayerTD Ref`)
  (`self.Get Barn Ref`)
  (bind _outactors (`GameplayStatics.GetAllActorsOfClass` "/Game/TeleportDoor/Blueprints/AnimalTeleportDoor_BP.AnimalTeleportDoor_BP_C"))
  (set `self.TotalWave` (`KismetArrayLibrary.Array_Length` (`EnemyTeleport.AnimalsInfo` (`|GetArrayItem` _outactors)))))

(event `self.ReceiveTick`
  (params (DeltaSeconds :type "Float (single-precision)"))
  (bind _barn (`self.Barn`))
  (if (not (`self.IsTakingResult`))
    (`|ExecutionSequence`
      (:`then_0`
        (switch `/Game/LevelManager/ELevelState` (`self.State`)
          (:`NewEnumerator5`
            ;[1 1 1] Start Count Down
            (`/Engine/EditorBlueprintResources/ActorMacros.Switch Has Authority`
              (:`Authority`
                (bind _outactors (`GameplayStatics.GetAllActorsOfClass` "/Game/TeleportDoor/Blueprints/AnimalTeleportDoor_BP.AnimalTeleportDoor_BP_C"))
                (for _array_element _outactors
                  (`/Game/TeleportDoor/Blueprints/AnimalTeleportDoor_BP.StartCountDown` _array_element))
                (if (not (`self.IsChangingWave`))
                  (set `self.WaveIndex` (+ (`self.WaveIndex`) 1))
                  (set `self.IsChangingWave` true)))))
          (:`NewEnumerator4`
            ;[1 1 1] Animal Invade to Waiting
            (`/Engine/EditorBlueprintResources/ActorMacros.Switch Has Authority`
              (:`Authority`
                (set `self.TmpBoolean` false)
                (bind _outactors_2 (`GameplayStatics.GetAllActorsOfClass` "/Game/TeleportDoor/Blueprints/AnimalTeleportDoor_BP.AnimalTeleportDoor_BP_C"))
                (for _array_element_2 _outactors_2
                  (bind _asanimal_teleport_door_bp (cast `/Game/TeleportDoor/Blueprints/AnimalTeleportDoor_BP` _array_element_2))
                  (set `self.TmpBoolean` (or (`self.TmpBoolean`) (`EnemyTeleport.IsStartSpawning` _asanimal_teleport_door_bp))))
                (if (not (`self.TmpBoolean`))
                  (bind _outactors_3 (`GameplayStatics.GetAllActorsOfClass` "/Script/Guardian_TheTrap.Animal"))
                  (if (== (`KismetArrayLibrary.Array_Length` _outactors_3) 0)
                    (set `self.State` "NewEnumerator5")
                    (set `self.IsChangingWave` false)
                    (if (!= (`self.WaveIndex`) (`self.TotalWave`))
                      (`self.Multicast HandleUICommand` "WaveClear" 5.0)))))))
          (:`NewEnumerator2`
            (`self.Win Handle Event`))
          (:`NewEnumerator3`
            (`self.Event Handle Lose`))))
      (:`then_1`
        ;[1 1 1] Determine Win or not
        (`/Engine/EditorBlueprintResources/ActorMacros.Switch Has Authority`
          (:`Authority`
            (bind _outactors_4 (`GameplayStatics.GetAllActorsOfClass` "/Game/TeleportDoor/Blueprints/AnimalTeleportDoor_BP.AnimalTeleportDoor_BP_C"))
            (set `self.TmpBoolean_2` true)
            (for _array_element_3 _outactors_4
              (bind _asanimal_teleport_door_bp_2 (cast `/Game/TeleportDoor/Blueprints/AnimalTeleportDoor_BP` _array_element_3))
              (set `self.TmpBoolean_2` (and (`EnemyTeleport.IsFinishSpawning` _asanimal_teleport_door_bp_2) (`self.TmpBoolean_2`))))
            (if (`self.TmpBoolean_2`)
              (bind _outactors_5 (`GameplayStatics.GetAllActorsOfClass` "/Script/Guardian_TheTrap.Animal"))
              (if (== (`KismetArrayLibrary.Array_Length` _outactors_5) 0)
                (set `self.State` "NewEnumerator2"))))))
      (:`then_2`
        ;[1 1 1] Determine Lose or not
        (`/Engine/EditorBlueprintResources/ActorMacros.Switch Has Authority`
          (:`Authority`
            (bind _outactors_6 (`GameplayStatics.GetAllActorsOfClass` "/Game/Barn/Blueprints/Barn_BP.Barn_BP_C"))
            (if (== (`KismetArrayLibrary.Array_Length` _outactors_6) 0)
              _
              (elif (<= (`Barn.HP` (`|GetArrayItem` _outactors_6)) 0.0)
                (set `self.State` "NewEnumerator3"))))))
      (:`then_3`
        ;[1 1 1] Play Fight Sound
        (bind _outactors_7 (`GameplayStatics.GetAllActorsOfClass` "/Game/Enemy/Elephant/Blueprints/Elephant_BP.Elephant_BP_C"))
        (if (and (> (`KismetArrayLibrary.Array_Length` _outactors_7) 0) (`|EnumInequality` (`self.State`) "NewEnumerator3"))
          (if (`AudioComponent.IsPlaying` (`self.BossFight`))
            _
            (elif (not (`self.IsTakingResult`))
              (`AudioComponent.Play` (`self.BossFight`) 0.0)))
          (elif (`AudioComponent.IsPlaying` (`self.BossFight`))
            (`AudioComponent.Stop` (`self.BossFight`))
            (else
              (bind _outactors_8 (`GameplayStatics.GetAllActorsOfClass` "/Script/Guardian_TheTrap.Animal"))
              (if (> (`KismetArrayLibrary.Array_Length` _outactors_8) 0)
                (`|ExecutionSequence`
                  (:`then_0`
                    (if (`AudioComponent.IsPlaying` (`self.NormalFight`))
                      _
                      (elif (not (`self.IsTakingResult`))
                        (`AudioComponent.Play` (`self.NormalFight`) 0.0))))
                  (:`then_1`
                    (if (>= (/ (`Barn.HP` _barn) (`Barn.MaxHP` _barn)) 0.5)
                      (`AudioComponent.SetIntParameter` (`self.NormalFight`) "BarnHP" 0)
                      (else
                        (`AudioComponent.SetIntParameter` (`self.NormalFight`) "BarnHP" 1)))))
                (elif (`AudioComponent.IsPlaying` (`self.NormalFight`))
                  (`AudioComponent.Stop` (`self.NormalFight`)))))))))))

(event `Multicast HandleUICommand`
  (params (UICommand :type String) (duration :type "Float (double-precision)"))
  ;[1 1 1] Animal Invade to Waiting
  (`AudioComponent.Play` (`self.WaveClear`) 0.0)
  (bind _asvrpawn (cast `/Game/Player/VRPawn` (`GameplayStatics.GetPlayerPawn` 0)))
  (bind _aswidget_manager_bp (cast `/Game/Player/Widgets/information/WidgetManager_BP` (`ChildActorComponent.ChildActor` (`/Game/Player/VRPawn.WidgetManager` _asvrpawn))))
  (`/Game/Player/Widgets/information/WidgetManager_BP.Interface` _aswidget_manager_bp UICommand duration false))

(event `Get Barn Ref`
  (bind _outactors (`GameplayStatics.GetAllActorsOfClass` "/Game/Barn/Blueprints/Barn_BP.Barn_BP_C"))
  (set `self.Barn` (`|GetArrayItem` _outactors)))

(event `Get PlayerTD Ref`
  (bind _outactors (`GameplayStatics.GetAllActorsOfClass` "/Game/LevelManager/PlayerTeleportDoor_BP.PlayerTeleportDoor_BP_C"))
  (set `self.Player Teleport Door` (`|GetArrayItem` _outactors)))

(event `Win Handle Event`
  (set `self.IsTakingResult` true)
  (if (`AudioComponent.IsPlaying` (`self.NormalFight`))
    (`AudioComponent.Stop` (`self.NormalFight`))
    (elif (`AudioComponent.IsPlaying` (`self.BossFight`))
      (`AudioComponent.Stop` (`self.BossFight`))))
  (`AudioComponent.Play` (`self.WinSound`) 0.0)
  (`SceneComponent.SetVisibility` (`/Game/LevelManager/PlayerTeleportDoor_BP.StaticMesh` (`self.Player Teleport Door`)) true true)
  (`StaticMeshComponent.SetStaticMesh` (`self.StaticMesh`) "/Game/LevelManager/Victory.Victory")
  (bind _asvrpawn (cast `/Game/Player/VRPawn` (`GameplayStatics.GetPlayerPawn` 0)))
  (bind _aswidget_manager_bp (cast `/Game/Player/Widgets/information/WidgetManager_BP` (`ChildActorComponent.ChildActor` (`/Game/Player/VRPawn.WidgetManager` _asvrpawn))))
  (`/Game/Player/Widgets/information/WidgetManager_BP.Interface` _aswidget_manager_bp "Win" 5.0 false))

(event `Event Handle Lose`
  (set `self.IsTakingResult` true)
  (if (`AudioComponent.IsPlaying` (`self.NormalFight`))
    (`AudioComponent.Stop` (`self.NormalFight`))
    (elif (`AudioComponent.IsPlaying` (`self.BossFight`))
      (`AudioComponent.Stop` (`self.BossFight`))))
  (`SceneComponent.SetVisibility` (`/Game/LevelManager/PlayerTeleportDoor_BP.StaticMesh` (`self.Player Teleport Door`)) true true)
  (`StaticMeshComponent.SetStaticMesh` (`self.StaticMesh`) "/Game/LevelManager/Failure.Failure")
  (bind _asvrpawn (cast `/Game/Player/VRPawn` (`GameplayStatics.GetPlayerPawn` 0)))
  (bind _aswidget_manager_bp (cast `/Game/Player/Widgets/information/WidgetManager_BP` (`ChildActorComponent.ChildActor` (`/Game/Player/VRPawn.WidgetManager` _asvrpawn))))
  (`/Game/Player/Widgets/information/WidgetManager_BP.Interface` _aswidget_manager_bp "Lose" 5.0 false))

(event `Multicast PlayLevelBGM`
  (`AudioComponent.Play` (`self.LevelBGM`) 0.0))

(event `self.WaveClear.OnAudioFinished`
  (`AudioComponent.Play` (`self.LevelBGM`) 0.0))

(fn `CheckLevel1Achi`
  (returns (`Achi 1` :type Boolean) (`Achi 2` :type Boolean))
  (locals (TotalUsedMoney :type "Float (double-precision)") (`Local Achi1` :type Boolean) (`Local Achi2` :type Boolean :default false))
  (bind _outactors (`GameplayStatics.GetAllActorsOfClass` "/Game/Player/VRPawn.VRPawn_C"))
  (for _array_element _outactors
    (set `local.TotalUsedMoney` (+ (`/Game/Player/VRPawn.MoneyInUsed` _array_element) (`local.TotalUsedMoney`))))
  (set `local.Local Achi2` (<= (`local.TotalUsedMoney`) 300.0))
  (bind _outactors_2 (`GameplayStatics.GetAllActorsOfClass` "/Game/Barn/Blueprints/Barn_BP.Barn_BP_C"))
  (bind _output (`|GetArrayItem` _outactors_2))
  (set `local.Local Achi1` (== (`Barn.HP` _output) (`Barn.MaxHP` _output)))
  (return (`local.Local Achi1`) (`local.Local Achi2`)))

(fn `GetRemainAnimals`
  (returns (amount :type Integer))
  (bind _outactors (`GameplayStatics.GetAllActorsOfClass` "/Script/Guardian_TheTrap.Animal"))
  (return (`KismetArrayLibrary.Array_Length` _outactors)))

(fn `UserConstructionScript`)