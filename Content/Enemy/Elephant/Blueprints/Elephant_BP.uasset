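; Elephant enemy character for a VR game that claims an attack socket, casts a magic attack and skill with multicast effects, and turns its health bar toward the player.
; AnyDamage branches on damage type to reduce HP, credit the attacking pawn's damage and show damage numbers.
; Enchants re-enter as typed damage: fire burns through a timeline, while ice and thunder handlers are empty, their logic left disconnected alongside the stuck-suicide check.
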(event `self.ReceiveTick`
  (params (DeltaSeconds :type "Float (single-precision)"))
  (`|ExecutionSequence`
    (:`then_0`
      (`self.HealthBar face player`))
    (:`then_1`
      (if (`self.IsArriveAtSocket`)
        (if (`self.IsReadyToMagicAttack`)
          (`SceneComponent.SetVisibility` (`self.AttackParticle`) true false)
          (else
            (`SceneComponent.SetVisibility` (`self.AttackParticle`) false false :!label _label)))
        (else
          (set `self.IsReadyToMagicAttack` false)
          (`ActorComponent.Deactivate` (`self.AttackReadyParticle`))
          (goto _label))))
    (:`then_2`
      (`/Engine/EditorBlueprintResources/ActorMacros.Switch Has Authority`
        (:`Authority`
          (`/Engine/EditorBlueprintResources/StandardMacros.IsValid` (`self.Barn`)
            (:`Is Not Valid`
              (if (`AudioComponent.IsPlaying` (`self.AttackSound`))
                (`self.Multicast StopAttackSound`)))))))))

(event `HealthBar face player`
  ;[0.01179 0.6964 1] HealthBar setting
  (bind _asvrpawn (cast `/Game/Player/VRPawn` (`GameplayStatics.GetPlayerPawn` 0)))
  (`SceneComponent.K2_SetWorldRotation` (`self.HealthBar`) (`KismetMathLibrary.FindLookAtRotation` (`SceneComponent.K2_GetComponentLocation` (`self.HealthBar`)) (`SceneComponent.K2_GetComponentLocation` (`/Game/Player/VRPawn.Head` _asvrpawn))) false false))

(event `self.ReceiveBeginPlay`
  (`self.InitHealthBar`))

(event `Multicast UpdateArriveStatus`
  (params (StatusToSet :type Boolean))
  (set `self.IsArriveAtSocket` StatusToSet))

(event `InitHealthBar`
  ;[0.01179 0.6964 1] HealthBar setting
  (bind _asw_animal_health_bar (cast `/Game/Enemy/Widgets/W_AnimalHealthBar` (`WidgetComponent.GetUserWidgetObject` (`self.HealthBar`))))
  (set `/Game/Enemy/Widgets/W_AnimalHealthBar.Animal` self _asw_animal_health_bar))

(event `self.ReceiveDestroyed`
  (`self.ReleaseSocket`))

(event `SetSpeed`
  (params (SpeedToSet :type "Float (double-precision)"))
  (if (not (== SpeedToSet (`self.PreviousSpeed`)))
    (set `CharacterMovementComponent.MaxWalkSpeed` SpeedToSet (`self.CharacterMovement`))
    (set `self.PreviousSpeed` SpeedToSet)))

(event `Multicast PlayBeAttackedSound`
  ;[1 1 1] Sound
  (if (<= (`self.HP`) (/ (`self.MaxHP`) 2.0))
    (`AudioComponent.Play` (`self.AngrySound`) 0.0)
    (else
      (`AudioComponent.Play` (`self.HurtSound`) 0.0))))

(event `AcquireSocket`
  (params (TargetSocket :type "/Game/Barn/Blueprints/BarnSocket_BP Object Reference"))
  (bind _output_get (set `self.SelectedSocket` TargetSocket))
  (set `BarnSocket.BeSeleced` true _output_get)
  (set `self.DistanceToSocket` (`self.GetDistanceTo` _output_get))
  (set `BarnSocket.CustomerAnimal` self _output_get))

(event `self.ReceiveAnyDamage`
  (params (Damage :type "Float (single-precision)") (DamageType :type "DamageType Object Reference") (InstigatedBy :type "Controller Object Reference") (DamageCauser :type "Actor Object Reference"))
  (bind (_returnvalue_x _returnvalue_y _returnvalue_z) (`KismetMathLibrary.BreakVector` (`SceneComponent.K2_GetComponentLocation` (`self.HealthBar`))))
  (bind _returnvalue (`KismetMathLibrary.FClamp` (`self.LocalDamage`) 0.0 (`self.HP`)))
  (bind _returnvalue_2 (`KismetMathLibrary.FClamp` (`self.LocalDamage`) 0.0 (`self.HP`)))
  (bind (_returnvalue_x_2 _returnvalue_y_2 _returnvalue_z_2) (`KismetMathLibrary.BreakVector` (`SceneComponent.K2_GetComponentLocation` (`self.HealthBar`))))
  (set `self.LocalDamage` Damage)
  (set `self.LocalDamageType` DamageType)
  (set `self.LocalDamageCauser` DamageCauser)
  (`|ExecutionSequence`
    (:`then_0`
      (if (== (`GameplayStatics.GetObjectClass` (`self.LocalDamageType`)) "/Game/Enemy/DamageType/NormalDamage_BP.NormalDamage_BP_C")
        (`self.Multicast PlayBeAttackedSound`)
        (bind _asvrpawn (cast `/Game/Player/VRPawn` (`self.LocalDamageCauser`))
          (:`then`
            (set `/Game/Player/VRPawn.Damage` (+ (`/Game/Player/VRPawn.Damage` _asvrpawn) _returnvalue) _asvrpawn))
          (:`CastFailed`
            _))
        (bind _output_get (set `self.HP` (- (`self.HP`) _returnvalue)))
        (`|SpawnActorFromClass` "/Game/Enemy/DamageValue_BP.DamageValue_BP_C" (`KismetMathLibrary.MakeTransform` (`KismetMathLibrary.MakeVector` (+ _returnvalue_x_2 (`KismetMathLibrary.RandomFloatInRange` -15.0 15.0)) (+ _returnvalue_y_2 (`KismetMathLibrary.RandomFloatInRange` -15.0 15.0)) (+ _returnvalue_z_2 (`KismetMathLibrary.RandomFloatInRange` -10.0 5.0)))) "Undefined" "OverrideRootScale" null (`self.LocalDamage`) null)
        (if (<= _output_get (/ (`self.MaxHP`) 2.0))
          (set `self.GetAttacked` true)
          (`KismetSystemLibrary.Delay` (`self.RecoveryCD`))
          (set `self.GetAttacked` false))))
    (:`then_1`
      (if (== (`GameplayStatics.GetObjectClass` (`self.LocalDamageType`)) "/Game/Enemy/DamageType/FireDamage_BP.FireDamage_BP_C")
        (`self.ProcessingBurnDamage` (`self.LocalDamage`) (`self.FireDuration`) (`self.LocalDamageCauser`))))
    (:`then_2`
      (if (== (`GameplayStatics.GetObjectClass` (`self.LocalDamageType`)) "/Game/Enemy/DamageType/IceDamage_BP.IceDamage_BP_C")
        (`self.ProcessingIceDamage` (`self.IceDuration`) (`self.LocalDamageCauser`))))
    (:`then_3`
      (if (== (`GameplayStatics.GetObjectClass` (`self.LocalDamageType`)) "/Game/Enemy/DamageType/ThunderDamage_BP.ThunderDamage_BP_C")
        (`self.ProcessingPalsy` (`self.ThunderDuration`) (`self.LocalDamageCauser`))))
    (:`then_4`
      (if (== (`GameplayStatics.GetObjectClass` (`self.LocalDamageType`)) "/Game/Enemy/DamageType/WeaponDamage_BP.WeaponDamage_BP_C")
        (if (not (`self.IsHurtByWeapon`))
          (set `self.IsHurtByWeapon` true)
          (`self.Multicast PlayBeAttackedSound`)
          (bind _asvrpawn_2 (cast `/Game/Player/VRPawn` (`self.LocalDamageCauser`))
            (:`then`
              (set `/Game/Player/VRPawn.Damage` (+ (`/Game/Player/VRPawn.Damage` _asvrpawn_2) _returnvalue_2) _asvrpawn_2))
            (:`CastFailed`
              _))
          (set `self.HP` (- (`self.HP`) _returnvalue_2))
          (`|SpawnActorFromClass` "/Game/Enemy/DamageValue_BP.DamageValue_BP_C" (`KismetMathLibrary.MakeTransform` (`KismetMathLibrary.MakeVector` (+ _returnvalue_x (`KismetMathLibrary.RandomFloatInRange` -15.0 15.0)) (+ _returnvalue_y (`KismetMathLibrary.RandomFloatInRange` -15.0 15.0)) (+ _returnvalue_z (`KismetMathLibrary.RandomFloatInRange` -10.0 5.0)))) "Undefined" "OverrideRootScale" null (`self.LocalDamage`) null)
          (`KismetSystemLibrary.Delay` (`self.HurtWeaponCD`))
          (set `self.IsHurtByWeapon` false))))))

(event `Multicast PlayDeadSound`
  ;[1 1 1] Sound
  (`AudioComponent.Play` (`self.DeadSound`) 0.3))

(event `Multicast StopAttackSound`
  ;[1 1 1] Sound
  (`AudioComponent.Stop` (`self.AttackSound`)))

(event `/Game/ElementBottle/EnchantableInterface.Enchanted`
  (params (EnchantType :type "EnchantType Enum" :default "Fire") (Duration :type "Float (single-precision)") (Damage :type "Float (single-precision)") (EnchantBottle :type "ElementBottle Object Reference") (Player :type "/Game/Player/VRPawn Object Reference"))
  ;[1 1 1] Enchant
  (switch `EnchantType` EnchantType
    (:`Fire`
      (set `self.FireSufferDamage` Damage)
      (set `self.FireDuration` Duration)
      (`GameplayStatics.ApplyDamage` self (`self.FireSufferDamage`) null Player "/Game/Enemy/DamageType/FireDamage_BP.FireDamage_BP_C")
      (set `self.IsFireEnchantEffect` true))
    (:`Ice`
      (set `self.IceDuration` Duration)
      (`GameplayStatics.ApplyDamage` self Damage null Player "/Game/Enemy/DamageType/IceDamage_BP.IceDamage_BP_C")
      (set `self.IsIceEnchantEffect` true))
    (:`Thunder`
      (set `self.ThunderDuration` Duration)
      (`GameplayStatics.ApplyDamage` self Damage null Player "/Game/Enemy/DamageType/ThunderDamage_BP.ThunderDamage_BP_C")
      (set `self.IsThunderEnchantEffect` true))))

(event `ProcessingBurnDamage`
  (params (`Fire Damage` :type "Float (double-precision)") (Duration :type "Float (double-precision)") (DamageCauser :type "Actor Object Reference"))
  (bind _hp (`self.HP`))
  (bind _returnvalue (* (`GameplayStatics.GetWorldDeltaSeconds`) `Fire Damage`))
  (`self.Multicast Activate ElementBottle` "Fire")
  (bind _asvrpawn (cast `/Game/Player/VRPawn` DamageCauser))
  (bind _result (`/Engine/EditorBlueprintResources/StandardMacros.IncrementFloat` (`self.FireColorBoost`))
    (:`  `
      (`TimelineComponent.SetTimelineLength` (`self.Burn`) Duration)
      (`Timeline|Burn` :!via `PlayFromStart`
        (:`Update`
          (if (>= _hp 0.0)
            (set `self.HP` (- _hp _returnvalue))
            (set `/Game/Player/VRPawn.Damage` (+ _returnvalue (`/Game/Player/VRPawn.Damage` _asvrpawn)) _asvrpawn)))
        (:`Finished`
          (set `self.IsFireEnchantEffect` false)
          (set `self.FireColorBoost` 0.0)
          (`self.Multicast Deactivate ElementBottle` "Fire"))))))

(event `Server SpawnReward`
  (bind (_returnvalue_x _returnvalue_y _returnvalue_z) (`KismetMathLibrary.BreakVector` (`self.K2_GetActorLocation`)))
  (`|SpawnActorFromClass` "/Game/Resources/Reward_BP.Reward_BP_C" (`KismetMathLibrary.MakeTransform` (`KismetMathLibrary.MakeVector` _returnvalue_x _returnvalue_y (+ _returnvalue_z 90.0))) "AlwaysSpawn" "OverrideRootScale" (`self.LocalDamageCauser`) (`self.Reward`) "NewEnumerator0" null))

(event `ProcessingIceDamage`
  (params (Duration :type "Float (double-precision)") (DamageCauser :type "Actor Object Reference")))

(event `Attack`
  ;[1 1 1] Attack
  (`ActorComponent.Activate` (`self.AttackReadyParticle`) true)
  (`AudioComponent.Play` (`self.AttackSound`) 0.0)
  (set `self.IsAttacking` true)
  (`KismetSystemLibrary.Delay` (`self.AttackAnimDuration`))
  (set `self.IsAttacking` false)
  (set `self.IsReadyToMagicAttack` true)
  (`ActorComponent.Activate` (`self.AttackParticle`) true))

(event `Multicast UseSkill`
  ;[1 1 1] Attack
  (`ActorComponent.Activate` (`self.SkillParticle`) false)
  (`AudioComponent.Play` (`self.SkillSound`) 0.0)
  (set `self.IsUsingAlt` true)
  (`KismetSystemLibrary.Delay` 6.2)
  (`SceneComponent.SetHiddenInGame` (`self.MagicFloor`) false true))

(event `ProcessingPalsy`
  (params (Duration :type "Float (double-precision)") (DamageCauser :type "Actor Object Reference")))

(event `Multicast ShowMagicFloor`
  ;[1 1 1] Attack
  (`SceneComponent.SetHiddenInGame` (`self.MagicFloor`) false true))

(event `Multicast FinishUsingSkill`
  ;[1 1 1] Attack
  (set `self.IsUsingAlt` false))

(event `Multicast ChangeAnimationSpeed`
  (params (GlobalAnimRateScale :type "Float (double-precision)"))
  (set `SkeletalMeshComponent.GlobalAnimRateScale` GlobalAnimRateScale (`self.Mesh`)))

(event `Multicast ChangeEnchantColor`
  (params (Target :type "PrimitiveComponent Object Reference") (SourceMaterial :type "MaterialInterface Object Reference") (ParamName :type Name) (Color :type "LinearColor Structure"))
  (bind _returnvalue (`PrimitiveComponent.CreateDynamicMaterialInstance` Target 0 SourceMaterial "None"))
  (`MaterialInstanceDynamic.SetVectorParameterValue` _returnvalue ParamName Color))

(event `Multicast Activate ElementBottle`
  (params (`Enchant Type` :type "EnchantType Enum" :default "Fire"))
  (switch `EnchantType` `Enchant Type`
    (:`Fire`
      (`ActorComponent.Activate` (`self.OnFire`) false))
    (:`Ice`
      (`SceneComponent.SetVisibility` (`self.OnIce`) true false))
    (:`Thunder`
      (`ActorComponent.Activate` (`self.OnPalsy`) false))))

(event `Multicast Deactivate ElementBottle`
  (params (`Enchant Type` :type "EnchantType Enum" :default "Fire"))
  (switch `EnchantType` `Enchant Type`
    (:`Fire`
      (`ActorComponent.Deactivate` (`self.OnFire`)))
    (:`Ice`
      (`SceneComponent.SetVisibility` (`self.OnIce`) false false))
    (:`Thunder`
      (`ActorComponent.Deactivate` (`self.OnPalsy`)))))

(fn `Suicide`
  (returns (StartSuicide :type Boolean))
  (`/Engine/EditorBlueprintResources/ActorMacros.Switch Has Authority`
    (:`Authority`
      (if (or (and (> (`self.GetDistanceTo` (`self.SelectedSocket`)) 500.0) (<= (`KismetMathLibrary.VSize` (`self.GetVelocity`)) 0.0) (not (`self.GetAttacked`)) (not (`self.IsUsingAlt`))) (>= (`KismetMathLibrary.VSize` (`self.GetVelocity`)) 1000.0))
        (bind _output_get (set `self.CurrentSecondsToSuicide` (+ (`self.CurrentSecondsToSuicide`) (`GameplayStatics.GetWorldDeltaSeconds`))))
        (return (>= _output_get (`self.MaxSecondsToSuicide`)))
        (else
          (set `self.CurrentSecondsToSuicide` 0.0))))))

(fn `UserConstructionScript`)