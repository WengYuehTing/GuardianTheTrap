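; Floor plane child actor of the Elephant enemy that gives overlapping animals a speed buff during the Elephant's alt ability.
; On server-side mesh overlap, it checks that the parent Elephant_BP is using alt and that BossStraightRound is visible.
; It then sets the Animal's Speed to 1.5 times MaxSpeed and multicasts a buff particle on Pigs and Rabbits.
; End overlap is empty, so this actor never reverts the boost.
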(event `self.StaticMesh.OnComponentBeginOverlap`
  (params (OverlappedComponent :type "PrimitiveComponent Object Reference") (OtherActor :type "Actor Object Reference") (OtherComp :type "PrimitiveComponent Object Reference") (OtherBodyIndex :type Integer) (bFromSweep :type Boolean) (SweepResult :type "HitResult Structure (by ref)"))
  (`/Engine/EditorBlueprintResources/ActorMacros.Switch Has Authority`
    (:`Authority`
      (bind _aselephant_bp (cast `/Game/Enemy/Elephant/Blueprints/Elephant_BP` (`self.GetParentActor`)))
      (if (`/Game/Enemy/Elephant/Blueprints/Elephant_BP.IsUsingAlt` _aselephant_bp)
        (if (not (`SceneComponent.bHiddenInGame` (`self.BossStraightRound`)))
          (bind _asanimal (cast `Animal` OtherActor))
          (set `Animal.Speed` (* (`Animal.MaxSpeed` _asanimal) 1.5) _asanimal)
          (bind _aspig_bp (cast `/Game/Enemy/Pig/Blueprints/Pig_BP` _asanimal)
            (:`then`
              (`/Game/Enemy/Pig/Blueprints/Pig_BP.Multicast PlayBuffParticle` _aspig_bp))
            (:`CastFailed`
              (bind _asrabbit_bp (cast `/Game/Enemy/Rabbit/Blueprints/Rabbit_BP` _asanimal))
              (`/Game/Enemy/Rabbit/Blueprints/Rabbit_BP.Multicast PlayBuffParticle` _asrabbit_bp))))))))

(event `self.StaticMesh.OnComponentEndOverlap`
  (params (OverlappedComponent :type "PrimitiveComponent Object Reference") (OtherActor :type "Actor Object Reference") (OtherComp :type "PrimitiveComponent Object Reference") (OtherBodyIndex :type Integer)))

(fn `UserConstructionScript`)