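; Multiplayer VR teleport door that opens its target level once every player's VRPawn stays inside its box for a set time.
; The server accumulates a replicated timer while the initially hidden StaticMesh is visible, resetting it when the headcount mismatches, then optionally multicasts a save before travel.
; The timer's OnRep darkens the local VR camera through a post-process blendable.
; Tick also sets the door material to match the destination.
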(event `self.ReceiveBeginPlay`
  (`SceneComponent.SetVisibility` (`self.StaticMesh`) false true))

(event `ChangeSkin`
  (switch `name` (`self.LevelToTeleport`)
    (:`Level01_re2`
      (`PrimitiveComponent.SetMaterial` (`self.Door`) 0 "/Game/NewFolder/TeleporterForPlayer/MI_ToLevel01Teleporter.MI_ToLevel01Teleporter"))
    (:`Level02`
      (`PrimitiveComponent.SetMaterial` (`self.Door`) 0 "/Game/NewFolder/TeleporterForPlayer/MI_ToLevel02Teleporter.MI_ToLevel02Teleporter"))
    (:`Level_03`
      (`PrimitiveComponent.SetMaterial` (`self.Door`) 0 "/Game/NewFolder/TeleporterForPlayer/MI_ToLevel03Teleporter.MI_ToLevel03Teleporter"))
    (:`Hall`
      (`PrimitiveComponent.SetMaterial` (`self.Door`) 0 "/Game/NewFolder/TeleporterForPlayer/MI_ToLevel00Teleporter.MI_ToLevel00Teleporter"))))

(event `self.ReceiveTick`
  (params (DeltaSeconds :type "Float (single-precision)"))
  (`|ExecutionSequence`
    (:`then_0`
      (`/Engine/EditorBlueprintResources/ActorMacros.Switch Has Authority`
        (:`Authority`
          (bind _returnvalue (`GameModeBase.GetNumPlayers` (`GameplayStatics.GetGameMode`)))
          (if (== _returnvalue (`KismetArrayLibrary.Array_Length` (`PrimitiveComponent.GetOverlappingActors` (`self.Box`) "/Game/Player/VRPawn.VRPawn_C")))
            (if (`SceneComponent.IsVisible` (`self.StaticMesh`))
              (set `self.LocalDuration` (+ (`self.LocalDuration`) (`GameplayStatics.GetWorldDeltaSeconds`))))
            (elif (> (`self.LocalDuration`) 0.0)
              (set `self.LocalDuration` 0.0))))))
    (:`then_1`
      (if (>= (`self.LocalDuration`) (`self.StaySecondsToTeleport`))
        (if (`self.AutoSavePS`)
          (`self.Multicast SaveGame`))
        (`/Engine/EditorBlueprintResources/ActorMacros.Switch Has Authority`
          (:`Authority`
            (bind _asvrpawn (cast `/Game/Player/VRPawn` (`GameplayStatics.GetPlayerPawn` 0)))
            (`/Game/Player/VRPawn.Server OpenLevel` _asvrpawn (`self.LevelToTeleport`) false 0.0)))))
    (:`then_2`
      (`self.ChangeSkin`))))

(event `Multicast SaveGame`
  (bind _asgtt_game_instance_bp (cast `/Game/GameInstance/GTT_GameInstance_BP` (`GameplayStatics.GetGameInstance`)))
  (bind _asvrpawn (cast `/Game/Player/VRPawn` (`GameplayStatics.GetPlayerPawn` 0)))
  (`/Game/GameInstance/GTT_GameInstance_BP.Save` _asgtt_game_instance_bp (`/Game/Player/VRPawn.UniqueID` _asvrpawn)))

(fn `OnRep_LocalDuration`
  (bind _asvrpawn (cast `/Game/Player/VRPawn` (`GameplayStatics.GetPlayerPawn` 0)))
  (bind _returnvalue (`KismetMaterialLibrary.CreateDynamicMaterialInstance` "/Game/Maps/Level1/Shader/PP_CameraDark_Inst.PP_CameraDark_Inst"))
  (`CameraComponent.AddOrUpdateBlendable` (`/Game/Player/VRPawn.VRCamera` _asvrpawn) _returnvalue 1.0)
  (`MaterialInstanceDynamic.SetScalarParameterValue` _returnvalue "DarkScale" (`KismetMathLibrary.FClamp` (/ (`self.LocalDuration`) (`self.StaySecondsToTeleport`)))))

(fn `UserConstructionScript`)