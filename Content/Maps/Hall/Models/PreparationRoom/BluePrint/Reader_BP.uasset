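; Preparation-room VR reader that detects a map plate and sets the player teleport door's destination to that plate's level.
; Tick polls the overlap, toggles plate particles and door visibility, and requests on/off through VRPawn server calls.
; Active state, driven by ReaderCanFire's OnRep, shows a player-facing level info widget and ramps material glow.
; OnTeleportFire can open the level, but the all-hands-on-reader trigger is disconnected, though hand overlaps are still tracked.
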(event `self.ReceiveBeginPlay`
  (bind _aslevel_info (cast `/Game/Maps/Hall/Widgets/LevelInfo` (`WidgetComponent.GetUserWidgetObject` (`self.LevelInfo`))))
  (set `/Game/Maps/Hall/Widgets/LevelInfo.Reader` self _aslevel_info)
  (`self.Get PlayerTD Ref`))

(event `self.ReceiveTick`
  (params (DeltaSeconds :type "Float (single-precision)"))
  (bind _returnvalue (`GameplayStatics.GetPlayerPawn` 0))
  (bind _localmapplate (`self.LocalMapPlate`))
  (bind _playerteleportdoor (`self.PlayerTeleportDoor`))
  (bind _overlappingactors (`PrimitiveComponent.GetOverlappingActors` (`self.Active Toggle`) "/Game/Maps/Hall/Models/PreparationRoom/BluePrint/MapPlate_BP.MapPlate_BP_C"))
  (`|ExecutionSequence`
    (:`then_0`
      (`self.LevelInfo face player`))
    (:`then_2`
      (if (!= (`KismetArrayLibrary.Array_Length` _overlappingactors) 0)
        (bind _asvrpawn (cast `/Game/Player/VRPawn` _returnvalue))
        (`/Game/Player/VRPawn.Server TurnOnReader` _asvrpawn self)
        (bind _asmap_plate_bp (cast `/Game/Maps/Hall/Models/PreparationRoom/BluePrint/MapPlate_BP` (`|GetArrayItem` _overlappingactors)))
        (bind _output_get (set `self.LocalMapPlate` _asmap_plate_bp))
        (`ActorComponent.Activate` (`/Game/Maps/Hall/Models/PreparationRoom/BluePrint/MapPlate_BP.ParticleSystem` _output_get) true)
        (set `/Game/Maps/Hall/Models/PreparationRoom/BluePrint/MapPlate_BP.IsActiving` true _output_get)
        (set `/Game/LevelManager/PlayerTeleportDoor_BP.LevelToTeleport` (`KismetStringLibrary.Conv_StringToName` (`/Game/Maps/Hall/Models/PreparationRoom/BluePrint/MapPlate_BP.LevelToTeleport` _output_get)) _playerteleportdoor)
        (`SceneComponent.SetVisibility` (`/Game/LevelManager/PlayerTeleportDoor_BP.StaticMesh` _playerteleportdoor) true true)
        (else
          (`/Engine/EditorBlueprintResources/StandardMacros.IsValid` _localmapplate
            (:`Is Valid`
              (`ActorComponent.Deactivate` (`/Game/Maps/Hall/Models/PreparationRoom/BluePrint/MapPlate_BP.ParticleSystem` _localmapplate))
              (set `/Game/Maps/Hall/Models/PreparationRoom/BluePrint/MapPlate_BP.IsActiving` false _localmapplate)
              (set `self.LocalMapPlate` null))
            (:`Is Not Valid`
              _))
          (bind _asvrpawn_2 (cast `/Game/Player/VRPawn` _returnvalue))
          (`/Game/Player/VRPawn.Server Turnoff Reader` _asvrpawn_2 self)
          (`SceneComponent.SetVisibility` (`/Game/LevelManager/PlayerTeleportDoor_BP.StaticMesh` (`self.PlayerTeleportDoor`)) false true))))
    (:`then_3`
      (if (`self.IsActive`)
        (bind _output_get_2 (set `self.ActiveDuration` (`KismetMathLibrary.FClamp` (+ (`self.ActiveDuration`) (* (`GameplayStatics.GetWorldDeltaSeconds`) (`self.ActiveEffectScale`))) 0.0 6.0)))
        (bind _returnvalue_2 (`PrimitiveComponent.CreateDynamicMaterialInstance` (`self.StaticMesh`) 0 "/Game/Maps/Hall/Models/PreparationRoom/Material/M_Reader_Inst.M_Reader_Inst" "None"))
        (`MaterialInstanceDynamic.SetScalarParameterValue` _returnvalue_2 "ExtraLightingRange" _output_get_2)
        (else
          (bind _output_get_3 (set `self.ActiveDuration` (`KismetMathLibrary.FClamp` (- (`self.ActiveDuration`) (* (`GameplayStatics.GetWorldDeltaSeconds`) (`self.ActiveEffectScale`))) 0.0 6.0)))
          (bind _returnvalue_3 (`PrimitiveComponent.CreateDynamicMaterialInstance` (`self.StaticMesh`) 0 "/Game/Maps/Hall/Models/PreparationRoom/Material/M_Reader_Inst.M_Reader_Inst" "None"))
          (`MaterialInstanceDynamic.SetScalarParameterValue` _returnvalue_3 "ExtraLightingRange" _output_get_3))))))

(event `Get PlayerTD Ref`
  (bind _outactors (`GameplayStatics.GetAllActorsOfClass` "/Game/LevelManager/PlayerTeleportDoor_BP.PlayerTeleportDoor_BP_C"))
  (set `self.PlayerTeleportDoor` (`|GetArrayItem` _outactors)))

(event `OnTeleportFire`
  (if (and (`self.CanTeleport`) (`self.IsActive`))
    (bind _asvrpawn (cast `/Game/Player/VRPawn` (`GameplayStatics.GetPlayerPawn` 0)))
    (set `self.CanTeleport` false)
    (`/Game/Player/VRPawn.Server OpenLevel` _asvrpawn (`KismetStringLibrary.Conv_StringToName` (`/Game/Maps/Hall/Models/PreparationRoom/BluePrint/MapPlate_BP.LevelToTeleport` (`self.LocalMapPlate`))) true (`self.TransitionFadeDuration`))))

(event `Reader Active`
  ;[1 1 1] Reader Active/Deactive
  (if (not (`self.IsActive`))
    (`SceneComponent.SetVisibility` (`self.LevelInfo`) true false)
    (set `self.IsActive` true)))

(event `LevelInfo face player`
  ;[1 1 1] Level Info Widget Always Face to Local Player
  (bind _asvrpawn (cast `/Game/Player/VRPawn` (`GameplayStatics.GetPlayerPawn` 0)))
  (bind (_returnvalue_roll _returnvalue_pitch _returnvalue_yaw) (`KismetMathLibrary.BreakRotator` (`KismetMathLibrary.FindLookAtRotation` (`SceneComponent.K2_GetComponentLocation` (`self.LevelInfo`)) (`SceneComponent.K2_GetComponentLocation` (`/Game/Player/VRPawn.Head` _asvrpawn)))))
  (`SceneComponent.K2_SetWorldRotation` (`self.LevelInfo`) (`KismetMathLibrary.MakeRotator` 0.0 0.0 _returnvalue_yaw) false false))

(event `Reader Deactive`
  ;[1 1 1] Reader Active/Deactive
  (if (`self.IsActive`)
    (`SceneComponent.SetVisibility` (`self.LevelInfo`) false false)
    (set `self.IsActive` false)))

(event `ChangeFlagFromPlayer`
  (params (`Reader Can Fire` :type Boolean))
  ;[1 1 1] Handle Active Toggle Event
  (set `self.ReaderCanFire` `Reader Can Fire`))

(event `self.Teleport Toggle.OnComponentEndOverlap`
  (params (OverlappedComponent :type "PrimitiveComponent Object Reference") (OtherActor :type "Actor Object Reference") (OtherComp :type "PrimitiveComponent Object Reference") (OtherBodyIndex :type Integer))
  ;[1 1 1] Handle Teleport Toggle Event
  (bind _assphere_collision (cast `SphereComponent` OtherComp))
  (`KismetArrayLibrary.Array_RemoveItem` (`self.MCArray`) _assphere_collision))

(event `self.Active Toggle.OnComponentBeginOverlap`
  (params (OverlappedComponent :type "PrimitiveComponent Object Reference") (OtherActor :type "Actor Object Reference") (OtherComp :type "PrimitiveComponent Object Reference") (OtherBodyIndex :type Integer) (bFromSweep :type Boolean) (SweepResult :type "HitResult Structure (by ref)"))
  ;[1 1 1] Handle Active Toggle Event
)

(event `self.Teleport Toggle.OnComponentBeginOverlap`
  (params (OverlappedComponent :type "PrimitiveComponent Object Reference") (OtherActor :type "Actor Object Reference") (OtherComp :type "PrimitiveComponent Object Reference") (OtherBodyIndex :type Integer) (bFromSweep :type Boolean) (SweepResult :type "HitResult Structure (by ref)"))
  ;[1 1 1] Handle Teleport Toggle Event
  (bind _assphere_collision (cast `SphereComponent` OtherComp))
  (for _array_element (`self.MCArray`)
    (if (`KismetStringLibrary.EqualEqual_StrStr` (`KismetSystemLibrary.GetDisplayName` _array_element) (`KismetSystemLibrary.GetDisplayName` _assphere_collision))
      (set `self.MCRepeat` true)
      (break)))
  (if (not (`self.MCRepeat`))
    (`KismetArrayLibrary.Array_Add` (`self.MCArray`) _assphere_collision)))

(event `self.Active Toggle.OnComponentEndOverlap`
  (params (OverlappedComponent :type "PrimitiveComponent Object Reference") (OtherActor :type "Actor Object Reference") (OtherComp :type "PrimitiveComponent Object Reference") (OtherBodyIndex :type Integer))
  ;[1 1 1] Handle Active Toggle Event
)

(fn `OnRep_ReaderCanFire`
  (if (`self.ReaderCanFire`)
    (`self.Reader Active`)
    (else
      (`self.Reader Deactive`))))

(fn `UserConstructionScript`)