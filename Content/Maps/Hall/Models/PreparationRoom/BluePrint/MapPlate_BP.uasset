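; Grabbable map plate for the Hall's preparation room that swaps mesh and material to match its Level on BeginPlay.
; BP_MotionController pickup disables physics and attaches it, drop reverses this, and Tick passes its transform to a server update.
; Hard impacts play a stone sound, throttled by a cooldown.
; The GrowScale activation glow is disconnected and the particle multicast is empty.
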(event `self.ReceiveBeginPlay`
  (`self.ChangeSkin`))

(event `ChangeSkin`
  (bind _staticmesh (`self.StaticMesh`))
  (bind _staticmesh_2 (`self.StaticMesh`))
  (bind _staticmesh_3 (`self.StaticMesh`))
  (switch `/Game/LevelManager/ELevels` (`self.Level`)
    (:`NewEnumerator0`
      (`StaticMeshComponent.SetStaticMesh` _staticmesh_2 "/Game/Maps/Hall/Models/MapPlates/Plate_Level1.Plate_Level1")
      (`PrimitiveComponent.SetMaterial` _staticmesh_2 0 "/Game/Maps/Hall/Models/MapPlates/MI_Plate_Level1.MI_Plate_Level1"))
    (:`NewEnumerator1`
      (`StaticMeshComponent.SetStaticMesh` _staticmesh_3 "/Game/Maps/Hall/Models/MapPlates/Plate_Level2.Plate_Level2")
      (`PrimitiveComponent.SetMaterial` _staticmesh_3 0 "/Game/Maps/Hall/Models/MapPlates/MI_Plate_Level2.MI_Plate_Level2"))
    (:`NewEnumerator2`
      (`StaticMeshComponent.SetStaticMesh` _staticmesh "/Game/Maps/Hall/Models/MapPlates/Plate_Level3.Plate_Level3")
      (`PrimitiveComponent.SetMaterial` _staticmesh 0 "/Game/Maps/Hall/Models/MapPlates/MI_Plate_Level3.MI_Plate_Level3"))))

(event `self.ReceiveTick`
  (params (DeltaSeconds :type "Float (single-precision)"))
  (`|ExecutionSequence`
    (:`then_0`
      (`self.UpdatePosAndRot_Server` (`self.K2_GetActorLocation`) (`self.K2_GetActorRotation`)))))

(event `UpdatePosAndRot_Server`
  (params (NewLocation :type "Vector Structure") (NewRotation :type "Rotator Structure"))
  (`self.K2_SetActorLocationAndRotation` NewLocation NewRotation))

(event `/Game/VirtualRealityBP/Blueprints/PickupActorInterface.Pickup`
  (params (AttachTo :type "SceneComponent Object Reference"))
  (`PrimitiveComponent.SetSimulatePhysics` (`self.StaticMesh`) false)
  (`SceneComponent.K2_AttachToComponent` (`self.K2_GetRootComponent`) AttachTo "None" "KeepWorld" "KeepWorld" "KeepWorld" false)
  (`KismetSystemLibrary.Delay` 1.0)
  (set `self.IsGrabbed` true))

(event `/Game/VirtualRealityBP/Blueprints/PickupActorInterface.Drop`
  (`PrimitiveComponent.SetSimulatePhysics` (`self.StaticMesh`) true)
  (`self.K2_DetachFromActor` "KeepWorld" "KeepWorld" "KeepWorld")
  (set `self.IsGrabbed` false))

(event `self.StaticMesh.OnComponentHit`
  (params (HitComponent :type "PrimitiveComponent Object Reference") (OtherActor :type "Actor Object Reference") (OtherComp :type "PrimitiveComponent Object Reference") (NormalImpulse :type "Vector Structure") (Hit :type "HitResult Structure (by ref)"))
  (bind _staticmesh (`self.StaticMesh`))
  (if (>= (`KismetMathLibrary.VSize` (`SceneComponent.GetComponentVelocity` (`self.StaticMesh`))) 200.0)
    (if (`self.CanPlaySound`)
      (`GameplayStatics.PlaySoundAtLocation` "/Game/Sounds/S_Stone.S_Stone" (`SceneComponent.K2_GetComponentLocation` _staticmesh) (`SceneComponent.K2_GetComponentRotation` _staticmesh) 1.0 1.0 0.0 null null null)
      (set `self.CanPlaySound` false)
      (`KismetSystemLibrary.Delay` (`self.CD`))
      (set `self.CanPlaySound` true))))

(event `Multicast PlayParticle`)

(fn `UserConstructionScript`)