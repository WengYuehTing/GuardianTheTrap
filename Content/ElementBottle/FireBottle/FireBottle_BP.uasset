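; Throwable VR fire bottle that players grab from a belt and throw to spawn a FireZone_BP.
; While simulating physics, hitting an Animal or Floor-tagged component makes the authority multicast the zone spawn and show a cooldown particle at the belt.
; The used bottle is parked out of sight rather than destroyed, then returns to the belt's Fire socket after cooldown.
; HandleEnchant separately applies the enchantment to a target and destroys the bottle.
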(event `self.ReceiveBeginPlay`)

(event `self.ReceiveTick`
  (params (DeltaSeconds :type "Float (single-precision)"))
  (bind _overlappingactors (`PrimitiveComponent.GetOverlappingActors` (`self.StaticMesh`) "/Game/Player/VRPawn.VRPawn_C"))
  (bind _returnvalue (!= (`KismetArrayLibrary.Array_Length` _overlappingactors) 0))
  (`|ExecutionSequence`
    (:`then_0`
      (`self.UpdatePosAndRot_Server` (`self.K2_GetActorLocation`) (`self.K2_GetActorRotation`)))
    (:`then_1`
      (if _returnvalue
        (bind _asvrpawn (cast `/Game/Player/VRPawn` (`|GetArrayItem` _overlappingactors)))
        (set `self.PlayerGrabbed` _asvrpawn)))
    (:`then_2`
      (if _returnvalue
        (`ParticleSystemComponent.SetEmitterEnable` (`self.ParticleSystem`) "PE_Tow" false)
        (else
          (`ParticleSystemComponent.SetEmitterEnable` (`self.ParticleSystem`) "PE_Tow" true))))
    (:`then_3`
      (if (`self.IsUsed`)
        (bind _output_get (set `self.CurDuration` (+ (`self.CurDuration`) (`GameplayStatics.GetWorldDeltaSeconds`))))
        (if (>= _output_get (`self.UsedCD`))
          (set `self.IsUsed` false)
          (bind _asvrpawn_2 (cast `/Game/Player/VRPawn` (`self.GetParentActor`)))
          (bind _belt (`/Game/Player/VRPawn.Belt` _asvrpawn_2))
          (`SceneComponent.K2_SetWorldLocationAndRotation` (`self.StaticMesh`) (`SceneComponent.GetSocketLocation` _belt "Fire") (`SceneComponent.GetSocketRotation` _belt "Fire") false false)
          (`self.K2_AttachToComponent` _belt "None" "KeepWorld" "KeepWorld" "KeepWorld")
          (`PrimitiveComponent.SetCollisionResponseToChannel` (`self.StaticMesh`) "ECC_Pawn" "ECR_Overlap"))
        (else
          (set `self.CurDuration` 0.0))))))

(event `UpdatePosAndRot_Server`
  (params (NewLocation :type "Vector Structure") (NewRotation :type "Rotator Structure"))
  (`self.K2_SetActorLocationAndRotation` NewLocation NewRotation))

(event `/Game/VirtualRealityBP/Blueprints/PickupActorInterface.Pickup`
  (params (AttachTo :type "SceneComponent Object Reference"))
  (`PrimitiveComponent.SetSimulatePhysics` (`self.StaticMesh`) false)
  (`SceneComponent.K2_AttachToComponent` (`self.K2_GetRootComponent`) AttachTo "None" "KeepWorld" "KeepWorld" "KeepWorld" false)
  (`PrimitiveComponent.SetCollisionResponseToChannel` (`self.StaticMesh`) "ECC_Pawn" "ECR_Block"))

(event `/Game/VirtualRealityBP/Blueprints/PickupActorInterface.Drop`
  (`PrimitiveComponent.SetSimulatePhysics` (`self.StaticMesh`) true)
  (`self.K2_DetachFromActor` "KeepWorld" "KeepWorld" "KeepWorld"))

(event `self.StaticMesh.OnComponentHit`
  (params (HitComponent :type "PrimitiveComponent Object Reference") (OtherActor :type "Actor Object Reference") (OtherComp :type "PrimitiveComponent Object Reference") (NormalImpulse :type "Vector Structure") (Hit :type "HitResult Structure (by ref)"))
  (bind (_bblockinghit _binitialoverlap _time _distance _location) (`GameplayStatics.BreakHitResult` Hit))
  (if (`SceneComponent.IsSimulatingPhysics` (`self.StaticMesh`) "None")
    (cast `Animal` OtherActor
      (:`then`
        (`/Engine/EditorBlueprintResources/ActorMacros.Switch Has Authority`
          (:`Authority`
            (`self.Multicast SpawnZone` "/Game/ElementBottle/FireZone/FireZone_BP.FireZone_BP_C" (`KismetMathLibrary.MakeTransform` (`KismetMathLibrary.MakeVector` (.x _location) (.y _location))))
            (bind _asvrpawn (cast `/Game/Player/VRPawn` (`self.GetParentActor`)))
            (bind _returnvalue (`SceneComponent.GetSocketLocation` (`/Game/Player/VRPawn.Belt` _asvrpawn) "Fire"))
            (`self.Spawn CDParticle` _asvrpawn (+ (* (`KismetMathLibrary.Normal` (- (`SceneComponent.K2_GetComponentLocation` (`/Game/Player/VRPawn.VRCamera` _asvrpawn)) _returnvalue)) 10.0) _returnvalue)))))
      (:`CastFailed`
        (if (`ActorComponent.ComponentHasTag` OtherComp "Floor")
          (`/Engine/EditorBlueprintResources/ActorMacros.Switch Has Authority`
            (:`Authority`
              (`self.Multicast SpawnZone` "/Game/ElementBottle/FireZone/FireZone_BP.FireZone_BP_C" (`KismetMathLibrary.MakeTransform` (`.Location` (`GameplayStatics.BreakHitResult` Hit))))
              (`self.Spawn CDParticle` null)
              (bind _asvrpawn_2 (cast `/Game/Player/VRPawn` (`self.GetParentActor`)))
              (bind _returnvalue_2 (`SceneComponent.GetSocketLocation` (`/Game/Player/VRPawn.Belt` _asvrpawn_2) "Fire"))
              (`self.Spawn CDParticle` _asvrpawn_2 (+ (* (`KismetMathLibrary.Normal` (- (`SceneComponent.K2_GetComponentLocation` (`/Game/Player/VRPawn.VRCamera` _asvrpawn_2)) _returnvalue_2)) 10.0) _returnvalue_2)))))))))

(event `self.HandleEnchant`
  (params (Target :type "Actor Object Reference"))
  (`/Engine/EditorBlueprintResources/ActorMacros.Switch Has Authority`
    (:`Authority`
      (bind _asvrpawn (cast `/Game/Player/VRPawn` (`self.PlayerGrabbed`)))
      (message `/Game/ElementBottle/EnchantableInterface.Enchanted` Target (`self.Type`) (`self.EnchantDuration`) (`self.DamagePerSecond`) self _asvrpawn)
      (`self.K2_DestroyActor`))))

(event `Multicast SpawnZone`
  (params (Enchant :type "Actor Class Reference") (SpawnTransform :type "Transform Structure"))
  (`AudioComponent.Play` (`self.S_Firebottlecrack`) 0.0)
  (bind _returnvalue (`|SpawnActorFromClass` Enchant SpawnTransform "AdjustIfPossibleButAlwaysSpawn" "OverrideRootScale" null null))
  (bind _aselement_zone (cast `ElementZone` _returnvalue))
  (set `ElementZone.ElementBottle` self _aselement_zone)
  (`ElementZone.SetupBasicInfo` _aselement_zone)
  (`PrimitiveComponent.SetSimulatePhysics` (`self.StaticMesh`) false)
  (`SceneComponent.K2_SetWorldLocation` (`self.StaticMesh`) (0.0 0.0 1000.0) false false)
  (set `self.IsUsed` true))

(event `Spawn CDParticle`
  (params (Player :type "/Game/Player/VRPawn Object Reference") (Location :type "Vector Structure"))
  ;[1 1 1] Comment
  (`/Engine/EditorBlueprintResources/StandardMacros.IsValid` Player
    (:`Is Valid`
      (`GameplayStatics.SpawnEmitterAttached` "/Game/ElementBottle/P_CD.P_CD" (`/Game/Player/VRPawn.Belt` Player) "None" Location (struct) (0.25 0.25 0.25) "KeepWorldPosition"))))

(fn `UserConstructionScript`)