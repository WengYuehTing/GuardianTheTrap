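; AI controller for the Rabbit enemy that claims and tracks an attack socket around the barn.
; After a short delay it caches the pawn, finds the barn, picks a socket and starts the behavior tree.
; Tick then updates movement state, barn validity, arrival and stuck detection, and re-evaluates the nearest idle socket.
; A closer rabbit can take a claimed idle socket from the animal holding it.
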(event `self.ReceiveBeginPlay`
  (`KismetSystemLibrary.Delay` 0.2)
  ;[1 1 1] Init : Proprecessing property
  (`self.SetControlledRabbitRef`)
  (`self.FindBarn`)
  (`self.SelectBarnSocket`)
  (bind _returnvalue (`self.RunBehaviorTree` "/Game/Enemy/Rabbit/AI/Rabbit_BT.Rabbit_BT"))
  (if _returnvalue
    (`self.UseBlackboard` "/Game/Enemy/Rabbit/AI/Rabbit_BD.Rabbit_BD")
    (set `Animal.SelfAwareness` true (`self.ControlledRabbit`))
    (set `self.InitFinish` true)))

(event `self.ReceiveTick`
  (params (DeltaSeconds :type "Float (single-precision)"))
  (if (`self.InitFinish`)
    ;[1 1 1] RunTime: Update
    (`self.UpdateSpeed`)
    (`self.CheckOnGround`)
    (`self.UpdateBarn`)
    (`/Engine/EditorBlueprintResources/StandardMacros.IsValid` (`Animal.Barn` (`self.ControlledRabbit`))
      (:`Is Valid`
        (`self.CalculateDistance`)
        (`self.UpdateArrivalStatus`)
        (`self.CheckForStucking`)
        (`self.GetNearestIdleSocket`)
        (`self.ReSelectSocket`)))))

(event `SetControlledRabbitRef`
  ;[1 1 1] Get Controlled Pig References
  (bind _asrabbit_bp (cast `/Game/Enemy/Rabbit/Blueprints/Rabbit_BP` (`self.K2_GetPawn`)))
  (set `self.ControlledRabbit` _asrabbit_bp))

(event `FIndBarn`
  ;[1 1 1] Find Barn Method, Set to Controlled Pig Target, And Set Distance Between Pig & Barn.
  (bind _outactors (`GameplayStatics.GetAllActorsOfClass` "/Game/Barn/Blueprints/Barn_BP.Barn_BP_C"))
  (set `Animal.Barn` (`|GetArrayItem` _outactors) (`self.ControlledRabbit`)))

(event `InitHealthBar`
  (bind _controlledrabbit (`self.ControlledRabbit`))
  ;[1 1 1] Init Health Bar
  (bind _asw_animal_health_bar (cast `/Game/Enemy/Widgets/W_AnimalHealthBar` (`WidgetComponent.GetUserWidgetObject` (`/Game/Enemy/Rabbit/Blueprints/Rabbit_BP.HealthBar` _controlledrabbit))))
  (set `/Game/Enemy/Widgets/W_AnimalHealthBar.Animal` _controlledrabbit _asw_animal_health_bar))

(event `SelectBarnSocket`
  (bind _controlledrabbit (`self.ControlledRabbit`))
  (bind _index (`self.Index`))
  ;[1 1 1] Select Barn Socket To Move
  (`/Engine/EditorBlueprintResources/StandardMacros.IsValid` (`Animal.Barn` _controlledrabbit)
    (:`Is Valid`
      (set `self.MinDis` 100000.0)
      (set `self.Index` -1)
      (bind _outactors (`GameplayStatics.GetAllActorsOfClass` "/Game/Barn/Blueprints/BarnSocket_BP.BarnSocket_BP_C"))
      (for (_array_element _array_index) _outactors
        (if (not (`BarnSocket.BeSeleced` _array_element))
          (bind _returnvalue (`self.GetDistanceTo` (`self.ControlledRabbit`) _array_element))
          (if (<= _returnvalue (`self.MinDis`))
            (set `self.MinDis` _returnvalue)
            (set `self.Index` _array_index))
          (elif (`BarnSocket.Idle` _array_element)
            (bind _asanimal (cast `Animal` (`BarnSocket.CustomerAnimal` _array_element)))
            (bind _returnvalue_2 (`self.GetDistanceTo` _array_element (`self.ControlledRabbit`)))
            (if (> (`Animal.DistanceToSocket` _asanimal) _returnvalue_2)
              (set `self.MinDis` _returnvalue_2)
              (set `self.Index` _array_index)))))
      (if (>= _index 0)
        (bind _output (`|GetArrayItem` _outactors _index))
        (if (not (`BarnSocket.BeSeleced` _output))
          (`/Game/Enemy/Rabbit/Blueprints/Rabbit_BP.AcquireSocket` (`self.ControlledRabbit`) _output)
          (else
            (bind _asanimal_2 (cast `Animal` (`BarnSocket.CustomerAnimal` _output)))
            (`/Game/Enemy/Pig/Blueprints/Pig_BP.ReleaseSocket` _asanimal_2)
            (set `Animal.IsReselected` true _asanimal_2)
            (`/Game/Enemy/Rabbit/Blueprints/Rabbit_BP.AcquireSocket` (`self.ControlledRabbit`) _output)))))
    (:`Is Not Valid`
      (set `Animal.SelectedSocket` null _controlledrabbit))))

(event `UpdateSpeed`
  (bind _controlledrabbit (`self.ControlledRabbit`))
  ;[1 1 1] Update Speed Method
  (`/Game/Enemy/Rabbit/Blueprints/Rabbit_BP.SetSpeed` _controlledrabbit (`Animal.Speed` _controlledrabbit)))

(event `CheckOnGround`
  (bind _controlledrabbit (`self.ControlledRabbit`))
  ;[1 1 1] Check Pig is on ground on not
  (set `Animal.IsOnGround` (not (`NavMovementComponent.IsFalling` (`Character.CharacterMovement` _controlledrabbit))) _controlledrabbit))

(event `UpdateBarn`
  (bind _controlledrabbit (`self.ControlledRabbit`))
  ;[1 1 1] Update Barn Info
  (bind _outactors (`GameplayStatics.GetAllActorsOfClass` "/Game/Barn/Blueprints/Barn_BP.Barn_BP_C"))
  (if (== (`KismetArrayLibrary.Array_Length` _outactors) 0)
    (set `Animal.Barn` null _controlledrabbit)
    (`/Game/Enemy/Rabbit/Blueprints/Rabbit_BP.ReleaseSocket` _controlledrabbit)))

(event `CalculateDistance`
  (bind _controlledrabbit (`self.ControlledRabbit`))
  ;[1 1 1] Calculate Pig & Barn Distance
  (`/Engine/EditorBlueprintResources/StandardMacros.IsValid` (`Animal.SelectedSocket` _controlledrabbit)
    (:`Is Valid`
      (set `Animal.DistanceToSocket` (`self.GetHorizontalDistanceTo` _controlledrabbit (`Animal.SelectedSocket` _controlledrabbit)) (`self.ControlledRabbit`)))
    (:`Is Not Valid`
      (set `Animal.DistanceToSocket` 10000.0 _controlledrabbit))))

(event `UpdateArrivalStatus`
  (bind _controlledrabbit (`self.ControlledRabbit`))
  ;[1 1 1] Update Arrival Status Method, Check Pig Is Arriving At Target Or Not.
  (set `Animal.IsArriveAtSocket` (and (<= (`KismetMathLibrary.VSize` (`self.GetVelocity` (`self.ControlledRabbit`))) 0.0) (<= (`Animal.DistanceToSocket` _controlledrabbit) 50.0)) _controlledrabbit))

(event `ReSelectSocket`
  ;[1 1 1] Reselect Socket If Enemy Can't detech Socket.
  (if (`KismetSystemLibrary.IsValid` (`Animal.SelectedSocket` (`self.ControlledRabbit`)))
    (`self.CheckBestPath`)
    (else
      (`self.SelectBarnSocket`))))

(event `CheckForStucking`
  (bind _controlledrabbit (`self.ControlledRabbit`))
  (bind _controlledrabbit_2 (`self.ControlledRabbit`))
  (bind _controlledrabbit_3 (`self.ControlledRabbit`))
  (bind _controlledrabbit_4 (`self.ControlledRabbit`))
  (bind _barn (`Animal.Barn` _controlledrabbit))
  ;[1 1 1] Check For Stucking Method.
  (if (and (and (not (`Animal.GetAttacked` _controlledrabbit_4)) (and (and (and (not (`Animal.IsArriveAtSocket` _controlledrabbit_4)) (<= (`KismetMathLibrary.VSize` (`self.GetVelocity` _controlledrabbit_4)) 0.0)) (<= (`self.GetDistanceTo` _controlledrabbit _barn) (`Barn.InRange` _barn))) (`KismetSystemLibrary.IsValid` (`Animal.SelectedSocket` (`self.ControlledRabbit`))))) (not (`Animal.IsThunderEnchantEffect` (`self.ControlledRabbit`))))
    (bind _output_get (set `Animal.StuckSeconds` (+ (`Animal.StuckSeconds` _controlledrabbit_3) (`GameplayStatics.GetWorldDeltaSeconds`)) (`self.ControlledRabbit`)))
    (if (>= _output_get 1.0)
      (set `Animal.IsStuck` true _controlledrabbit_2)
      (set `Animal.StuckSeconds` 0.0 _controlledrabbit_2))
    (else
      (set `Animal.StuckSeconds` 0.0 _controlledrabbit_3))))

(event `CheckBestPath`
  (bind _controlledrabbit (`self.ControlledRabbit`))
  (bind _controlledrabbit_2 (`self.ControlledRabbit`))
  (bind _controlledrabbit_3 (`self.ControlledRabbit`))
  (bind _controlledrabbit_4 (`self.ControlledRabbit`))
  (bind _nearestsocket (`Animal.NearestSocket` _controlledrabbit_2))
  ;[1 1 1] Reselect Socket If Need
  (if (not (`Animal.IsArriveAtSocket` (`self.ControlledRabbit`)))
    (if (`KismetStringLibrary.NotEqual_StrStr` (`KismetSystemLibrary.GetDisplayName` (`Animal.NearestSocket` _controlledrabbit)) (`KismetSystemLibrary.GetDisplayName` (`Animal.SelectedSocket` _controlledrabbit)))
      (if (`BarnSocket.BeSeleced` (`Animal.NearestSocket` (`self.ControlledRabbit`)))
        (if (`BarnSocket.Idle` (`Animal.NearestSocket` (`self.ControlledRabbit`)))
          (bind _asanimal (cast `Animal` (`BarnSocket.CustomerAnimal` _nearestsocket)))
          (if (> (`Animal.DistanceToSocket` _asanimal) (`self.GetDistanceTo` _nearestsocket _controlledrabbit_2))
            (`Animal.ReleaseSocket` _asanimal)
            (set `Animal.IsReselected` false _asanimal)
            (bind _asbarn_socket_bp (cast `/Game/Barn/Blueprints/BarnSocket_BP` (`Animal.NearestSocket` _controlledrabbit_4)))
            (`/Game/Enemy/Rabbit/Blueprints/Rabbit_BP.ReleaseSocket` _controlledrabbit_4)
            (`/Game/Enemy/Rabbit/Blueprints/Rabbit_BP.AcquireSocket` _controlledrabbit_4 _asbarn_socket_bp)
            (set `Animal.IsReselected` true _controlledrabbit_4)))
        (else
          (`/Game/Enemy/Rabbit/Blueprints/Rabbit_BP.ReleaseSocket` _controlledrabbit_3)
          (bind _asbarn_socket_bp_2 (cast `/Game/Barn/Blueprints/BarnSocket_BP` (`Animal.NearestSocket` _controlledrabbit_3)))
          (`/Game/Enemy/Rabbit/Blueprints/Rabbit_BP.AcquireSocket` _controlledrabbit_3 _asbarn_socket_bp_2)
          (set `Animal.IsReselected` true _controlledrabbit_3))))))

(event `GetNearestIdleSocket`
  (bind _index (`self.Index`))
  ;[1 1 1] Get Nearest Socket
  (set `self.MinDis` 100000.0)
  (set `self.Index` -1)
  (bind _outactors (`GameplayStatics.GetAllActorsOfClass` "/Game/Barn/Blueprints/BarnSocket_BP.BarnSocket_BP_C"))
  (for (_array_element _array_index) _outactors
    (if (`BarnSocket.Idle` _array_element)
      (bind _returnvalue (`self.GetDistanceTo` (`self.ControlledRabbit`) _array_element))
      (if (<= _returnvalue (`self.MinDis`))
        (set `self.MinDis` _returnvalue)
        (set `self.Index` _array_index))))
  (if (>= _index 0)
    (set `Animal.NearestSocket` (`|GetArrayItem` _outactors _index) (`self.ControlledRabbit`))))

(fn `UserConstructionScript`)