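; Spike trap for a VR game that VR players can grab, drop and level up, damaging Animals in its zone.
; An Animal overlap on the server fires it, applying damage with animation, sound and particles, then re-arming after a cooldown if repeating.
; Level, synced from TrapManager at BeginPlay, sets mesh, damage and particles.
; Tick sends its transform to the server, fades in level 1 materials and forces CanGrab true, overriding the LevelManager check.
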(event `self.ReceiveBeginPlay`
  ;[0 0.8148 1] Main BeginPlay
  (`|ExecutionSequence`
    (:`then_0`
      (bind _asvrpawn (cast `/Game/Player/VRPawn` (`self.GetOwner`)))
      (set `self.PlayerSpawned` _asvrpawn)
      (`self.SetOwner` null))
    (:`then_1`
      (`self.Multicast UpdateProperty`))))

(event `/Game/VirtualRealityBP/Blueprints/PickupActorInterface.Pickup`
  (params (AttachTo :type "SceneComponent Object Reference"))
  ;[1 0.4516 0] PickUp Interface Event
  (if (`self.CanGrab`)
    (`PrimitiveComponent.SetSimulatePhysics` (`self.SkeletalMesh`) false)
    (`SceneComponent.K2_AttachToComponent` (`self.K2_GetRootComponent`) AttachTo "None" "KeepWorld" "KeepWorld" "KeepWorld" false)))

(event `UpdatePosAndRot_Server`
  (params (NewLocation :type "Vector Structure") (NewRotation :type "Rotator Structure"))
  ;[1 0.9336 0] Main Tick
  (`self.K2_SetActorLocationAndRotation` NewLocation NewRotation))

(event `self.ReceiveTick`
  (params (DeltaSeconds :type "Float (single-precision)"))
  (bind _returnvalue (+ (`self.LocalFadeInDuration`) (`GameplayStatics.GetWorldDeltaSeconds`)))
  ;[1 0.9336 0] Main Tick
  (`|ExecutionSequence`
    (:`then_0`
      (`self.UpdatePosAndRot_Server` (`self.K2_GetActorLocation`) (`self.K2_GetActorRotation`)))
    (:`then_1`
      ;;[1 1 1] Detect Can Grab or not
      (bind _outactors (`GameplayStatics.GetAllActorsOfClass` "/Game/LevelManager/LevelManager_BP.LevelManager_BP_C"))
      (if (> (`KismetArrayLibrary.Array_Length` _outactors) 0)
        (set `self.CanGrab` (not (`|EnumEquality` (`/Game/LevelManager/LevelManager_BP.State` (`|GetArrayItem` _outactors)) "NewEnumerator4")))))
    (:`then_2`)
    (:`then_3`
      (set `self.CanGrab` true)
      ;;[1 1 1] Fade In Effect
      (`self.FadeInEffect` _returnvalue)
      (set `self.LocalFadeInDuration` _returnvalue))))

(event `/Game/VirtualRealityBP/Blueprints/PickupActorInterface.Drop`
  ;[1 0.4516 0] PickUp Interface Event
  (`PrimitiveComponent.SetSimulatePhysics` (`self.SkeletalMesh`) true)
  (`self.K2_DetachFromActor` "KeepWorld" "KeepWorld" "KeepWorld"))

(event `Multicast Play Activating Sound`
  ;[1 0.9336 0] Main Tick
  (`AudioComponent.Play` (`self.ActivatingSound`) 0.4))

(event `/Game/Trap/HighlightInterface.Highlight`
  ;[0 1 0.2142] Highlight Interface Event
  (if (`self.CanTrigger`)
    (`PrimitiveComponent.SetRenderCustomDepth` (`self.SkeletalMesh`) true)))

(event `/Game/Trap/HighlightInterface.CancelHighlight`
  ;[0 1 0.2142] Highlight Interface Event
  (`PrimitiveComponent.SetRenderCustomDepth` (`self.SkeletalMesh`) false))

(event `self.Activate Zone.OnComponentBeginOverlap`
  (params (OverlappedComponent :type "PrimitiveComponent Object Reference") (OtherActor :type "Actor Object Reference") (OtherComp :type "PrimitiveComponent Object Reference") (OtherBodyIndex :type Integer) (bFromSweep :type Boolean) (SweepResult :type "HitResult Structure (by ref)"))
  ;[1 0 0] Detect Animal
  (`/Engine/EditorBlueprintResources/ActorMacros.Switch Has Authority`
    (:`Authority`
      (cast `Animal` OtherActor)
      (if (`self.CanFire`)
        (set `self.CanFire` false)
        (`self.Fire` (`self.PlayerSpawned`))))))

(event `self.HandleFire`
  (params (Player :type "Pawn Object Reference"))
  ;[1 0 0.008526] Fire Event
  (for _array_element (`PrimitiveComponent.GetOverlappingActors` (`self.Activate Zone`) "/Script/Guardian_TheTrap.Animal")
    (bind _asanimal (cast `Animal` _array_element))
    (`GameplayStatics.ApplyDamage` _asanimal (`self.Damage`) null Player "/Game/Enemy/DamageType/NormalDamage_BP.NormalDamage_BP_C"))
  (`SkeletalMeshComponent.PlayAnimation` (`self.SkeletalMesh`) "/Game/Trap/Spike/Models/Spikes/Spike_L1_Attack.Spike_L1_Attack" false)
  (`self.Multicast Play Activating Sound`)
  (`ActorComponent.Activate` (`self.FireParticle`) true)
  (set `self.IsFire` true)
  (if (`self.CanRepeating`)
    (`KismetSystemLibrary.Delay` (- (`self.CD`) 0.5))
    (`SkeletalMeshComponent.PlayAnimation` (`self.SkeletalMesh`) "/Game/Trap/Spike/Models/Spikes/Spike_L1_TurnBack.Spike_L1_TurnBack" false)
    (`KismetSystemLibrary.Delay` 0.5)
    (set `self.CanFire` true)))

(event `self.HandleLevelUp`
  (bind _level (`self.Level`))
  (bind _skeletalmesh (`self.SkeletalMesh`))
  (bind _skeletalmesh_2 (`self.SkeletalMesh`))
  ;[1 0.7878 0] Level Up
  (if (not (`|EnumEquality` _level (`self.MaxLevel`)))
    (switch `TrapLevel` _level
      (:`Level_1`
        (set `self.Level` "Level_2")
        (`SkinnedMeshComponent.SetSkinnedAssetAndUpdate` _skeletalmesh "/Game/Trap/Spike/Models/Spikes/Spike_L2.Spike_L2" true)
        (`PrimitiveComponent.SetMaterial` _skeletalmesh 0 "/Game/Trap/Materials/MI_SpikeLv2_0.MI_SpikeLv2_0")
        (`PrimitiveComponent.SetMaterial` _skeletalmesh 1 "/Game/Trap/Materials/MI_SpikeLv2_1.MI_SpikeLv2_1")
        (`PrimitiveComponent.SetMaterial` _skeletalmesh 2 "/Game/Trap/Materials/MI_SpikeLv2_2.MI_SpikeLv2_2")
        (set `self.Damage` 70.0)
        (`ActorComponent.Activate` (`self.LevelUp`) true)
        (`ActorComponent.Activate` (`self.Level2Particle`) false))
      (:`Level_2`
        (set `self.Level` "Level_3")
        (`SkinnedMeshComponent.SetSkinnedAssetAndUpdate` _skeletalmesh_2 "/Game/Trap/Spike/Models/Spikes/Spike_L3.Spike_L3" true)
        (`PrimitiveComponent.SetMaterial` _skeletalmesh_2 0 "/Game/Trap/Materials/MI_SpikeLv2_0.MI_SpikeLv2_0")
        (`PrimitiveComponent.SetMaterial` _skeletalmesh_2 1 "/Game/Trap/Materials/MI_SpikeLv2_1.MI_SpikeLv2_1")
        (`PrimitiveComponent.SetMaterial` _skeletalmesh_2 2 "/Game/Trap/Materials/MI_SpikeLv2_2.MI_SpikeLv2_2")
        (set `self.Damage` 100.0)
        (`ActorComponent.Activate` (`self.LevelUp`) true)
        (`ActorComponent.Activate` (`self.Level3Particle`) false)
        (`ActorComponent.Deactivate` (`self.Level2Particle`))))))

(event `Multicast UpdateProperty`
  (bind _skeletalmesh (`self.SkeletalMesh`))
  (bind _skeletalmesh_2 (`self.SkeletalMesh`))
  ;[1 1 1] Update Property When beginplay
  (bind _outactors (`GameplayStatics.GetAllActorsOfClass` "/Game/LevelManager/TrapManager_BP.TrapManager_BP_C"))
  (switch `TrapLevel` (`/Game/LevelManager/TrapManager_BP.SpikeLevel` (`|GetArrayItem` _outactors))
    (:`Level_2`
      (set `self.Level` "Level_2")
      (`SkinnedMeshComponent.SetSkinnedAssetAndUpdate` _skeletalmesh_2 "/Game/Trap/Spike/Models/Spikes/Spike_L2.Spike_L2" true)
      (`PrimitiveComponent.SetMaterial` _skeletalmesh_2 0 "/Game/Trap/Materials/MI_SpikeLv2_0.MI_SpikeLv2_0")
      (`PrimitiveComponent.SetMaterial` _skeletalmesh_2 1 "/Game/Trap/Materials/MI_SpikeLv2_1.MI_SpikeLv2_1")
      (`PrimitiveComponent.SetMaterial` _skeletalmesh_2 2 "/Game/Trap/Materials/MI_SpikeLv2_2.MI_SpikeLv2_2")
      (set `self.Damage` 70.0)
      (`KismetSystemLibrary.Delay` 0.2)
      (`ActorComponent.Activate` (`self.Level2Particle`) false))
    (:`Level_3`
      (set `self.Level` "Level_3")
      (`SkinnedMeshComponent.SetSkinnedAssetAndUpdate` _skeletalmesh "/Game/Trap/Spike/Models/Spikes/Spike_L3.Spike_L3" true)
      (`PrimitiveComponent.SetMaterial` _skeletalmesh 0 "/Game/Trap/Materials/MI_SpikeLv2_0.MI_SpikeLv2_0")
      (`PrimitiveComponent.SetMaterial` _skeletalmesh 1 "/Game/Trap/Materials/MI_SpikeLv2_1.MI_SpikeLv2_1")
      (`PrimitiveComponent.SetMaterial` _skeletalmesh 2 "/Game/Trap/Materials/MI_SpikeLv2_2.MI_SpikeLv2_2")
      (set `self.Damage` 100.0)
      (`KismetSystemLibrary.Delay` 0.2)
      (`ActorComponent.Activate` (`self.Level3Particle`) false)
      (`ActorComponent.Deactivate` (`self.Level2Particle`)))))

(event `FadeInEffect`
  (params (Duration :type "Float (double-precision)"))
  ;[1 1 1] Fade In Effect
  (if (<= Duration 5.0)
    (switch `TrapLevel` (`self.Level`)
      (:`Level_1`
        (bind _returnvalue (`PrimitiveComponent.CreateDynamicMaterialInstance` (`self.SkeletalMesh`) 0 "/Game/Trap/Materials/MI_Spike_0.MI_Spike_0" "None"))
        (`MaterialInstanceDynamic.SetScalarParameterValue` _returnvalue "MaskScale" Duration)
        (bind _returnvalue_2 (`PrimitiveComponent.CreateDynamicMaterialInstance` (`self.SkeletalMesh`) 2 "/Game/Trap/Materials/MI_Spike_1.MI_Spike_1" "None"))
        (`MaterialInstanceDynamic.SetScalarParameterValue` _returnvalue_2 "MaskScale" Duration)
        (bind _returnvalue_3 (`PrimitiveComponent.CreateDynamicMaterialInstance` (`self.SkeletalMesh`) 1 "/Game/Trap/Materials/MI_Spike_2.MI_Spike_2" "None"))
        (`MaterialInstanceDynamic.SetScalarParameterValue` _returnvalue_3 "MaskScale" Duration)))))

(fn `UserConstructionScript`)