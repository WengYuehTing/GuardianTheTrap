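; Resource socket actor that spawns a tree or ore resource at its own transform, chosen by its ResourceType, and respawns it after it is gone.
; On BeginPlay the server spawns the initial resource and stores a reference to it.
; Server-side Tick starts a countdown once that reference becomes invalid, accumulating delta time until the cooldown elapses, then spawns a replacement and resets the timer.
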(event `self.ReceiveBeginPlay`
  (`/Engine/EditorBlueprintResources/ActorMacros.Switch Has Authority`
    (:`Authority`
      (switch `/Game/Resources/EResourceType` (`self.ResourceType`)
        (:`NewEnumerator1`
          (bind _returnvalue (`|SpawnActorFromClass` "/Game/Resources/Wood/Tree_BP.Tree_BP_C" (`self.GetTransform`) "AlwaysSpawn" "OverrideRootScale" null null))
          (set `self.SpawnedResource` _returnvalue))
        (:`NewEnumerator2`
          (bind _returnvalue_2 (`|SpawnActorFromClass` "/Game/Resources/Ore/Ore_BP.Ore_BP_C" (`self.GetTransform`) "AlwaysSpawn" "OverrideRootScale" null null))
          (set `self.SpawnedResource` _returnvalue_2))))))

(event `self.ReceiveTick`
  (params (DeltaSeconds :type "Float (single-precision)"))
  (`/Engine/EditorBlueprintResources/ActorMacros.Switch Has Authority`
    (:`Authority`
      (`|ExecutionSequence`
        (:`then_0`
          (`/Engine/EditorBlueprintResources/StandardMacros.IsValid` (`self.SpawnedResource`)
            (:`Is Not Valid`
              (if (not (`self.IsStartCountDown`))
                (set `self.IsStartCountDown` true)))))
        (:`then_1`
          (if (`self.IsStartCountDown`)
            (bind _output_get (set `self.SpawnDuration` (+ (`self.SpawnDuration`) (`GameplayStatics.GetWorldDeltaSeconds`))))
            (if (>= _output_get (`self.CD`))
              (switch `/Game/Resources/EResourceType` (`self.ResourceType`)
                (:`NewEnumerator1`
                  (bind _returnvalue (`|SpawnActorFromClass` "/Game/Resources/Wood/Tree_BP.Tree_BP_C" (`self.GetTransform`) "AlwaysSpawn" "OverrideRootScale" null null))
                  (set `self.SpawnedResource` _returnvalue)
                  (set `self.SpawnDuration` 0.0)
                  (set `self.IsStartCountDown` false))
                (:`NewEnumerator2`
                  (bind _returnvalue_2 (`|SpawnActorFromClass` "/Game/Resources/Ore/Ore_BP.Ore_BP_C" (`self.GetTransform`) "AlwaysSpawn" "OverrideRootScale" null null))
                  (set `self.SpawnedResource` _returnvalue_2)
                  (set `self.SpawnDuration` 0.0)
                  (set `self.IsStartCountDown` false))))))))))

(fn `UserConstructionScript`)