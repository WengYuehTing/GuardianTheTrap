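; TrapManager is an actor Blueprint that tracks trap upgrade levels and supplies trap resource costs.
; UpdateLevel stores the new level for Spike, Bow or Catcher, then calls LevelUp on every actor of that class in the world.
; LevelMapResource returns Money, Wood and Ore per trap class, varying by level only for Bow and Spike.
; EnumToClass maps the six trap enum values to their Blueprint classes.
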(event `self.ReceiveBeginPlay`)

(event `self.ReceiveTick`
  (params (DeltaSeconds :type "Float (single-precision)")))

(event `UpdateLevel`
  (params (`trap name` :type String) (LevelToSet :type "TrapLevel Enum" :default "Level_1"))
  (switch `string` `trap name`
    (:`Spike`
      (set `self.SpikeLevel` LevelToSet)
      (bind _outactors (`GameplayStatics.GetAllActorsOfClass` "/Game/Trap/Spike/Blueprints/Spike_BP.Spike_BP_C"))
      (for _array_element _outactors
        (`Trap.LevelUp` _array_element)))
    (:`Bow`
      (set `self.BowLevel` LevelToSet)
      (bind _outactors_2 (`GameplayStatics.GetAllActorsOfClass` "/Game/Trap/Bow/Blueprints/Bow_BP.Bow_BP_C"))
      (for _array_element_2 _outactors_2
        (`Trap.LevelUp` _array_element_2)))
    (:`Catcher`
      (set `self.CatcherLevel` LevelToSet)
      (bind _outactors_3 (`GameplayStatics.GetAllActorsOfClass` "/Game/Trap/Catcher/Blueprint/Catcher_BP.Catcher_BP_C"))
      (for _array_element_3 _outactors_3
        (`Trap.LevelUp` _array_element_3)))))

(fn `EnumToClass`
  (params (Trap :type "/Game/Player/Widgets/BubbleMenu/ETrapBubbleType Enum" :default "NewEnumerator0"))
  (returns (Class :type "Trap Class Reference"))
  (switch `/Game/Player/Widgets/BubbleMenu/ETrapBubbleType` Trap
    (:`NewEnumerator0`
      (return "/Game/Trap/Barrel/Blueprints/Barrel_BP.Barrel_BP_C"))
    (:`NewEnumerator1`
      (return "/Game/Trap/Spike/Blueprints/Spike_BP.Spike_BP_C"))
    (:`NewEnumerator2`
      (return "/Game/Trap/Bow/Blueprints/Bow_BP.Bow_BP_C"))
    (:`NewEnumerator3`
      (return "/Game/Trap/Catcher/Blueprint/Catcher_BP.Catcher_BP_C"))
    (:`NewEnumerator4`
      (return "/Game/Trap/Fan/Blueprints/Fan_BP.Fan_BP_C"))
    (:`NewEnumerator5`
      (return "/Game/Trap/Spring/Blueprints/Spring_BP.Spring_BP_C"))))

(fn `LevelMapResource`
  (params (Class :type "Trap Class Reference"))
  (returns (Money :type "Float (double-precision)") (Wood :type "Float (double-precision)") (Ore :type "Float (double-precision)"))
  (if (== Class "/Game/Trap/Bow/Blueprints/Bow_BP.Bow_BP_C")
    (switch `TrapLevel` (`self.BowLevel`)
      (:`Level_1`
        (return 0.0 3.0 1.0))
      (:`Level_2`
        (return 0.0 5.0 2.0))
      (:`Level_3`
        (return 0.0 5.0 3.0)))
    (elif (== Class "/Game/Trap/Catcher/Blueprint/Catcher_BP.Catcher_BP_C")
      (return 0.0 2.0 2.0)
      (elif (== Class "/Game/Trap/Spike/Blueprints/Spike_BP.Spike_BP_C")
        (switch `TrapLevel` (`self.SpikeLevel`)
          (:`Level_1`
            (return 0.0 2.0 3.0))
          (:`Level_2`
            (return 0.0 4.0 4.0))
          (:`Level_3`
            (return 0.0 5.0 7.0)))
        (elif (== Class "/Game/Trap/Fan/Blueprints/Fan_BP.Fan_BP_C")
          (return 0.0 2.0 1.0)
          (elif (== Class "/Game/Trap/Barrel/Blueprints/Barrel_BP.Barrel_BP_C")
            (return 1.0 3.0 0.0)
            (elif (== Class "/Game/Trap/Spring/Blueprints/Spring_BP.Spring_BP_C")
              (return 0.0 1.0 1.0))))))))

(fn `UserConstructionScript`)