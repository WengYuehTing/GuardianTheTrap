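; BP_Barrel is a physics barrel that BP_MotionController can pick up and drop.
; Pickup turns off mesh physics and attaches the barrel to the given component, while Drop restores physics and detaches it.
; Tick passes the current location and rotation every frame to a server update event that sets the actor transform.
; Mesh hits above a speed threshold play an impact sound, gated by a cooldown.
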(event `self.ReceiveTick`
  (params (DeltaSeconds :type "Float (single-precision)"))
  (`self.UpdatePosAndRot_Server` (`self.K2_GetActorLocation`) (`self.K2_GetActorRotation`)))

(event `UpdatePosAndRot_Server`
  (params (NewLocation :type "Vector Structure") (NewRotation :type "Rotator Structure"))
  (`self.K2_SetActorLocationAndRotation` NewLocation NewRotation))

(event `/Game/VirtualRealityBP/Blueprints/PickupActorInterface.Pickup`
  (params (AttachTo :type "SceneComponent Object Reference"))
  (`PrimitiveComponent.SetSimulatePhysics` (`self.StaticMesh`) false)
  (`SceneComponent.K2_AttachToComponent` (`self.K2_GetRootComponent`) AttachTo "None" "KeepWorld" "KeepWorld" "KeepWorld" false))

(event `/Game/VirtualRealityBP/Blueprints/PickupActorInterface.Drop`
  (`PrimitiveComponent.SetSimulatePhysics` (`self.StaticMesh`) true)
  (`self.K2_DetachFromActor` "KeepWorld" "KeepWorld" "KeepWorld"))

(event `self.StaticMesh.OnComponentHit`
  (params (HitComponent :type "PrimitiveComponent Object Reference") (OtherActor :type "Actor Object Reference") (OtherComp :type "PrimitiveComponent Object Reference") (NormalImpulse :type "Vector Structure") (Hit :type "HitResult Structure (by ref)"))
  (if (>= (`KismetMathLibrary.VSize` (`SceneComponent.GetComponentVelocity` (`self.StaticMesh`))) 300.0)
    (if (`self.CanPlaySound`)
      (`AudioComponent.Play` (`self.Audio`) 0.0)
      (set `self.CanPlaySound` false)
      (`KismetSystemLibrary.Delay` (`self.CD`))
      (set `self.CanPlaySound` true))))

(fn `UserConstructionScript`)