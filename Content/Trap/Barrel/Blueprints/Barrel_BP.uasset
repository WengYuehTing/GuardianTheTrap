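; Explosive barrel trap that a VR player can pick up, drop and highlight, detonating when an Animal enters its activation zone.
; Server-side overlap triggers Fire after a delay; HandleFire plays effects and applies distance-scaled damage and outward impulse to nearby animals via a linear Map helper.
; It then re-arms after a cooldown or hides and destroys itself.
; Tick syncs transform to the server and drives a material fade-in on spawn.
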(event `self.ReceiveBeginPlay`
  ;[0 0.8148 1] Main BeginPlay
  (bind _asvrpawn (cast `/Game/Player/VRPawn` (`self.GetOwner`)))
  (set `self.PlayerSpawned` _asvrpawn)
  (`self.SetOwner` null))

(event `UpdatePosAndRot_Server`
  (params (NewLocation :type "Vector Structure") (NewRotation :type "Rotator Structure"))
  ;[1 0.901 0] Main Tick
  ;;[1 1 1] Sync Positon and Rotation
  (`self.K2_SetActorLocationAndRotation` NewLocation NewRotation))

(event `self.ReceiveTick`
  (params (DeltaSeconds :type "Float (single-precision)"))
  (bind _returnvalue (+ (`self.LocalDuration`) (`GameplayStatics.GetWorldDeltaSeconds`)))
  ;[1 0.901 0] Main Tick
  (`|ExecutionSequence`
    (:`then_0`
      ;;[1 1 1] Sync Positon and Rotation
      (`self.UpdatePosAndRot_Server` (`self.K2_GetActorLocation`) (`self.K2_GetActorRotation`)))
    (:`then_1`
      ;;[1 1 1] Fade In Effect
      (`self.FadeInEffect` _returnvalue)
      (set `self.LocalDuration` _returnvalue))
    (:`then_2`
      (set `self.CanGrab` true))))

(event `/Game/VirtualRealityBP/Blueprints/PickupActorInterface.Pickup`
  (params (AttachTo :type "SceneComponent Object Reference"))
  ;[1 0.5145 0] PickUp interface
  (if (`self.CanGrab`)
    (`PrimitiveComponent.SetSimulatePhysics` (`self.Body`) false)
    (`SceneComponent.K2_AttachToComponent` (`self.K2_GetRootComponent`) AttachTo "None" "KeepWorld" "KeepWorld" "KeepWorld" false)))

(event `self.HandleFire`
  (params (Player :type "Pawn Object Reference"))
  (bind _body (`self.Body`))
  ;[1 0 0] Fire Event
  (cast `/Game/Player/VRPawn` Player)
  (`AudioComponent.Play` (`self.ExplosionSound`) 0.0)
  (`ActorComponent.Activate` (`self.FireParticle`) false)
  (bind _outactors (`GameplayStatics.GetAllActorsOfClass` "/Script/Guardian_TheTrap.Animal"))
  (for _array_element _outactors
    (bind _returnvalue (`self.GetHorizontalDistanceTo` _array_element))
    (if (<= _returnvalue (`self.Range`))
      (`GameplayStatics.ApplyDamage` _array_element (`self.Map` _returnvalue 0.0 (`self.Range`) (`self.Damage`)) null (`self.PlayerSpawned`) "/Game/Enemy/DamageType/NormalDamage_BP.NormalDamage_BP_C")
      (`self.FireImpulse` _array_element _returnvalue)))
  (if (`self.CanRepeating`)
    (`KismetSystemLibrary.Delay` (`self.CD`))
    (set `self.CanFire` true)
    (else
      (`SceneComponent.SetVisibility` _body false false)
      (`PrimitiveComponent.SetSimulatePhysics` _body false)
      (`PrimitiveComponent.SetCollisionEnabled` _body "NoCollision")
      (bind _returnvalue_2 (`PrimitiveComponent.CreateDynamicMaterialInstance` (`self.HintZone`) 0 "/Game/Trap/Materials/MI_ActivateZone.MI_ActivateZone" "None"))
      (`MaterialInstanceDynamic.SetScalarParameterValue` _returnvalue_2 "OpacityMultipier" 0.0)
      (`KismetSystemLibrary.Delay` (`self.DeadDelay`))
      (`self.K2_DestroyActor`))))

(event `/Game/VirtualRealityBP/Blueprints/PickupActorInterface.Drop`
  ;[1 0.5145 0] PickUp interface
  (`PrimitiveComponent.SetSimulatePhysics` (`self.Body`) true)
  (`self.K2_DetachFromActor` "KeepWorld" "KeepWorld" "KeepWorld"))

(event `FireImpulse`
  (params (Animal :type "Animal Object Reference") (Distance :type "Float (double-precision)"))
  (bind _charactermovement (`Character.CharacterMovement` Animal))
  ;[1 0 0] Fire Event
  (`/Engine/EditorBlueprintResources/StandardMacros.IsValid` Animal
    (:`Is Valid`
      (if (`Animal.CanBeBounceOff` Animal)
        (`MovementComponent.StopMovementImmediately` _charactermovement)
        (`CharacterMovementComponent.AddImpulse` _charactermovement (* (`KismetMathLibrary.Normal` (- (`self.K2_GetActorLocation`) (`SceneComponent.K2_GetComponentLocation` (`MovementComponent.UpdatedPrimitive` _charactermovement)))) (* (`self.Map` Distance 0.0 (`self.Range`) (`self.ImpulseLength `) 30000.0) -1.0)) false)))))

(event `/Game/Trap/HighlightInterface.Highlight`
  ;[0 1 0.03866] Hightlight interface
  (`PrimitiveComponent.SetRenderCustomDepth` (`self.Body`) true))

(event `/Game/Trap/HighlightInterface.CancelHighlight`
  ;[0 1 0.03866] Hightlight interface
  (`PrimitiveComponent.SetRenderCustomDepth` (`self.Body`) false))

(event `FadeInEffect`
  (params (Duration :type "Float (double-precision)"))
  ;[1 1 1] Fade In Effect
  (if (<= Duration 3.0)
    (bind _returnvalue (`PrimitiveComponent.CreateDynamicMaterialInstance` (`self.Body`) 0 "/Game/Trap/Materials/MI_BombCast.MI_BombCast" "None"))
    (`MaterialInstanceDynamic.SetScalarParameterValue` _returnvalue "MaskScale" Duration)))

(event `self.ActivateZone.OnComponentBeginOverlap`
  (params (OverlappedComponent :type "PrimitiveComponent Object Reference") (OtherActor :type "Actor Object Reference") (OtherComp :type "PrimitiveComponent Object Reference") (OtherBodyIndex :type Integer) (bFromSweep :type Boolean) (SweepResult :type "HitResult Structure (by ref)"))
  ;[1 1 1] Detect Animal Come In
  (`/Engine/EditorBlueprintResources/ActorMacros.Switch Has Authority`
    (:`Authority`
      (cast `Animal` OtherActor)
      (if (`self.CanFire`)
        (set `self.CanFire` false)
        (`KismetSystemLibrary.Delay` (`self.FireDelay`))
        (`self.Fire` (`self.PlayerSpawned`))))))

(fn `Map`
  (params (Value :type "Float (double-precision)") (start1 :type "Float (double-precision)") (stop1 :type "Float (double-precision)") (start2 :type "Float (double-precision)") (stop2 :type "Float (double-precision)"))
  (returns (`target value` :type "Float (double-precision)"))
  (locals (Length1 :type "Float (double-precision)" :default 0.0) (Length2 :type "Float (double-precision)" :default 0.0) (Unit :type "Float (double-precision)" :default 0.0) (SourceLength :type "Float (double-precision)"))
  (set `local.Length1` (- start1 stop1))
  (set `local.Length2` (- start2 stop2))
  (set `local.Unit` (/ (`local.Length2`) (`local.Length1`)))
  (bind _output_get (set `local.SourceLength` (- start1 Value)))
  (return (- start2 (* _output_get (`local.Unit`)))))

(fn `UserConstructionScript`)