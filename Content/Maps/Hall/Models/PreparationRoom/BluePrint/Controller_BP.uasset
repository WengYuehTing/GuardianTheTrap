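; Grabbable color-picker handle in the preparation room that lets a VR player choose a glove color for the hand holding it.
; While held, it follows the hand's horizontal movement, clamped to a radius around its starting point.
; Angle around that origin sets hue and distance sets saturation, updating the glove's dynamic material and the pawn's left or right hand color.
; Each tick it sends its transform through a server update event.
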(event `self.ReceiveBeginPlay`
  (bind _staticmesh (`self.StaticMesh`))
  (set `self.Origin` (`SceneComponent.K2_GetComponentLocation` _staticmesh))
  (set `self.OriginRightVector` (* (`SceneComponent.GetRightVector` _staticmesh) -1.0)))

(event `self.ReceiveTick`
  (params (DeltaSeconds :type "Float (single-precision)"))
  (bind (_returnvalue_x _returnvalue_y _returnvalue_z) (`KismetMathLibrary.BreakVector` (`self.K2_GetActorLocation`)))
  (bind (_returnvalue_x_2 _returnvalue_y_2 _returnvalue_z_2) (`KismetMathLibrary.BreakVector` (`self.K2_GetActorLocation`)))
  (bind _hand (`self.Hand`))
  (bind (_pickuplocation_x _pickuplocation_y) (`KismetMathLibrary.BreakVector` (`self.PickupLocation`)))
  (bind _hand_2 (`self.Hand`))
  (bind _player (`self.Player`))
  (bind (_origin_x _origin_y) (`KismetMathLibrary.BreakVector` (`self.Origin`)))
  (bind (_returnvalue_x_3 _returnvalue_y_3) (`KismetMathLibrary.BreakVector` (`SceneComponent.K2_GetComponentLocation` _hand_2)))
  (bind _returnvalue (`KismetMathLibrary.HSVToRGB` (`self.H`) (`self.S`) 1.0))
  (bind _returnvalue_2 (`KismetMathLibrary.VSizeXY` (- (`self.K2_GetActorLocation`) (`self.Origin`))))
  (bind (_returnvalue_x_4 _returnvalue_y_4) (`KismetMathLibrary.BreakVector` (* (`KismetMathLibrary.Normal` (- (`self.K2_GetActorLocation`) (`self.Origin`))) (`self.Radius`))))
  (`|ExecutionSequence`
    (:`then_0`
      ;[1 1 1] Update Location
      (`/Engine/EditorBlueprintResources/StandardMacros.IsValid` _hand_2
        (:`Is Valid`
          (`SceneComponent.K2_SetWorldLocation` (`self.StaticMesh`) (`KismetMathLibrary.MakeVector` (+ (- _returnvalue_x_3 _pickuplocation_x) _returnvalue_x) (+ (- _returnvalue_y_3 _pickuplocation_y) _returnvalue_y) _returnvalue_z) false false)
          (set `self.PickupLocation` (`SceneComponent.K2_GetComponentLocation` (`self.Hand`))))))
    (:`then_1`
      (set `self.DistanceToOrigin` _returnvalue_2)
      (if (>= _returnvalue_2 (`self.Radius`))
        (`SceneComponent.K2_SetWorldLocation` (`self.StaticMesh`) (`KismetMathLibrary.MakeVector` (+ _origin_x _returnvalue_x_4) (+ _origin_y _returnvalue_y_4) _returnvalue_z_2) false false)
        (set `self.DistanceToOrigin` (`self.Radius`))))
    (:`then_2`
      (set `self.S` (/ (`self.DistanceToOrigin`) (`self.Radius`)))
      (set `self.H` (- (`KismetMathLibrary.DegAtan2` (.x (`self.OriginRightVector`)) (.y (`self.OriginRightVector`))) (`KismetMathLibrary.DegAtan2` (.x (`KismetMathLibrary.Normal` (- (`SceneComponent.K2_GetComponentLocation` (`self.StaticMesh`)) (`self.Origin`)))) (.y (`KismetMathLibrary.Normal` (- (`SceneComponent.K2_GetComponentLocation` (`self.StaticMesh`)) (`self.Origin`))))))))
    (:`then_3`
      (`/Engine/EditorBlueprintResources/StandardMacros.IsValid` _hand
        (:`Is Valid`
          (bind _asskeletal_mesh_component (cast `SkeletalMeshComponent` (`SceneComponent.GetChildComponent` _hand 0)))
          (bind _returnvalue_3 (`PrimitiveComponent.CreateDynamicMaterialInstance` _asskeletal_mesh_component 0 "/Game/Player/Hand/MI_Glove.MI_Glove" "None"))
          (`MaterialInstanceDynamic.SetVectorParameterValue` _returnvalue_3 "Color_1" _returnvalue)
          (if (`KismetStringLibrary.EqualEqual_StrStr` (`KismetSystemLibrary.GetObjectName` _hand) "LeftMotionController")
            (set `/Game/Player/VRPawn.LocalLeftHandColor` _returnvalue _player)
            (else
              (set `/Game/Player/VRPawn.LocalRightHandColor` _returnvalue _player))))))
    (:`then_4`
      ;[1 1 1] Sync Position and Rotation
      (`self.UpdatePosAndRot_Server` (`self.K2_GetActorLocation`) (`self.K2_GetActorRotation`)))))

(event `/Game/VirtualRealityBP/Blueprints/PickupActorInterface.Pickup`
  (params (AttachTo :type "SceneComponent Object Reference"))
  (bind _output_get (set `self.Hand` AttachTo))
  (bind _asvrpawn (cast `/Game/Player/VRPawn` (`ActorComponent.GetOwner` _output_get)))
  (set `self.Player` _asvrpawn)
  (set `self.PickUpLocation` (`SceneComponent.K2_GetComponentLocation` AttachTo)))

(event `/Game/VirtualRealityBP/Blueprints/PickupActorInterface.Drop`
  (set `self.Hand` null)
  (set `self.Player` null))

(event `UpdatePosAndRot_Server`
  (params (NewLocation :type "Vector Structure") (NewRotation :type "Rotator Structure"))
  ;[1 1 1] Sync Position and Rotation
  (`self.K2_SetActorLocationAndRotation` NewLocation NewRotation))

(fn `UserConstructionScript`)