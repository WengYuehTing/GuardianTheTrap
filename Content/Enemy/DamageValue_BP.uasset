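; DamageValue_BP is a floating damage number actor with a W_DamageValue widget, built for the VR player.
; On BeginPlay it hands itself to the widget, scales the font size by clamped Value, and runs a timeline that moves the actor vertically and drives text alpha.
; Each Tick yaws the widget toward the VRPawn's head.
; A DestroyActor node exists but is unconnected, so this graph never removes the actor.
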(event `self.ReceiveBeginPlay`
  (bind (_origin_x _origin_y _origin_z) (`KismetMathLibrary.BreakVector` (`self.Origin`)))
  (`|ExecutionSequence`
    (:`then_0`
      (set `self.Origin` (`self.K2_GetActorLocation`))
      (bind _asw_damage_value (cast `/Game/Enemy/Widgets/W_DamageValue` (`WidgetComponent.GetUserWidgetObject` (`self.Widget`))))
      (set `/Game/Enemy/Widgets/W_DamageValue.DamageValue_BP` self _asw_damage_value)
      (bind (_direction _height _alpha) (`Timeline|Damage1` :!via `PlayFromStart`)
        (:`Update`
          (`self.K2_SetActorLocation` (`KismetMathLibrary.MakeVector` _origin_x _origin_y (+ _origin_z _height)))
          (bind _asw_damage_value_2 (cast `/Game/Enemy/Widgets/W_DamageValue` (`WidgetComponent.GetUserWidgetObject` (`self.Widget`))))
          (set `/Game/Enemy/Widgets/W_DamageValue.TextAlpha` _alpha _asw_damage_value_2))))
    (:`then_1`
      (bind _asw_damage_value_3 (cast `/Game/Enemy/Widgets/W_DamageValue` (`WidgetComponent.GetUserWidgetObject` (`self.Widget`))))
      (bind _text (`/Game/Enemy/Widgets/W_DamageValue.Text` _asw_damage_value_3))
      (bind (_font_fontobject _font_fontmaterial _font_outlinesettings _font_typefacefontname) (break `SlateFontInfo` (`TextBlock.Font` _text)))
      (`TextBlock.SetFont` _text (make `SlateFontInfo` _font_fontobject _font_fontmaterial _font_outlinesettings _font_typefacefontname (`KismetMathLibrary.FTrunc` (`KismetMathLibrary.Lerp` 24.0 48.0 (`KismetMathLibrary.FClamp` (/ (`self.Value`) 100.0)))))))))

(event `self.ReceiveTick`
  (params (DeltaSeconds :type "Float (single-precision)"))
  (bind _asvrpawn (cast `/Game/Player/VRPawn` (`GameplayStatics.GetPlayerPawn` 0)))
  (bind (_returnvalue_roll _returnvalue_pitch _returnvalue_yaw) (`KismetMathLibrary.BreakRotator` (`KismetMathLibrary.FindLookAtRotation` (`SceneComponent.K2_GetComponentLocation` (`self.Widget`)) (`SceneComponent.K2_GetComponentLocation` (`/Game/Player/VRPawn.Head` _asvrpawn)))))
  (`SceneComponent.K2_SetWorldRotation` (`self.Widget`) (`KismetMathLibrary.MakeRotator` 0.0 0.0 _returnvalue_yaw) false false))

(fn `UserConstructionScript`)