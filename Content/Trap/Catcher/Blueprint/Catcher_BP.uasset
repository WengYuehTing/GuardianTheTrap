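; Catcher trap for VR players that damages an Animal entering its ActivateZone, sucks it inward and holds it stuck for a time.
; The authority calls Fire; HandleFire plays effects, applies damage and impulse, then restores speed and re-arms after cooldown if repeatable.
; TrapManager_BP sets the starting level, and level-ups swap mesh, damage and particles.
; It supports motion-controller pickup and highlighting, while Tick syncs its transform to the server and drives a level-one material fade-in.
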(event `self.ReceiveBeginPlay`
  ;[0 0.8853 1] Main BeginPlay
  (`|ExecutionSequence`
    (:`then_0`
      (bind _asvrpawn (cast `/Game/Player/VRPawn` (`self.GetOwner`)))
      (set `self.PlayerSpawned` _asvrpawn)
      (`self.SetOwner` null))
    (:`then_1`
      (`self.Multicast UpdateProperty`))))

(event `self.ReceiveTick`
  (params (DeltaSeconds :type "Float (single-precision)"))
  ;[1 0.9199 0.08081] Main Tick
  (`|ExecutionSequence`
    (:`then_0`
      (`self.UpdatePosAndRot_Server` (`self.K2_GetActorLocation`) (`self.K2_GetActorRotation`)))
    (:`then_1`
      (bind _output_get (set `self.LocalFadeInDuration` (+ (`GameplayStatics.GetWorldDeltaSeconds`) (`self.LocalFadeInDuration`))))
      (`self.FadeInEffect` _output_get))
    (:`then_2`
      (set `self.CanGrab` true))))

(event `UpdatePosAndRot_Server`
  (params (NewLocation :type "Vector Structure") (NewRotation :type "Rotator Structure"))
  ;[1 0.9199 0.08081] Main Tick
  (`self.K2_SetActorLocationAndRotation` NewLocation NewRotation))

(event `/Game/VirtualRealityBP/Blueprints/PickupActorInterface.Pickup`
  (params (AttachTo :type "SceneComponent Object Reference"))
  ;[1 0.5238 0] PickUp interface
  (if (`self.CanGrab`)
    (`PrimitiveComponent.SetSimulatePhysics` (`self.SkeletalMesh`) false)
    (`SceneComponent.K2_AttachToComponent` (`self.K2_GetRootComponent`) AttachTo "None" "KeepWorld" "KeepWorld" "KeepWorld" false)))

(event `/Game/VirtualRealityBP/Blueprints/PickupActorInterface.Drop`
  ;[1 0.5238 0] PickUp interface
  (`PrimitiveComponent.SetSimulatePhysics` (`self.SkeletalMesh`) true)
  (`self.K2_DetachFromActor` "KeepWorld" "KeepWorld" "KeepWorld"))

(event `self.HandleFire`
  (params (Player :type "Pawn Object Reference"))
  (bind _local_animal (`self.Local Animal`))
  (bind _charactermovement (`Character.CharacterMovement` _local_animal))
  (bind (_returnvalue_x _returnvalue_y _returnvalue_z) (`KismetMathLibrary.BreakVector` (* (- (`SceneComponent.K2_GetComponentLocation` (`MovementComponent.UpdatedPrimitive` _charactermovement)) (`self.K2_GetActorLocation`)) -1.0)))
  ;[1 0 0.03758] Fire Event
  (`/Engine/EditorBlueprintResources/StandardMacros.IsValid` Player
    (:`Is Valid`
      (switch `TrapLevel` (`self.Level`)
        (:`Level_1`
          (`SkeletalMeshComponent.PlayAnimation` (`self.SkeletalMesh`) "/Game/Trap/Catcher/Models/CatcherLV2_ani_Anim.CatcherLV2_ani_Anim" false))
        (:`Level_2`
          (`SkeletalMeshComponent.PlayAnimation` (`self.SkeletalMesh`) "/Game/Trap/Catcher/Models/CatcherLV2_ani_Anim.CatcherLV2_ani_Anim" false))
        (:`Level_3`
          (`SkeletalMeshComponent.PlayAnimation` (`self.SkeletalMesh`) "/Game/Trap/Catcher/Models/CatcherLV3_ani_Anim.CatcherLV3_ani_Anim" false)))
      (`AudioComponent.Play` (`self.AvctivateSound`) 0.0)
      (`ActorComponent.Activate` (`self.FireParticle`) true)
      (bind _returnvalue (`PrimitiveComponent.CreateDynamicMaterialInstance` (`self.HintZone`) 0 "/Game/Trap/Materials/MI_ActivateZone.MI_ActivateZone" "None"))
      (`MaterialInstanceDynamic.SetScalarParameterValue` _returnvalue "OpacityMultipier" 0.0)
      (`GameplayStatics.ApplyDamage` _local_animal (`self.Damage`) null (`self.PlayerSpawned`) "/Game/Enemy/DamageType/NormalDamage_BP.NormalDamage_BP_C")
      (`MovementComponent.StopMovementImmediately` _charactermovement)
      (`CharacterMovementComponent.AddImpulse` (`Character.CharacterMovement` _local_animal) (* (`KismetMathLibrary.Normal` (`KismetMathLibrary.MakeVector` _returnvalue_x _returnvalue_y (* _returnvalue_z -1.0))) (`self.SuctionImpulse`)) false)
      (`KismetSystemLibrary.Delay` 0.5)
      (`/Engine/EditorBlueprintResources/StandardMacros.IsValid` _local_animal
        (:`Is Valid`
          (set `Animal.Speed` 0.0 _local_animal)
          (`KismetSystemLibrary.Delay` (`self.StuckSeconds`))
          (`/Engine/EditorBlueprintResources/StandardMacros.IsValid` _local_animal
            (:`Is Valid`
              (set `Animal.Speed` (`Animal.MaxSpeed` _local_animal) _local_animal)
              (`self.Finish`))
            (:`Is Not Valid`
              (`self.Finish` :!label _label))))
        (:`Is Not Valid`
          (goto _label))))))

(event `self.Activate Zone.OnComponentBeginOverlap`
  (params (OverlappedComponent :type "PrimitiveComponent Object Reference") (OtherActor :type "Actor Object Reference") (OtherComp :type "PrimitiveComponent Object Reference") (OtherBodyIndex :type Integer) (bFromSweep :type Boolean) (SweepResult :type "HitResult Structure (by ref)"))
  ;[1 0 0.1059] Overlap Event
  (bind _asanimal (cast `Animal` OtherActor))
  (set `self.Local Animal` _asanimal)
  (if (`self.CanFire`)
    (set `self.CanFire` false)
    (`/Engine/EditorBlueprintResources/ActorMacros.Switch Has Authority`
      (:`Authority`
        (`self.Fire` (`self.PlayerSpawned`))))))

(event `Finish`
  ;[1 0 0.03758] Fire Event
  (if (`self.CanRepeating`)
    (`KismetSystemLibrary.Delay` (`self.CD`))
    (set `self.CanFire` true)))

(event `/Game/Trap/HighlightInterface.Highlight`
  ;[0 1 0.157] Highlight
  (`PrimitiveComponent.SetRenderCustomDepth` (`self.SkeletalMesh`) true))

(event `self.HandleLevelUp`
  (bind _level (`self.Level`))
  (bind _skeletalmesh (`self.SkeletalMesh`))
  (bind _skeletalmesh_2 (`self.SkeletalMesh`))
  ;[1 0.7878 0] Level Up
  (if (not (`|EnumEquality` _level (`self.MaxLevel`)))
    (switch `TrapLevel` _level
      (:`Level_1`
        (set `self.Level` "Level_2")
        (`SkinnedMeshComponent.SetSkinnedAssetAndUpdate` _skeletalmesh "/Game/Trap/Catcher/Models/CatcherLV2_ani.CatcherLV2_ani" true)
        (`PrimitiveComponent.SetMaterial` _skeletalmesh 0 "/Game/Trap/Materials/MI_CatcherLv2_0.MI_CatcherLv2_0")
        (`PrimitiveComponent.SetMaterial` _skeletalmesh 1 "/Game/Trap/Materials/MI_CatcherLv2_1.MI_CatcherLv2_1")
        (`PrimitiveComponent.SetMaterial` _skeletalmesh 2 "/Game/Trap/Materials/MI_CatcherLv2_2.MI_CatcherLv2_2")
        (set `self.Damage` 120.0)
        (`ActorComponent.Activate` (`self.LevelUpParticle`) true)
        (`ActorComponent.Activate` (`self.Level2Particle`) false))
      (:`Level_2`
        (set `self.Level` "Level_3")
        (`SkinnedMeshComponent.SetSkinnedAssetAndUpdate` _skeletalmesh_2 "/Game/Trap/Catcher/Models/CatcherLV3_ani.CatcherLV3_ani" true)
        (`PrimitiveComponent.SetMaterial` _skeletalmesh_2 0 "/Game/Trap/Materials/MI_CatcherLv2_0.MI_CatcherLv2_0")
        (`PrimitiveComponent.SetMaterial` _skeletalmesh_2 1 "/Game/Trap/Materials/MI_CatcherLv2_1.MI_CatcherLv2_1")
        (`PrimitiveComponent.SetMaterial` _skeletalmesh_2 2 "/Game/Trap/Materials/MI_CatcherLv2_2.MI_CatcherLv2_2")
        (set `self.Damage` 200.0)
        (`ActorComponent.Activate` (`self.LevelUpParticle`) true)
        (`ActorComponent.Activate` (`self.Level3Particle`) false)
        (`ActorComponent.Deactivate` (`self.Level2Particle`))))))

(event `/Game/Trap/HighlightInterface.CancelHighlight`
  ;[0 1 0.157] Highlight
  (`PrimitiveComponent.SetRenderCustomDepth` (`self.SkeletalMesh`) false))

(event `Multicast UpdateProperty`
  (bind _skeletalmesh (`self.SkeletalMesh`))
  (bind _skeletalmesh_2 (`self.SkeletalMesh`))
  ;[1 1 1] Update Property When beginplay
  (bind _outactors (`GameplayStatics.GetAllActorsOfClass` "/Game/LevelManager/TrapManager_BP.TrapManager_BP_C"))
  (switch `TrapLevel` (`/Game/LevelManager/TrapManager_BP.CatcherLevel` (`|GetArrayItem` _outactors))
    (:`Level_2`
      (set `self.Level` "Level_2")
      (`SkinnedMeshComponent.SetSkinnedAssetAndUpdate` _skeletalmesh_2 "/Game/Trap/Catcher/Models/CatcherLV2_ani.CatcherLV2_ani" true)
      (`PrimitiveComponent.SetMaterial` _skeletalmesh_2 0 "/Game/Trap/Materials/MI_CatcherLv2_0.MI_CatcherLv2_0")
      (`PrimitiveComponent.SetMaterial` _skeletalmesh_2 1 "/Game/Trap/Materials/MI_CatcherLv2_1.MI_CatcherLv2_1")
      (`PrimitiveComponent.SetMaterial` _skeletalmesh_2 2 "/Game/Trap/Materials/MI_CatcherLv2_2.MI_CatcherLv2_2")
      (set `self.Damage` 120.0)
      (`KismetSystemLibrary.Delay` 0.2)
      (`ActorComponent.Activate` (`self.Level2Particle`) false)
      (`SceneComponent.K2_SetWorldRotation` (`self.Level2Particle`) (struct :`Yaw` 90.0) false false))
    (:`Level_3`
      (set `self.Level` "Level_3")
      (`SkinnedMeshComponent.SetSkinnedAssetAndUpdate` _skeletalmesh "/Game/Trap/Catcher/Models/CatcherLV3_ani.CatcherLV3_ani" true)
      (`PrimitiveComponent.SetMaterial` _skeletalmesh 0 "/Game/Trap/Materials/MI_CatcherLv2_0.MI_CatcherLv2_0")
      (`PrimitiveComponent.SetMaterial` _skeletalmesh 1 "/Game/Trap/Materials/MI_CatcherLv2_1.MI_CatcherLv2_1")
      (`PrimitiveComponent.SetMaterial` _skeletalmesh 2 "/Game/Trap/Materials/MI_CatcherLv2_2.MI_CatcherLv2_2")
      (set `self.Damage` 200.0)
      (`KismetSystemLibrary.Delay` 0.2)
      (`SceneComponent.K2_SetWorldRotation` (`self.Level3Particle`) (struct :`Yaw` 90.0) false false)
      (`ActorComponent.Activate` (`self.Level3Particle`) false)
      (`ActorComponent.Deactivate` (`self.Level2Particle`)))))

(event `FadeInEffect`
  (params (Duration :type "Float (double-precision)"))
  ;[1 1 1] Fade In Effect
  (if (<= Duration 10.0)
    (switch `TrapLevel` (`self.Level`)
      (:`Level_1`
        (bind _returnvalue (`PrimitiveComponent.CreateDynamicMaterialInstance` (`self.SkeletalMesh`) 0 "/Game/Trap/Materials/MI_Catcher_0.MI_Catcher_0" "None"))
        (`MaterialInstanceDynamic.SetScalarParameterValue` _returnvalue "MaskScale" Duration)
        (bind _returnvalue_2 (`PrimitiveComponent.CreateDynamicMaterialInstance` (`self.SkeletalMesh`) 1 "/Game/Trap/Materials/MI_Catcher_1.MI_Catcher_1" "None"))
        (`MaterialInstanceDynamic.SetScalarParameterValue` _returnvalue_2 "MaskScale" Duration)
        (bind _returnvalue_3 (`PrimitiveComponent.CreateDynamicMaterialInstance` (`self.SkeletalMesh`) 2 "/Game/Trap/Materials/MI_Catcher_2.MI_Catcher_2" "None"))
        (`MaterialInstanceDynamic.SetScalarParameterValue` _returnvalue_3 "MaskScale" Duration)))))

(fn `UserConstructionScript`)