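; VR sword that hangs on the player's belt and damages Animals when swung fast enough while held.
; The PickUp interface attaches it to a motion controller; Tick tracks per-frame mesh movement for the server-side overlap hit, which adds rumble and particles.
; When left simulating physics unheld, it glows via emissive timelines, then teleports back to the VRPawn belt socket with particle effects.
; Tick also sends its transform through a server update event.
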(event `self.ReceiveBeginPlay`)

(event `UpdatePosAndRot_Server`
  (params (NewLocation :type "Vector Structure") (NewRotation :type "Rotator Structure"))
  ;[1 1 1] Sync Position and Rotation
  (`self.K2_SetActorLocationAndRotation` NewLocation NewRotation))

(event `self.ReceiveTick`
  (params (DeltaSeconds :type "Float (single-precision)"))
  (bind _staticmesh (`self.StaticMesh`))
  (bind _staticmesh_2 (`self.StaticMesh`))
  (bind _returnvalue (`SceneComponent.K2_GetComponentLocation` (`self.StaticMesh`)))
  (`|ExecutionSequence`
    (:`then_0`
      ;[1 1 1] Sync Position and Rotation
      (`self.UpdatePosAndRot_Server` (`self.K2_GetActorLocation`) (`self.K2_GetActorRotation`)))
    (:`then_1`
      ;[1 1 1] Detect Speed
      (set `self.VelocityPerFrame` (- _returnvalue (`self.PreviousLocation`)))
      (set `self.PreviousLocation` _returnvalue))
    (:`then_2`
      (`/Engine/EditorBlueprintResources/StandardMacros.IsValid` (`self.GrabMCComponent`)
        (:`Is Valid`
          (set `self.NotControlledTime` 0.0))
        (:`Is Not Valid`
          (if (`SceneComponent.IsSimulatingPhysics` (`self.StaticMesh`) "None")
            (bind _output_get (set `self.NotControlledTime` (+ (`self.NotControlledTime`) (`GameplayStatics.GetWorldDeltaSeconds`))))
            (if (>= _output_get 3.0)
              (bind _asvrpawn (cast `/Game/Player/VRPawn` (`self.GetParentActor`)))
              (`/Engine/EditorBlueprintResources/ActorMacros.Switch Has Authority`
                (:`Authority`
                  (`/Game/Player/VRPawn.Server SpawnEmitter` _asvrpawn "/Game/Player/Belt/Material/P_ToolsAppear.P_ToolsAppear" (`SceneComponent.K2_GetComponentLocation` _staticmesh) (`SceneComponent.K2_GetComponentRotation` _staticmesh) (1.0 1.0 1.0) true))
                (:`Remote`
                  _))
              (bind _belt (`/Game/Player/VRPawn.Belt` _asvrpawn))
              (`SceneComponent.K2_SetWorldLocationAndRotation` (`self.StaticMesh`) (`SceneComponent.GetSocketLocation` _belt "Sword") (`SceneComponent.GetSocketRotation` _belt "Sword") false false)
              (`/Engine/EditorBlueprintResources/ActorMacros.Switch Has Authority`
                (:`Authority`
                  (`/Game/Player/VRPawn.Server SpawnEmitter` _asvrpawn "/Game/Player/Belt/Material/P_ToolsAppear.P_ToolsAppear" (`SceneComponent.K2_GetComponentLocation` _staticmesh_2) (`SceneComponent.K2_GetComponentRotation` _staticmesh_2) (1.0 1.0 1.0) true))
                (:`Remote`
                  _))
              (`PrimitiveComponent.SetSimulatePhysics` (`self.StaticMesh`) false)
              (`self.K2_AttachToComponent` _belt "None" "KeepWorld" "KeepWorld" "KeepWorld")
              (`/Engine/EditorBlueprintResources/ActorMacros.Switch Has Authority`
                (:`Authority`
                  (`self.ToBecomeOriginal`)))
              (elif (>= _output_get 2.0)
                (`/Engine/EditorBlueprintResources/ActorMacros.Switch Has Authority`
                  (:`Authority`
                    (`self.ToShine`)))))
            (else
              (set `self.NotControlledTime` 0.0))))))))

(event `/Game/VirtualRealityBP/Blueprints/PickupActorInterface.Pickup`
  (params (AttachTo :type "SceneComponent Object Reference"))
  ;[1 0.3928 0] PickUp interface
  (`PrimitiveComponent.SetSimulatePhysics` (`self.StaticMesh`) false)
  (`SceneComponent.K2_AttachToComponent` (`self.K2_GetRootComponent`) AttachTo "None" "KeepWorld" "KeepWorld" "KeepWorld" false)
  (`PrimitiveComponent.SetCollisionResponseToChannel` (`self.StaticMesh`) "ECC_WorldStatic" "ECR_Overlap")
  (bind _asvrpawn (cast `/Game/Player/VRPawn` (`ActorComponent.GetOwner` AttachTo)))
  (set `self.PlayerGrabbed` _asvrpawn)
  (bind _asmotion_controller_component (cast `MotionControllerComponent` AttachTo))
  (set `self.GrabMCComponent` _asmotion_controller_component))

(event `/Game/VirtualRealityBP/Blueprints/PickupActorInterface.Drop`
  ;[1 0.3928 0] PickUp interface
  (`PrimitiveComponent.SetSimulatePhysics` (`self.StaticMesh`) true)
  (`self.K2_DetachFromActor` "KeepWorld" "KeepWorld" "KeepWorld")
  (`PrimitiveComponent.SetCollisionResponseToChannel` (`self.StaticMesh`) "ECC_WorldStatic" "ECR_Block")
  (set `self.PlayerGrabbed` null)
  (set `self.GrabMCComponent` null))

(event `self.StaticMesh.OnComponentBeginOverlap`
  (params (OverlappedComponent :type "PrimitiveComponent Object Reference") (OtherActor :type "Actor Object Reference") (OtherComp :type "PrimitiveComponent Object Reference") (OtherBodyIndex :type Integer) (bFromSweep :type Boolean) (SweepResult :type "HitResult Structure (by ref)"))
  (`/Engine/EditorBlueprintResources/ActorMacros.Switch Has Authority`
    (:`Authority`
      (bind _asanimal (cast `Animal` OtherActor))
      (if (>= (`KismetMathLibrary.VSize` (`self.VelocityPerFrame`)) (`self.SpeedLimit`))
        (`/Engine/EditorBlueprintResources/StandardMacros.IsValid` (`self.PlayerGrabbed`)
          (:`Is Valid`
            (`GameplayStatics.ApplyDamage` _asanimal (`self.Damage`) null (`self.PlayerGrabbed`) "/Game/Enemy/DamageType/WeaponDamage_BP.WeaponDamage_BP_C")
            (`/Game/Player/VRPawn.RumbleController` (`self.PlayerGrabbed`) 0.7 (`self.GrabMCComponent`))
            (bind _asvrpawn (cast `/Game/Player/VRPawn` (`GameplayStatics.GetPlayerPawn` 0)))
            (`/Game/Player/VRPawn.Multicast SpawnEmitter` :`self` _asvrpawn :`EmitterTemplate` "/Game/FirstPersonBP/Particle/Hit/P_Hit.P_Hit" :`Location` (`SceneComponent.GetSocketLocation` (`self.StaticMesh`) "Sharp") :`Scale` (1.0 1.0 1.0) :`bAutoDestroy` true)))))))

(event `ToShine`
  (if (not (`self.IsShining`))
    (set `self.IsShining` true)
    (bind (_direction _duration) (`Timeline|shine` :!via `PlayFromStart`)
      (:`Update`
        (bind _returnvalue (`PrimitiveComponent.CreateDynamicMaterialInstance` (`self.StaticMesh`) 0 "/Game/Player/Belt/Material/MI_Sword_0.MI_Sword_0" "None"))
        (`MaterialInstanceDynamic.SetScalarParameterValue` _returnvalue "EmissiveBoost" _duration)
        (bind _returnvalue_2 (`PrimitiveComponent.CreateDynamicMaterialInstance` (`self.StaticMesh`) 1 "/Game/Player/Belt/Material/MI_Sword_1.MI_Sword_1" "None"))
        (`MaterialInstanceDynamic.SetScalarParameterValue` _returnvalue_2 "EmissiveBoost" _duration)
        (bind _returnvalue_3 (`PrimitiveComponent.CreateDynamicMaterialInstance` (`self.StaticMesh`) 2 "/Game/Player/Belt/Material/MI_Sword_2.MI_Sword_2" "None"))
        (`MaterialInstanceDynamic.SetScalarParameterValue` _returnvalue_3 "EmissiveBoost" _duration))
      (:`Finished`
        (set `self.IsShining` false)))))

(event `ToBecomeOriginal`
  (if (not (`self.isDarking`))
    (set `self.isDarking` true)
    (bind (_direction _duration) (`Timeline|becomeOriginal` :!via `PlayFromStart`)
      (:`Update`
        (bind _returnvalue (`PrimitiveComponent.CreateDynamicMaterialInstance` (`self.StaticMesh`) 0 "/Game/Player/Belt/Material/MI_Sword_0.MI_Sword_0" "None"))
        (`MaterialInstanceDynamic.SetScalarParameterValue` _returnvalue "EmissiveBoost" _duration)
        (bind _returnvalue_2 (`PrimitiveComponent.CreateDynamicMaterialInstance` (`self.StaticMesh`) 1 "/Game/Player/Belt/Material/MI_Sword_1.MI_Sword_1" "None"))
        (`MaterialInstanceDynamic.SetScalarParameterValue` _returnvalue_2 "EmissiveBoost" _duration)
        (bind _returnvalue_3 (`PrimitiveComponent.CreateDynamicMaterialInstance` (`self.StaticMesh`) 2 "/Game/Player/Belt/Material/MI_Sword_2.MI_Sword_2" "None"))
        (`MaterialInstanceDynamic.SetScalarParameterValue` _returnvalue_3 "EmissiveBoost" _duration))
      (:`Finished`
        (set `self.isDarking` false)))))

(event `Server SpawnEmitter`
  (params (Location :type "Vector Structure"))
  (`self.Multicast SpawnEmitter` Location))

(event `Multicast SpawnEmitter`
  (params (Location :type "Vector Structure"))
  (`GameplayStatics.SpawnEmitterAtLocation` "/Game/FirstPersonBP/Particle/Hit/P_Hit.P_Hit" Location))

(fn `UserConstructionScript`)